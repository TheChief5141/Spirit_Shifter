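; Blob projectile attack, likely for the forest mini boss, that turns to face the player until launched.
; LaunchAttack destroys the actor if the player is out of range; otherwise it waits, stops tracking and runs SetTarget.
; SetTarget line-traces toward the player's offset position, marks the impact point with a fading decal and pauses.
; The actor then eases to that point while flagged as attacking, plays an explosion sound and fades out.
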(event EventBeginPlay
  (|CallParentFunction))

(event Collision|EventActorBeginOverlap
  (params (OtherActor :type Actor%20Object%20Reference))
  (|CallParentFunction OtherActor) ; This node is disabled and will not be called.\nDrag off pins to build functionality.
)

(event EventTick
  (params (DeltaSeconds :type Float%20%28single-precision%29))
  (Transformation|SetActorRotation (Math|Rotator|FindLookatRotation (Transformation|GetActorLocation) (Transformation|GetActorLocation (Game|GetPlayerCharacter 0)))))

(event EventLaunchAttack
  (bind _blob (Variables|Default|Getblob))
  (bind _rootcomponent (Variables|Transformation|GetRootComponent))
  ;[1 1 1] blob throw attac k
  (if (< (Math|Vector|Distance(Vector) (Transformation|GetActorLocation (Game|GetPlayerCharacter 0)) (Transformation|GetActorLocation)) 5e+03)
    (Utilities|FlowControl|Delay (Variables|Default|GetDelay%20Dur))
    (Components|MoveComponentTo _blob (Variables|/Script/Engine.SceneComponent|GetRelativeLocation _blob) "0, 0, 0" true true 0.2 false)
    (Utilities|FlowControl|Delay 1.0)
    (Actor|Tick|SetActorTickEnabled false)
    (|SetTarget)
    (Variables|Default|SetisAttacking true)
    (Components|MoveComponentTo _rootcomponent (Variables|Default|GetTarget) (Variables|/Script/Engine.SceneComponent|GetRelativeRotation _rootcomponent) true true 0.5 false)
    (Audio|PlaySoundatLocation "/Game/Audio/AudioClips/SFX/explosion_dull.explosion_dull" (Transformation|GetActorLocation) "0, 0, 0" 1.0 1.0 0.0 0 0 0 0)
    (Variables|Default|SetisAttacking false)
    (Utilities|FlowControl|Delay 1.0)
    (CallFunction|FadeOut)
    (else
      (Actor|DestroyActor))))

(fn ConstructionScript
  (|CallParentFunction))