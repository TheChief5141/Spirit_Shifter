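; Forest mini-boss (Gorf) that wakes on seeing the player, shows a boss health bar and faces them.
; Its attack loop leaps to a random tagged pad, then casts blob toss, slam or spin, escalating as health drops.
; Destruction plays an ending sequence if one is set.
; Pitfall and minion-spawning logic exists, but the calls the loop makes to it are empty stubs.
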(event OnSeePawn(PawnSensing)
  (params (Pawn :type Pawn%20Object%20Reference))
  (Utilities|Casting|CastToBP_Iso_PlayerCharacter Pawn)
  (Variables|Default|SetcanAttack true)
  (Utilities|FlowControl|DoOnce false
    (:Completed
      (CallFunction|FireNextAttack)
      (CallFunction|StartHealthBar))))

(event Custom|CheckHealth
  (if (<= (Variables|Default|GetunitHealth) 0.0)
    (Actor|DestroyActor)
    (else
      (|setNextAttackBasedOnHealth))))

(event Custom|BlobToss
  (CallFunction|GorfHop)
  (Utilities|FlowControl|Delay 3.5)
  (Audio|PlaySoundatLocation "/Game/Audio/AudioClips/SFX/Magic_Missiles.Magic_Missiles" (Transformation|GetActorLocation) "0, 0, 0" 1.0 1.0 0.0 0 0 0 0)
  (Animation|PlayAnimMontage "/Game/Animations/Gorf-Anims/Two_Hand_Spell_Casting_Montage.Two_Hand_Spell_Casting_Montage" 1.0 "None")
  (for _index (range -1 1)
    (bind _returnvalue (Game|SpawnActorfromClass "/Game/BluePrints/AI/Gorf/BP_BlobThrow.BP_BlobThrow_C" (Math|Transform|MakeTransform (+ (Transformation|GetActorLocation) (* (Transformation|GetActorRightVector) (* _index 400)) "0.000000,0.000000,300.000000") "0, 0, 0" "1.000000,1.000000,1.000000") "AlwaysSpawn" "MultiplyWithRoot" 0 0))
    (Variables|/Game/BluePrints/AI/Gorf/BP_BlobThrow.BP_BlobThrow_C|SetOffset _returnvalue (Math|Vector|MakeVector (Math|Conversions|ToFloat(Integer) (* _index 250)) (Math|Conversions|ToFloat(Integer) (* _index 250)) -1e+02))
    (Default|Charge _returnvalue (* (+ (Math|Conversions|ToFloat(Integer) _index) 1.0) 0.5))
    (Utilities|FlowControl|Delay (Variables|Default|GetattackCooldown))
    (CallFunction|FireNextAttack)))

(event Custom|BlobSpinAttack
  (bind _returnvalue (Transformation|GetActorLocation))
  (CallFunction|GorfHop)
  (Utilities|FlowControl|Delay 3.5)
  (Audio|PlaySoundatLocation "/Game/Audio/AudioClips/SFX/logSpawnin.logSpawnin" _returnvalue "0, 0, 0" 1.0 1.0 0.0 0 0 0 0)
  (Animation|PlayAnimMontage "/Game/Animations/Gorf-Anims/Mutant_Jumping_Montage.Mutant_Jumping_Montage" 1.0 "None")
  (bind _returnvalue_2 (Game|SpawnActorfromClass "/Game/BluePrints/AI/Gorf/BP_BlobSpin.BP_BlobSpin_C" (Math|Transform|MakeTransform _returnvalue "0, 0, 0" "1.000000,1.000000,1.000000") "AlwaysSpawn" "MultiplyWithRoot" 0 0))
  (Default|Charge _returnvalue_2 0.0)
  (Utilities|FlowControl|Delay (Variables|Default|GetattackCooldown))
  (CallFunction|FireNextAttack))

(event Custom|BlobSlam
  (bind _returnvalue (Transformation|GetActorLocation))
  (CallFunction|GorfHop)
  (Utilities|FlowControl|Delay 3.5)
  (Audio|PlaySoundatLocation "/Game/Audio/AudioClips/SFX/logSpawnin.logSpawnin" _returnvalue "0, 0, 0" 1.0 1.0 0.0 0 0 0 0)
  (Animation|PlayAnimMontage "/Game/Animations/Gorf-Anims/Two_Hand_Spell_Casting_Montage.Two_Hand_Spell_Casting_Montage" 1.0 "None")
  (bind _returnvalue_2 (Game|SpawnActorfromClass "/Game/BluePrints/AI/Gorf/BP_BlobAttack.BP_BlobAttack_C" (Math|Transform|MakeTransform (+ _returnvalue "0.000000,0.000000,-160.000000") "90.000000,0.000000,0.000000" "2.000000,2.000000,2.000000") "Undefined" "MultiplyWithRoot" 0 0))
  (Utilities|FlowControl|Delay 5.0)
  (Default|MoveForward _returnvalue_2)
  (Utilities|FlowControl|Delay (/ (Variables|Default|GetattackCooldown) 2.0))
  (CallFunction|FireNextAttack))

(event Custom|FireNextAttack
  ;[1 0.38 0.1686] Fire next attack
  (if (Variables|Default|GetcanAttack)
    (if (Variables|Default|GetcanPitFall)
      (CallFunction|CreatePitfalls 2))
    (CallFunction|SpawnEnemies)
    (Utilities|FlowControl|Delay 1.5)
    (switch int (Variables|Default|GetnextAttack)
      (:Default
        (CallFunction|BlobSpinAttack)
        (Variables|Default|SetnumEnemiesToSpawn 3))
      (:0
        (CallFunction|BlobToss))
      (:1
        (CallFunction|BlobSlam)
        (Variables|Default|SetnumEnemiesToSpawn 2)))))

(event Custom|FlashHealth
  (bind _mesh (Variables|Character|GetMesh))
  (Rendering|Material|SetScalarParameterValueonMaterials _mesh "color" 1e+03)
  (Utilities|FlowControl|Delay 0.2)
  (Rendering|Material|SetScalarParameterValueonMaterials _mesh "color" 1.0))

(event Custom|GorfHop
  (bind _returnvalue (Transformation|GetActorLocation))
  (bind (_x _y _z) (Class|KismetMathLibrary|BreakVector3f _returnvalue))
  (bind _outactors (Actor|GetAllActorswithTag "pad" :!label _label))
  (if (and (Variables|/Script/Engine.Actor|GetbHidden (.OutItem (Utilities|Array|Random _outactors))) (not (Utilities|Array|ContainsItem (Variables|Default|Getforpitfalls) (.OutItem (Utilities|Array|Random _outactors)))))
    (goto _label)
    (else
      (Variables|Default|SetjumpSpot (.OutItem (Utilities|Array|Random _outactors)))
      (Character|LaunchCharacter (+ (* (+ (Math|Vector|GetForwardVector (Math|Rotator|FindLookatRotation _returnvalue (Transformation|GetActorLocation (Variables|Default|GetjumpSpot)))) (Math|Vector|GetUpVector (Math|Rotator|FindLookatRotation _returnvalue (Transformation|GetActorLocation (Variables|Default|GetjumpSpot))))) (Math|Float|Sqrt (* (Math|Vector|Distance2D(Vector) (Math|Vector2D|MakeVector2D _x _y) (Math|Vector2D|MakeVector2D (.X (Class|KismetMathLibrary|BreakVector3f (Transformation|GetActorLocation (Variables|Default|GetjumpSpot)))) (.Y (Class|KismetMathLibrary|BreakVector3f (Transformation|GetActorLocation (Variables|Default|GetjumpSpot)))))) 4.9e+02))) (Math|Vector|MakeVector 0.0 0.0 (+ (Variables|Default|GetVerticalOffsetJump) (- (.Z (Class|KismetMathLibrary|BreakVector3f (Transformation|GetActorLocation (Variables|Default|GetjumpSpot)))) _z)))) false false))))

(event Custom|CreatePitfalls
  (params (numPitfals :type Integer)))

(event Custom|StartHealthBar
  (bind _returnvalue (UserInterface|CreateWidget "/Game/BluePrints/AI/WaterBoss/WB_WaterBossHPBar.WB_WaterBossHPBar_C" (Game|GetPlayerController 0)))
  (bind _output_get (Variables|Default|SetbossBar _returnvalue))
  (UserInterface|Viewport|AddtoViewport _output_get 0))

(event Custom|Move_Level
  (Game|OpenLevel(byName) " LVL_SpiritTemple"))

(event EventBeginPlay
  (CallFunction|SetPitTags)
  (CallFunction|FireNextAttack))

(event Collision|EventActorBeginOverlap
  (params (OtherActor :type Actor%20Object%20Reference)))

(event EventTick
  (params (DeltaSeconds :type Float%20%28single-precision%29))
  (bind _returnvalue (Transformation|GetActorLocation))
  (bind _returnvalue_2 (Game|GetPlayerCharacter 0))
  (bind _returnvalue_3 (Transformation|GetActorLocation _returnvalue_2))
  (bind _returnvalue_4 (Math|Rotator|FindLookatRotation _returnvalue _returnvalue_3))
  (CallFunction|SetHealthBar)
  (if (and (Variables|Default|GetcanAttack) (Utilities|IsValid (Game|GetPlayerCharacter 0)))
    (Transformation|SetActorRotation (Math|Rotator|MakeRotator (.roll _returnvalue_4) 0.0 (.yaw _returnvalue_4)))
    (CallFunction|CheckHealth)))

(event EventDestroyed
  (bind _ending_sequence (Variables|Default|GetEnding_Sequence))
  (bind _sequenceplayer (Variables|/Script/LevelSequence.LevelSequenceActor|GetSequencePlayer _ending_sequence))
  (Utilities|IsValid _ending_sequence
    (:Is%20Valid
      (Sequencer|Player|Play _sequenceplayer :!class /Script/MovieScene.MovieSceneSequencePlayer)
      (EventDispatchers|BindEventtoOnFinished _sequenceplayer (EventDispatchers|CreateEvent :!event Custom|Move_Level)))))

(event EventOnLanded
  (params (Hit :type Hit%20Result%20Structure%20%28by%20ref%29))
  (Development|PrintString "lalnded")
  (Camera|PlayWorldCameraShake "/Game/BluePrints/Camera/BP_CameraShake.BP_CameraShake_C" (Transformation|GetActorLocation) 0.0 5e+03))

(event Game|Damage|EventAnyDamage
  (params (Damage :type Float%20%28single-precision%29) (DamageType :type Damage%20Type%20Object%20Reference) (InstigatedBy :type Controller%20Object%20Reference) (DamageCauser :type Actor%20Object%20Reference))
  (|CallParentFunction Damage DamageType InstigatedBy DamageCauser)
  (Default|SetHealth (Variables|Default|GetbossBar) (/ (Variables|Default|GetunitHealth) (Variables|Default|GetmaxHealth))))

(fn ConstructionScript)

(fn SpawnEnemies)

(fn MakePitfalls
  (params (NumPitfalls :type Integer))
  (CallFunction|ResetPitfalls)
  (for _index (range 0 NumPitfalls)
    (bind _outactors (Actor|GetAllActorswithTag "pitfall"))
    (Utilities|Array|SetArrayElem (Variables|Default|Getforpitfalls) _index (Utilities|Array|Get(acopy) _outactors (Math|Random|RandomInteger (Math|Random|RandomIntegerinRange 0 (Utilities|Array|Length _outactors)))) true)
    (Rendering|Decal|SpawnDecalatLocation 0 "200.000000,200.000000,200.000000" (Transformation|GetActorLocation (Utilities|Array|Get(acopy) _outactors (Math|Random|RandomInteger (Math|Random|RandomIntegerinRange 0 (Utilities|Array|Length _outactors))))) "-90.000000,0.000000,0.000000" 1.0))
  (for _array_element (Variables|Default|Getforpitfalls)
    (Rendering|SetActorHiddenInGame _array_element true)
    (Collision|SetActorEnableCollision _array_element false)))

(fn ResetPitfalls
  (CallFunction|SetPitTags)
  (Utilities|Array|Clear (Variables|Default|Getforpitfalls))
  (bind _outactors (Actor|GetAllActorswithTag "pitfall"))
  (for _array_element _outactors
    (Rendering|SetActorHiddenInGame _array_element false)
    (Collision|SetActorEnableCollision _array_element true)))

(fn SetHealthBar
  (bind _aswb_frog_health_bar (Utilities|Casting|CastToWB_FrogHealthBar (UserInterface|GetWidget (Variables|Default|GetHealthbarwiddget))))
  (Progress|SetPercent (Variables|/Game/BluePrints/AI/Gorf/WB_FrogHealthBar.WB_FrogHealthBar_C|GetHealthbar _aswb_frog_health_bar) (/ (Variables|Default|GetunitHealth) (Variables|Default|GetmaxHealth))))

(fn SetPitTags
  (bind _outactors (Actor|GetAllActorswithTag "pitfall"))
  (for _array_element _outactors
    (Variables|/Script/Engine.Actor|SetTags _array_element (Utilities|Array|MakeArray (Utilities|Name|MakeLiteralName "pitfall") (Utilities|Name|MakeLiteralName "pad")))))