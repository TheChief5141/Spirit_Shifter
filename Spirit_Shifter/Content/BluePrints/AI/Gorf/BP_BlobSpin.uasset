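; BP_BlobSpin is a short-lived spinning blob attack, filed under Gorf's AI, that damages the isometric player character.
; LaunchAttack turns on a per-tick yaw spin while timed component moves sweep along local Y, then stops the spin and calls FadeOut.
; Box1 overlap applies fixed damage to the player, independent of the attack state.
; UpdateMaterials forwards scalar parameters to Blob's materials, and a lifespan set on BeginPlay removes the actor.
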(event OnComponentBeginOverlap(Box1)
  (params (OverlappedComponent :type Primitive%20Component%20Object%20Reference) (OtherActor :type Actor%20Object%20Reference) (OtherComp :type Primitive%20Component%20Object%20Reference) (OtherBodyIndex :type Integer) (bFromSweep :type Boolean) (SweepResult :type Hit%20Result%20Structure%20%28by%20ref%29))
  (Utilities|Casting|CastToBP_Iso_PlayerCharacter OtherActor)
  (Game|Damage|ApplyDamage 0 8.0 0 0))

(event EventBeginPlay
  (|CallParentFunction)
  (Actor|SetLifeSpan 7.0))

(event Collision|EventActorBeginOverlap
  (params (OtherActor :type Actor%20Object%20Reference))
  (|CallParentFunction OtherActor) ; This node is disabled and will not be called.\nDrag off pins to build functionality.
)

(event EventTick
  (params (DeltaSeconds :type Float%20%28single-precision%29))
  (if (Variables|Default|GetisAttacking)
    (Transformation|SetActorRotation (Math|Rotator|MakeRotator 0.0 0.0 (+ (.yaw (Transformation|GetActorRotation)) 2e+01)))))

(event EventLaunchAttack
  (Variables|Default|SetisAttacking true)
  (Components|MoveComponentTo (Variables|Default|Getblob) "0.000000,650.000000,0.000000" "0, 0, 0" false false 2.0 false)
  (Components|MoveComponentTo 0 "0.000000,-650.000000,0.000000" "0, 0, 0" false false 2.0 false)
  (Variables|Default|SetisAttacking false)
  (CallFunction|FadeOut))

(fn ConstructionScript
  (|CallParentFunction))

(fn UpdateMaterials
  (params (ParameterValue :type Float%20%28single-precision%29) (ParameterName :type Name :default "None"))
  (Rendering|Material|SetScalarParameterValueonMaterials (Variables|Default|Getblob) ParameterName ParameterValue))