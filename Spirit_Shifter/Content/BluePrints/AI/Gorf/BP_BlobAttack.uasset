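; Short-lived blob attack actor that fades in on spawn, slams down toward the player, then dissolves and destroys itself.
; It yaws toward the player on Tick until the attack disables ticking and tips the root over with MoveComponentTo.
; Timelines drive the material mask and dither fade through UpdateMaterials.
; Box overlap damages BP_Iso_PlayerCharacter at any stage, as the IsAttacking check is disconnected.
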(event OnComponentBeginOverlap(Box)
  (params (OverlappedComponent :type Primitive%20Component%20Object%20Reference) (OtherActor :type Actor%20Object%20Reference) (OtherComp :type Primitive%20Component%20Object%20Reference) (OtherBodyIndex :type Integer) (bFromSweep :type Boolean) (SweepResult :type Hit%20Result%20Structure%20%28by%20ref%29))
  ;[1 0 0.01983] where character will take damage
  (Utilities|Casting|CastToBP_Iso_PlayerCharacter OtherActor)
  (Game|Damage|ApplyDamage OtherActor 16.0 0 0))

(event Custom|Charge
  (params (Delay :type Float%20%28double-precision%29))
  (bind _mask (Timeline|Fade_IN Play)
    (:Update
      (CallFunction|UpdateMaterials _mask "mask"))
    (:Finished
      (CallFunction|LaunchAttack))))

(event Custom|LaunchAttack
  (bind _blob (Variables|Default|Getblob))
  (Components|MoveComponentTo _blob (Variables|/Script/Engine.SceneComponent|GetRelativeLocation _blob) "90.000000,0.000000,0.000000" true true 0.2 false)
  (Utilities|FlowControl|Delay 1.0)
  (Actor|Tick|SetActorTickEnabled false)
  (Variables|Default|SetisAttacking true)
  (Components|MoveComponentTo (Variables|Transformation|GetRootComponent) (Transformation|GetActorLocation) (Math|Rotator|MakeRotator 0.0 -9e+01 (.yaw (Transformation|GetActorRotation))) true true 0.5 false)
  (Variables|Default|SetisAttacking true)
  (Utilities|FlowControl|Delay 1.0)
  (CallFunction|FadeOut))

(event Custom|FadeOut
  (bind _ditheramount (Timeline|Dither_Fade Play)
    (:Update
      (CallFunction|UpdateMaterials _ditheramount "Alpha Threshold (S)"))
    (:Finished
      (Utilities|FlowControl|Delay 0.2)
      (Actor|SetLifeSpan 0.01))))

(event Custom|MoveForward
  (Components|MoveComponentTo (Variables|Default|Getblob) (Variables|/Script/Engine.SceneComponent|GetRelativeLocation (Variables|Default|GetArrow)) "90.000000,0.000000,0.000000" false true 0.5 false))

(event EventBeginPlay
  (CallFunction|Charge 0.0))

(event Collision|EventActorBeginOverlap
  (params (OtherActor :type Actor%20Object%20Reference)))

(event EventTick
  (params (DeltaSeconds :type Float%20%28single-precision%29))
  (Transformation|SetActorRotation (Math|Rotator|MakeRotator 0.0 0.0 (.yaw (Math|Rotator|FindLookatRotation (Transformation|GetActorLocation) (Transformation|GetActorLocation (Game|GetPlayerCharacter 0)))))))

(fn ConstructionScript)

(fn UpdateMaterials
  (params (ParameterValue :type Float%20%28single-precision%29) (ParameterName :type Name))
  (Rendering|Material|SetScalarParameterValueonMaterials (Variables|Default|Getblob) ParameterName ParameterValue))