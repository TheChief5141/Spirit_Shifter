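; Combat encounter manager that seals the player inside a ring arena and tracks the fight within it.
; Player overlap with the child volume raises the collidable ring, enters combat mode and lets enemies found by sphere trace attack.
; Death and destroy events prune enemy and spirit lists, updating projectile damage or retargeting enemies as spirits die, and removing the manager once enemies are gone.
; Toggling off autosaves, exits combat and can move a level-event actor.
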(event Custom|Destroy_Event_For_Units_In_Combat
  (params (DestroyedActor :type Actor%20Object%20Reference))
  (bind _enemy_list (Variables|Default|GetEnemy_List))
  (bind _returnvalue (Utilities|Array|Length _enemy_list))
  ;[1 1 1] Do Foreach to Check if still Valid
  (if (Utilities|Array|ContainsItem _enemy_list DestroyedActor)
    (Utilities|Array|RemoveItem _enemy_list DestroyedActor)
    (Development|PrintString (Utilities|String|ToString(Integer) _returnvalue))
    (if (<= _returnvalue 0)
      (CallFunction|DisableCombatManager)
      (Development|PrintString "turned off"))))

(event Custom|Collision_For_Volume
  (params (OverlappedComponent :type Primitive%20Component%20Object%20Reference) (OtherActor :type Actor%20Object%20Reference) (OtherComp :type Primitive%20Component%20Object%20Reference) (OtherBodyIndex :type Integer) (bFromSweep :type Boolean) (SweepResult :type Hit%20Result%20Structure%20%28by%20ref%29))
  (if (and (Utilities|ClassIsChildOf (Utilities|GetClass OtherActor) "/Game/BluePrints/Player/BP_Iso_PlayerCharacter.BP_Iso_PlayerCharacter_C") (Variables|Default|GetCanBattle?))
    (CallFunction|ToggleState true)))

(event Custom|Bind_Enemies_To_Disable
  (params (Enemy_Actor :type Actor%20Object%20Reference))
  (Game|BindEventtoOnDestroyed Enemy_Actor (EventDispatchers|CreateEvent :!event Custom|Destroy_Event_For_Units_In_Combat)))

(event Custom|Move_Volume
  (bind _mesh (Variables|Default|GetMesh))
  (Transformation|SetMobility _mesh "Movable")
  (Utilities|FlowControl|FlipFlop
    (:A
      (Development|PrintString "move up")
      (Rendering|SetVisibility _mesh true false)
      (bind _movement (Timeline|Timeline Play)
        (:Update
          (Transformation|SetWorldLocation _mesh (+ (Math|Vector|MakeVector 0.0 0.0 (* _movement (Variables|Default|GetDistance_Multiplier))) (Transformation|GetWorldLocation _mesh)) false false))
        (:Finished
          (Transformation|SetMobility _mesh "Static"))))
    (:B
      (Rendering|SetVisibility _mesh false false)
      (Variables|Default|SetCanBattle? false))))

(event Custom|Play_Level_Event
  (bind _level_event (Variables|Default|GetLevel_Event))
  (bind _returnvalue (Transformation|GetActorLocation _level_event))
  (bind _location (Timeline|Timeline_0 Play)
    (:Update
      (Transformation|SetActorLocation _level_event (Math|Vector|MakeVector (.x _returnvalue) (.y _returnvalue) (Math|Float|Lerp (.x _returnvalue) (+ (.x _returnvalue) (Variables|Default|GetDownMultiplier)) _location)) false false))))

(event Custom|Disable_Combat_Manager
  ;[1 1 1] Do Foreach to Check if still Valid
  (for _array_element (Variables|Default|GetEnemy_List)
    (Actor|DestroyActor _array_element))
  (for _array_element_2 (Variables|Default|GetSpirit_List)
    (bind _asbp_spirit (Utilities|Casting|CastToBP_Spirit _array_element_2))
    (Variables|/Game/BluePrints/Spirits/Parent/BP_Spirit.BP_Spirit_C|SetMy_State _asbp_spirit "NewEnumerator1"))
  (Actor|DestroyActor))

(event Custom|Enemy_Check
  (bind _enemy_list (Variables|Default|GetEnemy_List))
  ;[1 1 1] Do Foreach to Check if still Valid
  (for _array_element _enemy_list
    (Utilities|IsValid _array_element
      (:Is%20Not%20Valid
        (Utilities|Array|RemoveItem _enemy_list _array_element))))
  (if (== (Utilities|Array|Length _enemy_list) 0)
    (CallFunction|DisableCombatManager)
    (else
      (Utilities|FlowControl|Delay 2.0)
      (CallFunction|EnemyCheck))))

(event Custom|DeathAssigner
  (params (Enemy :type Actor%20Object%20Reference))
  ;[1 1 1] Do Foreach to Check if still Valid
  (bind _asbp_ai (Utilities|Casting|CastToBP_AI_Combine Enemy))
  (EventDispatchers|BindEventtoOnDeath _asbp_ai (delegate Custom|Checkers)))

(event Custom|Checkers
  (params (Actor :type Actor%20Object%20Reference))
  (bind _enemy_list (Variables|Default|GetEnemy_List))
  ;[1 1 1] Do Foreach to Check if still Valid
  (for _array_element _enemy_list
    (Utilities|IsValid _array_element
      (:Is%20Not%20Valid
        (Utilities|Array|RemoveItem _enemy_list _array_element))))
  (if (== (Utilities|Array|Length _enemy_list) 0)
    (CallFunction|DisableCombatManager)
    (else
      (Utilities|FlowControl|Delay 2.0)
      (CallFunction|EnemyCheck))))

(event Custom|AddSpirit
  (params (IncomingSpirit :type Actor%20Object%20Reference))
  (bind _asbp_spirit (Utilities|Casting|CastToBP_Spirit IncomingSpirit))
  (EventDispatchers|BindEventtoOnDeath _asbp_spirit (delegate Custom|CheckSpirit)))

(event Custom|CheckSpirit
  (bind _spirit_list (Variables|Default|GetSpirit_List))
  (Utilities|Array|RemoveIndex _spirit_list)
  (if (== (Utilities|Array|Length _spirit_list) 0)
    (Development|PrintString "ALL SPIRIT DEAD" true true "(R=0.434154,G=0.003474,B=0.000000,A=1.000000)" 2e+01)
    (Default|UpdateProjectileDamage (Variables|Default|GetisoChar) 1.0)
    (for _array_element (Variables|Default|GetEnemy_List)
      (if (Utilities|DoesObjectImplementInterface _array_element "/Game/BluePrints/AI/Combat/BPI_Attacker.BPI_Attacker_C")
        (Class|BPIAttacker|TargetPlayer(Message) _array_element)))
    (else
      (Default|UpdateProjectileDamage (Variables|Default|GetisoChar) 19.99))))

(event EventBeginPlay
  (bind _mesh (Variables|Default|GetMesh))
  (bind _mesh_2 (Variables|Default|GetMesh))
  (bind _relativelocation (Variables|/Script/Engine.SceneComponent|GetRelativeLocation _mesh))
  (bind _childactor (Variables|/Script/Engine.ChildActorComponent|GetChildActor _mesh_2))
  (if (Variables|Default|GetisBossArena)
    (bind _asbp_combat_ring_no_middle_1 (Utilities|Casting|CastToBP_Combat_Ring_NoMiddle1 _childactor))
    (Variables|Default|SetAs%20BP%20Combat%20Ring _asbp_combat_ring_no_middle_1)
    (else
      (bind _asbp_combat_ring (Utilities|Casting|CastToBP_Combat_Ring _childactor))
      (Variables|Default|SetAs%20BP%20Combat%20Ring _asbp_combat_ring)))
  (Collision|SetCollisionEnabled (Variables|/Game/BluePrints/AI/Combat/BP_Combat_Ring.BP_Combat_Ring_C|GetStaticMesh (Variables|Default|GetAs%20BP%20Combat%20Ring)) "NoCollision")
  (Rendering|SetVisibility _mesh_2 false false)
  (bind _asbp_combat_volume (Utilities|Casting|CastToBP_Combat_Volume (Variables|/Script/Engine.ChildActorComponent|GetChildActor (Variables|Default|GetVolume))))
  (bind _output_get (Variables|Default|SetAs%20BP%20Combat%20Volume _asbp_combat_volume))
  (Collision|BindEventtoOnComponentBeginOverlap (Variables|/Game/BluePrints/Volumes/BP_Combat_Volume.BP_Combat_Volume_C|GetBox _output_get) (EventDispatchers|CreateEvent :!event Custom|Collision_For_Volume))
  (CallFunction|SetupEnemies _relativelocation _relativelocation)
  (EventDispatchers|BindEventtoDisable (EventDispatchers|CreateEvent :!event Custom|Disable_Combat_Manager))
  (bind _asbp_iso_player_controller (Utilities|Casting|CastToBP_Iso_Player_Controller (Game|GetPlayerController 0)))
  (Variables|Default|SetAs%20BP%20Iso%20Player%20Controller _asbp_iso_player_controller)
  (bind _asbp_iso_player_character (Utilities|Casting|CastToBP_Iso_PlayerCharacter (Game|GetPlayerCharacter 0)))
  (Variables|Default|SetisoChar _asbp_iso_player_character))

(event EventToggleState
  (params (On/Off :type Boolean))
  (bind _returnvalue (Game|GetPlayerController 0))
  (bind _as_bp_combat_ring (Variables|Default|GetAs%20BP%20Combat%20Ring))
  (bind _asbp_iso_player_controller (Utilities|Casting|CastToBP_Iso_Player_Controller _returnvalue))
  (bind _staticmesh (Variables|/Game/BluePrints/AI/Combat/BP_Combat_Ring.BP_Combat_Ring_C|GetStaticMesh _as_bp_combat_ring))
  (if On/Off
    (Utilities|Casting|CastToBP_Combat_Ring (Variables|/Script/Engine.ChildActorComponent|GetChildActor (Variables|Default|GetMesh)))
    (Collision|SetCollisionEnabled _staticmesh "QueryAndPhysics")
    (Default|CallEnterCombatMode _asbp_iso_player_controller "NewEnumerator0")
    (CallFunction|MoveVolume)
    (Collision|UnbindEventfromOnComponentBeginOverlap (Variables|/Game/BluePrints/Volumes/BP_Combat_Volume.BP_Combat_Volume_C|GetBox (Variables|Default|GetAs%20BP%20Combat%20Volume)) (delegate Custom|Collision_For_Volume))
    (for _array_element (Variables|Default|GetEnemy_List)
      (Class|BPIAttacker|SetCanAttack(Message) _array_element true))
    (else
      (Default|AutosaveCheckpoint (Variables|Default|GetAs%20BP%20Iso%20Player%20Controller) self)
      (Rendering|SetVisibility _staticmesh false false)
      (Collision|SetCollisionEnabled _staticmesh "NoCollision")
      (Default|ExitCombatAreaEvent _asbp_iso_player_controller "NewEnumerator1")
      (CallFunction|MoveVolume)
      (Variables|Default|SetCanBattle? false)
      (Utilities|IsValid (Variables|Default|GetLevel_Event)
        (:Is%20Valid
          (CallFunction|PlayLevelEvent))))))

(fn ConstructionScript
  (Transformation|SetWorldScale3D (Variables|Default|GetMesh) (Variables|Default|GetRadius_of_Mesh)))

(fn SetupEnemies
  (params (End :type Vector) (Start :type Vector))
  (bind (_outhits _returnvalue) (Collision|MultiSphereTraceByChannel Start End 1e+03 "TraceTypeQuery1" false 0 "None"))
  (if _returnvalue
    (for _array_element _outhits
      (if (and (Utilities|ClassIsChildOf (Utilities|GetClass (.HitActor (Collision|BreakHitResult _array_element))) "/Game/BluePrints/AI/BP_UnitStats.BP_UnitStats_C") (not (Utilities|ClassIsChildOf (Utilities|GetClass (.HitActor (Collision|BreakHitResult _array_element))) "/Game/BluePrints/Player/BP_Iso_PlayerCharacter.BP_Iso_PlayerCharacter_C")))
        (Utilities|Array|Add (Variables|Default|GetEnemy_List) (.HitActor (Collision|BreakHitResult _array_element)))
        (Game|BindEventtoOnDestroyed (.HitActor (Collision|BreakHitResult _array_element)) (EventDispatchers|CreateEvent :!event Custom|Destroy_Event_For_Units_In_Combat))
        (Development|PrintString (Utilities|String|ToString(Text) (Utilities|Text|FormatText "Binded Event to: {X}" (Utilities|GetObjectName (.HitActor (Collision|BreakHitResult _array_element))))))))))