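; BP_Spawner is an AI spawner actor that spawns EnemyToSpawn at its own transform plus a stored location offset.
; When active, given a valid class and not in WaveSpawnMode, it starts a looping spawn timer on BeginPlay.
; Independently of those flags, player-class overlaps with its Box trigger a random-count burst, re-rolling the X/Y offset within SpawnDistance for each spawn.
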(event OnComponentBeginOverlap(Box)
  (params (OverlappedComponent :type Primitive%20Component%20Object%20Reference) (OtherActor :type Actor%20Object%20Reference) (OtherComp :type Primitive%20Component%20Object%20Reference) (OtherBodyIndex :type Integer) (bFromSweep :type Boolean) (SweepResult :type Hit%20Result%20Structure%20%28by%20ref%29))
  (bind _spawn_distance (Variables|Default|GetSpawn_Distance))
  (if (Utilities|ClassIsChildOf (Utilities|GetClass OtherActor) (Utilities|GetClass (Game|GetPlayerCharacter 0)))
    (for _index (range 0 (Math|Random|RandomInteger (Variables|Default|GetNumber_To_Spawn)))
      (Variables|Default|SetSpawn%20Transform (Math|Transform|MakeTransform (Math|Vector|MakeVector (* (Math|Random|RandomFloat) _spawn_distance) (* (Math|Random|RandomFloat) _spawn_distance) 0.0) "0, 0, 0" "1.000000,1.000000,1.000000"))
      (CallFunction|SpawnEnemy))))

(event Custom|Spawn_Enemy
  (bind _returnvalue (Transformation|GetActorTransform))
  (Game|SpawnActorfromClass (Variables|Default|GetEnemy_To_Spawn) (Math|Transform|MakeTransform (+ (.location _returnvalue) (.location (Variables|Default|GetSpawn%20Transform))) (.rotation _returnvalue) (.scale _returnvalue)) "Undefined" "MultiplyWithRoot" 0 0))

(event EventBeginPlay
  (if (Math|Boolean|ANDBoolean (Utilities|IsValidClass (Variables|Default|GetEnemy_To_Spawn)) (Variables|Default|GetActive_Spawner) (not (Variables|Default|GetWave_Spawn_Mode)))
    (Utilities|Time|SetTimerbyEvent (EventDispatchers|CreateEvent :!event Custom|Spawn_Enemy) (Variables|Default|GetSpawn_Time) true)))

(event Collision|EventActorBeginOverlap
  (params (OtherActor :type Actor%20Object%20Reference)))

(event EventTick
  (params (DeltaSeconds :type Float%20%28single-precision%29)))

(fn ConstructionScript)