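; BP_UnitStats is a unit Blueprint that handles health, damage feedback and death.
; After a two-second post-spawn delay, AnyDamage lowers and prints health, calling UnitDeath at zero.
; Surviving enemies play hit sound, Niagara effect and an empty HitRegistration event; bosses flash health on the first BP_ForestMiniBoss found.
; UnitDeath notifies the attached combat manager and destroys the actor, only for enemies or bosses.
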(event Custom|UnitDeath
  (if (or (Variables|Default|GetisEnemy) (Variables|Default|GetisBoss))
    (Default|DestroyEventforUnitsinCombat (Variables|Default|GetAttached_Combat_Manager) self)
    (Actor|DestroyActor)))

(event Custom|HitRegistration)

(event EventBeginPlay
  (Utilities|FlowControl|Delay 2.0)
  (Variables|Default|SetcanTakeDamage true))

(event Collision|EventActorBeginOverlap
  (params (OtherActor :type Actor%20Object%20Reference)))

(event EventTick
  (params (DeltaSeconds :type Float%20%28single-precision%29)))

(event Game|Damage|EventAnyDamage
  (params (Damage :type Float%20%28single-precision%29) (DamageType :type Damage%20Type%20Object%20Reference) (InstigatedBy :type Controller%20Object%20Reference) (DamageCauser :type Actor%20Object%20Reference))
  (bind _returnvalue (Transformation|GetActorLocation))
  (bind _returnvalue_2 (+ _returnvalue "0.000000,0.000000,50.000000"))
  (if (Variables|Default|GetcanTakeDamage)
    (Variables|Default|SetunitHealth (- (Variables|Default|GetunitHealth) Damage))
    (Development|PrintString (Utilities|String|ToString(Float) (Variables|Default|GetunitHealth)))
    (if (<= (Variables|Default|GetunitHealth) 0.0)
      (CallFunction|UnitDeath)
      (elif (Variables|Default|GetisEnemy)
        (Audio|PlaySoundatLocation "/Game/Audio/AudioClips/SFX/Monster-2.Monster-2" _returnvalue_2 "0, 0, 0" 1.0 1.0 0.0 "/Game/Audio/EnemyAtten.EnemyAtten" 0 0 0)
        (Niagara|SpawnSystematLocation "/Game/BluePrints/AI/NS_EnemyHIt.NS_EnemyHIt" _returnvalue_2 "0, 0, 0" (Transformation|GetActorScale3D))
        (CallFunction|HitRegistration)
        (elif (Variables|Default|GetisBoss)
          (bind _returnvalue_3 (Actor|GetActorOfClass "/Game/BluePrints/AI/MiniBoss/BP_ForestMiniBoss.BP_ForestMiniBoss_C"))
          (Default|FlashHealth _returnvalue_3))))))

(fn ConstructionScript)