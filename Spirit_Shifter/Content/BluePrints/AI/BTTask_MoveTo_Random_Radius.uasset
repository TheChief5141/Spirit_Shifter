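; Behavior tree task that moves a Combine AI pawn to a randomly chosen attack position relative to its target.
; It passes the blackboard TargetActor and a random one of four directions to the pawn's DetermineAttackLocation, with a fixed small radius.
; The result is saved as SenseLocation and used by AIMoveTo, whose outcome finishes the task.
; Pawns not derived from BP_AI_Combine never finish the task.
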(event EventReceiveExecuteAI
  (params (OwnerController :type AI%20Controller%20Object%20Reference) (ControlledPawn :type Pawn%20Object%20Reference))
  (bind _asbp_ai_combine (Utilities|Casting|CastToBP_AI_Combine ControlledPawn))
  (bind _returnvalue (AI|GetAIController _asbp_ai_combine))
  (bind _returnvalue_2 (AI|GetBlackboard _returnvalue))
  (if (Utilities|ClassIsChildOf (Utilities|GetClass ControlledPawn) "/Game/BluePrints/AI/BP_AI_Combine.BP_AI_Combine_C")
    (bind _attack_location (Default|DetermineAttackLocation _asbp_ai_combine (.AsActor (Utilities|Casting|CastToActor (AI|Components|Blackboard|GetValueasObject _returnvalue_2 (Utilities|Name|MakeLiteralName "TargetActor")))) (Math|Random|RandomInteger 4) 3e+01))
    (AI|Components|Blackboard|SetValueasVector _returnvalue_2 (Utilities|Name|MakeLiteralName "SenseLocation") _attack_location)
    (AI|AIMoveTo ControlledPawn _attack_location 0 5.0 false
      (:OnSuccess
        (AI|BehaviorTree|FinishExecute true))
      (:OnFail
        (AI|BehaviorTree|FinishExecute false)))))