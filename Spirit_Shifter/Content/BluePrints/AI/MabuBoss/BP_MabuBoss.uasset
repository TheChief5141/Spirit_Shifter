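; Mabu boss character that picks a random attack state and writes it to the AI blackboard.
; RunForward timeline charges along the player's direction captured at start; hitbox overlaps launch the player and damage once per charge.
; Incoming damage advances health-threshold phases, signals DPS completion below a target, and updates the boss bar widget.
; Health also drives a "Position" material parameter on the mesh.
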(event OnComponentBeginOverlap(hitbox)
  (params (OverlappedComponent :type Primitive%20Component%20Object%20Reference) (OtherActor :type Actor%20Object%20Reference) (OtherComp :type Primitive%20Component%20Object%20Reference) (OtherBodyIndex :type Integer) (bFromSweep :type Boolean) (SweepResult :type Hit%20Result%20Structure%20%28by%20ref%29))
  (bind _returnvalue (Transformation|GetActorRotation))
  (bind _launch_multiplier (Variables|Default|Getlaunch%20multiplier))
  (bind _returnvalue_2 (Math|Vector|GetForwardVector _returnvalue))
  (bind _returnvalue_3 (* _returnvalue_2 _launch_multiplier))
  (bind _asbp_iso_player_character (Utilities|Casting|CastToBP_Iso_PlayerCharacter OtherActor))
  (Character|LaunchCharacter _asbp_iso_player_character (Math|Vector|MakeVector (.x _returnvalue_3) (.y _returnvalue_3) 7.5e+02) false true)
  (if (Variables|Default|GetcanHit)
    (Game|Damage|ApplyDamage _asbp_iso_player_character 1e+01 0 0)
    (Variables|Default|SetcanHit false)))

(event Custom|RandomState
  (Utilities|FlowControl|Sequence
    (:then_0
      (switch int (Math|Random|RandomInteger 3)
        (:0
          (Variables|Default|SetMyState "NewEnumerator0"))
        (:1
          (Variables|Default|SetMyState "NewEnumerator1"))
        (:2
          (Variables|Default|SetMyState "NewEnumerator2"))))
    (:then_1
      (AI|Components|Blackboard|SetValueasEnum (AI|GetBlackboard (AI|GetAIController self)) (Utilities|Name|MakeLiteralName "AttackState") (Variables|Default|GetMyState)))))

(event Custom|RunForward
  (bind _returnvalue (Transformation|GetActorLocation))
  (bind _returnvalue_2 (Game|GetPlayerCharacter 0))
  (bind _returnvalue_3 (Transformation|GetActorLocation _returnvalue_2))
  (bind _returnvalue_4 (Math|Rotator|FindLookatRotation _returnvalue _returnvalue_3))
  (Variables|Default|SetcanHit true)
  (Transformation|SetActorRotation (Math|Rotator|MakeRotator (.roll _returnvalue_4) 0.0 (.yaw _returnvalue_4)))
  (Variables|Default|SetRunSpot (Math|Vector|GetForwardVector (Math|Rotator|MakeRotator (.roll _returnvalue_4) (.pitch _returnvalue_4) (.yaw _returnvalue_4))))
  (bind _speed (Timeline|MoveForward PlayFromStart)
    (:Update
      (Transformation|SetActorLocation (+ (Transformation|GetActorLocation) (* (Variables|Default|GetRunSpot) _speed)) true false))
    (:Finished
      (Variables|Default|SetcanHit false))))

(event Custom|LookAtPlayer
  (Timeline|LerpToPlayerRotation PlayFromStart))

(event Custom|StartHealthBar
  (bind _returnvalue (UserInterface|CreateWidget "/Game/BluePrints/AI/WaterBoss/WB_WaterBossHPBar.WB_WaterBossHPBar_C" (Game|GetPlayerController 0)))
  (bind _output_get (Variables|Default|SetbossBar _returnvalue))
  (UserInterface|Viewport|AddtoViewport _output_get 0))

(event EventBeginPlay
  (|CallParentFunction)
  (Animation|Montage|PlayMontage (Variables|Character|GetMesh) "/Game/Animations/Mabu/Animations/AM_MabuIdle.AM_MabuIdle"
    (:then
      (CallFunction|RandomState)
      (Variables|Default|SetmaxHealth (Variables|Default|GetunitHealth)))))

(event Collision|EventActorBeginOverlap
  (params (OtherActor :type Actor%20Object%20Reference))
  (|CallParentFunction OtherActor) ; This node is disabled and will not be called.\nDrag off pins to build functionality.
)

(event EventTick
  (params (DeltaSeconds :type Float%20%28single-precision%29))
  (|CallParentFunction DeltaSeconds) ; This node is disabled and will not be called.\nDrag off pins to build functionality.
)

(event EventAnyDamage
  (params (Damage :type Float%20%28single-precision%29) (DamageType :type Damage%20Type%20Object%20Reference) (InstigatedBy :type Controller%20Object%20Reference) (DamageCauser :type Actor%20Object%20Reference))
  ;[1 0 0] Healthstuff
  (|CallParentFunction Damage DamageType InstigatedBy DamageCauser)
  (CallFunction|UpdateHealth)
  (Utilities|FlowControl|Sequence
    (:then_0
      (if (< (Variables|Default|GetunitHealth) 3e+02)
        (Variables|Default|SetPhase 3)
        (Development|PrintString "new phase")
        (elif (< (Variables|Default|GetunitHealth) 6e+02)
          (Variables|Default|SetPhase 2)
          (Development|PrintString "phase 2"))))
    (:then_1
      (if (< (Variables|Default|GetunitHealth) 4.5e+02)
        _))
    (:then_2
      (if (< (Variables|Default|GetunitHealth) (Variables|Default|GetdpsTarget))
        (Default|CallOnDPSCompleted)))
    (:then_3
      (Default|SetHealth (Variables|Default|GetbossBar) (/ (Variables|Default|GetunitHealth) (Variables|Default|GetmaxHealth))))))

(fn ConstructionScript
  (|CallParentFunction))

(fn GetRunPoint
  (params (Speed :type Float%20%28double-precision%29))
  (return (+ (* Speed (Math|Vector|GetForwardVector (Math|Rotator|FindLookatRotation (Transformation|GetActorLocation) (Transformation|GetActorLocation (Game|GetPlayerCharacter 0))))) (Transformation|GetActorLocation))))

(fn UpdateHealth
  (Rendering|Material|SetScalarParameterValueonMaterials (Variables|Character|GetMesh) "Position" (Math|Float|Lerp 24.0 -72.0 (/ (Variables|Default|GetunitHealth) 9e+02))))