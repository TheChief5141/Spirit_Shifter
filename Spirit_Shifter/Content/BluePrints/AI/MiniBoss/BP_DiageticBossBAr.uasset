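; BP_DiageticBossBAr is a diegetic health bar for the forest miniboss, shown through the materials of three log components.
; Every tick it looks up BP_ForestMiniBoss with GetActorOfClass and passes its UnitHealth to UpdateMaterials.
; That event maps one 333-point band of health to each log, from Log at the top to Log3 at the bottom.
; Each log's "mask" scalar rises as health drops through its band, with no clamping.
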(event Custom|UpdateMaterials
  (params (health :type Float%20%28double-precision%29))
  (Variables|Default|SetHealth health)
  (Utilities|FlowControl|Sequence
    (:then_0
      (Rendering|Material|SetScalarParameterValueonMaterials (Variables|Default|GetLog) "mask" (* (- (/ (- (Variables|Default|GetHealth) 666.0) 333.0) 1.0) -1.0)))
    (:then_1
      (Rendering|Material|SetScalarParameterValueonMaterials (Variables|Default|Getlog2) "mask" (* (- (/ (- (Variables|Default|GetHealth) 333.0) 333.0) 1.0) -1.0)))
    (:then_2
      (Rendering|Material|SetScalarParameterValueonMaterials (Variables|Default|Getlog3) "mask" (* (- (/ (Variables|Default|GetHealth) 333.0) 1.0) -1.0)))))

(event EventBeginPlay)

(event Collision|EventActorBeginOverlap
  (params (OtherActor :type Actor%20Object%20Reference)))

(event EventTick
  (params (DeltaSeconds :type Float%20%28single-precision%29))
  (bind _returnvalue (Actor|GetActorOfClass "/Game/BluePrints/AI/MiniBoss/BP_ForestMiniBoss.BP_ForestMiniBoss_C"))
  (CallFunction|UpdateMaterials (Variables|/Game/BluePrints/AI/BP_UnitStats.BP_UnitStats_C|GetunitHealth _returnvalue)))

(fn ConstructionScript)