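; BP_BlobThrow is a mini-boss attack actor that performs a timed tipping attack when LaunchAttack is called.
; LaunchAttack rotates the Blob component, waits, disables tick, then pitches the root to 90 degrees in place while IsAttacking is set.
; It then clears the flag, pauses and calls FadeOut.
; Tick is empty, and the logic to face the player is disconnected, so it never runs.
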(event EventBeginPlay
  (|CallParentFunction) ; This node is disabled and will not be called.\nDrag off pins to build functionality.
)

(event Collision|EventActorBeginOverlap
  (params (OtherActor :type Actor%20Object%20Reference))
  (|CallParentFunction OtherActor) ; This node is disabled and will not be called.\nDrag off pins to build functionality.
)

(event EventTick
  (params (DeltaSeconds :type Float%20%28single-precision%29)))

(event EventLaunchAttack
  (bind _blob (Variables|Default|Getblob))
  (Components|MoveComponentTo _blob (Variables|/Script/Engine.SceneComponent|GetRelativeLocation _blob) "0.000000,90.000000,0.000000" true true 0.2 false)
  (Utilities|FlowControl|Delay 1.0)
  (Actor|Tick|SetActorTickEnabled false)
  (Variables|Default|SetisAttacking true)
  (Components|MoveComponentTo (Variables|Transformation|GetRootComponent) (Transformation|GetActorLocation) (Math|Rotator|MakeRotator 0.0 9e+01 (.yaw (Transformation|GetActorRotation))) true true 0.5 false)
  (Variables|Default|SetisAttacking false)
  (Utilities|FlowControl|Delay 1.0)
  (CallFunction|FadeOut))

(fn ConstructionScript
  (|CallParentFunction))