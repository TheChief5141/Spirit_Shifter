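; Enemy AI unit that chases and damages the player on overlap and can merge with nearby units of its kind.
; CheckEnemies box-traces for combinable allies, randomly gathers them through blackboard keys, destroys them and grows into a tougher big form.
; On death it shrinks, then a big unit splits into two new units while a small one releases a random spirit.
; It auto-registers with a nearby BP_Combat_Manager; timelines drive scale and spin animations.
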(event OnSeePawn(PawnSensing)
  (params (Pawn :type Pawn%20Object%20Reference))
  (Utilities|Casting|CastToBP_Iso_PlayerCharacter Pawn)
  (AI|Components|Blackboard|SetValueasBool (AI|GetBlackboard (AI|GetAIController self)) (Utilities|Name|MakeLiteralName "hasSeenPlayer") true)
  (Variables|/Script/Engine.CharacterMovementComponent|SetMaxWalkSpeed (Variables|Character|GetCharacterMovement) 1e+03))

(event OnComponentBeginOverlap(hitbox)
  (params (OverlappedComponent :type Primitive%20Component%20Object%20Reference) (OtherActor :type Actor%20Object%20Reference) (OtherComp :type Primitive%20Component%20Object%20Reference) (OtherBodyIndex :type Integer) (bFromSweep :type Boolean) (SweepResult :type Hit%20Result%20Structure%20%28by%20ref%29))
  (Utilities|Casting|CastToBP_Iso_PlayerCharacter OtherActor)
  (Utilities|FlowControl|DoOnce false :!label _label
    (:Completed
      (Game|Damage|ApplyDamage OtherActor (Variables|Default|GetunitDamage) 0 0)
      (bind _scalar (Timeline|ScaleUp PlayFromStart)
        (:Update
          (Transformation|SetActorScale3D (+ (Transformation|GetActorScale3D) (Math|Vector|MakeVector _scalar _scalar _scalar))))
        (:Finished
          (Utilities|FlowControl|Delay 1.5)
          (if (Variables|Default|GetisBig)
            (Transformation|SetActorScale3D "4.000000,4.000000,4.000000")
            (else
              (Transformation|SetActorScale3D "1.300000,1.300000,1.300000")))
          (Utilities|FlowControl|Delay 1.5)
          (goto _label Reset))))))

(event Custom|CheckHealth
  (if (<= (Variables|Default|GetunitHealth) 15.0)
    _))

(event Custom|CheckEnemies
  (bind _self self)
  (bind _returnvalue (AI|GetAIController _self))
  (bind _returnvalue_2 (AI|GetBlackboard _returnvalue))
  (if (Variables|Default|GetcanCombine)
    (bind _outhits (Class|KismetSystemLibrary|BoxTraceMulti (Transformation|GetWorldLocation (Variables|Default|Getstartbox)) (Transformation|GetWorldLocation (Variables|Default|Getendbox)) "1000.000000,1000.000000,100.000000" "0, 0, 0" "TraceTypeQuery1" false 0 "None" true))
    (for _array_element _outhits
      (bind _asbp_ai_combine (Utilities|Casting|CastToBP_AI_Combine (.hitactor _array_element)))
      (if (<= (Utilities|Array|Length (Variables|Default|Gethitactors)) 3)
        (if (Variables|BP_AI_Combine_C|GetcanCombine _asbp_ai_combine)
          (Utilities|Array|Add (Variables|Default|Gethitactors) _asbp_ai_combine))))
    (if (and (>= (Utilities|Array|Length (Variables|Default|Gethitactors)) 3) (<= (Math|Random|RandomFloatinRange 0.0 1e+01) 2.0))
      (for _array_element_2 (Variables|Default|Gethitactors)
        (Variables|BP_AI_Combine_C|SetcanCombine _array_element_2 false)
        (AI|Components|Blackboard|SetValueasVector (AI|GetBlackboard (AI|GetAIController _array_element_2)) (Utilities|Name|MakeLiteralName "Combine_Location") (Transformation|GetActorLocation))
        (AI|Components|Blackboard|SetValueasBool (AI|GetBlackboard (AI|GetAIController _array_element_2)) (Utilities|Name|MakeLiteralName "canCombine") true))
      (Variables|Default|SetcanCombine false)
      (bind _returnvalue_3 (Niagara|SpawnSystematLocation "/Game/Particles/V_EnemyMagic/VFX_EnemyBullet.VFX_EnemyBullet" (Transformation|GetActorLocation) "0, 0, 0" "5.000000,5.000000,5.000000"))
      (AI|Components|Blackboard|SetValueasVector _returnvalue_2 (Utilities|Name|MakeLiteralName "Combine_Location") (Transformation|GetActorLocation))
      (AI|Components|Blackboard|SetValueasBool _returnvalue_2 (Utilities|Name|MakeLiteralName "canCombine") true)
      (Utilities|FlowControl|Delay 3.0)
      (for _array_element_3 (Variables|Default|Gethitactors)
        (Actor|DestroyActor _array_element_3))
      (bind _scale (Timeline|CombineUp Play)
        (:Update
          (Transformation|SetActorTransform (Math|Transform|MakeTransform (Transformation|GetActorLocation) (Transformation|GetActorRotation) (Math|Vector|MakeVector _scale _scale _scale))))
        (:Finished
          (Components|DestroyComponent _returnvalue_3)
          (AI|Components|Blackboard|SetValueasBool (AI|GetBlackboard (AI|GetAIController self)) (Utilities|Name|MakeLiteralName "canCombine") false)
          (Variables|Default|SetunitHealth (+ (Variables|Default|GetunitHealth) 2e+02))
          (bind _output_get (Variables|Default|SetisBig true))
          (AI|Components|Blackboard|SetValueasBool (AI|GetBlackboard (AI|GetAIController self)) (Utilities|Name|MakeLiteralName "isBig") _output_get)))
      (else
        (Utilities|Array|Clear (Variables|Default|Gethitactors))))))

(event Custom|Spinner
  (Variables|/Script/Engine.CharacterMovementComponent|SetMaxWalkSpeed (Variables|Character|GetCharacterMovement) 0.0)
  (Variables|Default|SetisAttacking true)
  (bind _rotator (Timeline|Spine_Timeline PlayFromStart)
    (:Update
      (Transformation|SetActorRotation (Math|Rotator|MakeRotator 0.0 0.0 _rotator)))
    (:Finished
      (CallFunction|Spinner))))

(event Custom|Start_Dash_Attack)

(event EventBeginPlay
  (Variables|Default|SetcanTakeDamage false)
  (Transformation|SetActorScale3D "0, 0, 0")
  (bind _newscale (Timeline|SpawnedIn PlayFromStart)
    (:Update
      (Transformation|SetActorScale3D (Math|Vector|MakeVector _newscale _newscale _newscale)))
    (:Finished
      (Utilities|FlowControl|Delay 2.0)
      (Variables|Default|SetcanTakeDamage true)
      ;[1 1 1] Get Rid of Autoassign, put into Combat Manager
      (bind _outactors (Actor|GetAllActorsOfClass "/Game/BluePrints/AI/Combat/BP_Combat_Manager.BP_Combat_Manager_C"))
      (bind _array_element (Utilities|Array|ForEachLoopwithBreak _outactors :!label _label)
        (:LoopBody
          (if (< (Math|Vector|Distance(Vector) (Transformation|GetActorLocation _array_element) (Transformation|GetActorLocation)) 6e+03)
            (Default|DeathAssigner _array_element self)
            (Utilities|Array|AddUnique (Variables|/Game/BluePrints/AI/Combat/BP_Combat_Manager.BP_Combat_Manager_C|GetEnemy_List _array_element) self)
            (goto _label Break)))))))

(event Collision|EventActorBeginOverlap
  (params (OtherActor :type Actor%20Object%20Reference)))

(event EventTick
  (params (DeltaSeconds :type Float%20%28single-precision%29))
  (Collision|BoxTraceByChannel (Transformation|GetWorldLocation (Variables|Default|Getstartbox)) (Transformation|GetWorldLocation (Variables|Default|Getendbox)) "1000.000000,1000.000000,100.000000" "0, 0, 0" "TraceTypeQuery1" false 0 "None"))

(event EventChase
  (params (AttackTarget :type Actor%20Object%20Reference))
  (Variables|/Script/Engine.CharacterMovementComponent|SetMaxWalkSpeed (Variables|Character|GetCharacterMovement) 845.0)
  (Variables|Default|SetisAttacking false)
  (Utilities|FlowControl|Sequence
    (:then_0
      (Utilities|FlowControl|DoOnce false) ; enters at Reset
    )
    (:then_1
      (bind _rotator (Timeline|Spine_Timeline Stop)
        (:Update
          (Transformation|SetActorRotation (Math|Rotator|MakeRotator 0.0 0.0 _rotator)))
        (:Finished
          (CallFunction|Spinner))))))

(event EventCelebrate
  (Utilities|FlowControl|DoOnce false
    (:Completed
      (bind _rotator (Timeline|Spine_Timeline PlayFromStart)
        (:Update
          (Transformation|SetActorRotation (Math|Rotator|MakeRotator 0.0 0.0 _rotator)))
        (:Finished
          (CallFunction|Spinner))))))

(event EventHitRegistration
  (Rendering|Material|SetScalarParameterValueonMaterials (Variables|Character|GetMesh) "health" 2e+02)
  (Utilities|FlowControl|Delay 0.2)
  (Rendering|Material|SetScalarParameterValueonMaterials (Variables|Character|GetMesh) "health" 1.0))

(event EventUnitDeath
  (bind _returnvalue (Transformation|GetActorLocation))
  (bind _returnvalue_2 (Transformation|GetActorTransform))
  (Default|CallOnDeath self)
  (Rendering|Material|SetScalarParameterValueonMaterials (Variables|Character|GetMesh) "health" 2e+02)
  (bind _scale (Timeline|scaleDown PlayFromStart)
    (:Update
      (if (<= (- (.x (.scale _returnvalue_2)) _scale) 0.0)
        (Utilities|FlowControl|Sequence :!label _label
          (:then_0
            (if (Variables|Default|GetisBig)
              (Utilities|FlowControl|DoOnce false
                (:Completed
                  (Game|SpawnActorfromClass "BP_AI_Combine_C" (Math|Transform|MakeTransform (+ (Transformation|GetActorLocation) "0.000000,100.000000,0.000000") "0, 0, 0" "1.000000,1.000000,1.000000") "AdjustIfPossibleButAlwaysSpawn" "MultiplyWithRoot" 0 0)
                  (Game|SpawnActorfromClass "BP_AI_Combine_C" (Math|Transform|MakeTransform (+ (Transformation|GetActorLocation) "100.000000,-100.000000,0.000000") "0, 0, 0" "1.000000,1.000000,1.000000") "AdjustIfPossibleButAlwaysSpawn" "MultiplyWithRoot" 0 0)))))
          (:then_1
            (Default|DestroyEventforUnitsinCombat (Variables|Default|GetAttached_Combat_Manager) self))
          (:then_2
            (if (Variables|Default|GetisBig)
              _
              (else
                (bind _returnvalue_3 (Game|SpawnActorfromClass "/Game/BluePrints/Spirits/Parent/BP_Spirit.BP_Spirit_C" (Math|Transform|MakeTransform (+ (Transformation|GetActorLocation) "0.000000,0.000000,600.000000") (Transformation|GetActorRotation) "1.000000,1.000000,1.000000") "Undefined" "MultiplyWithRoot" 0 0))
                (bind _output_get (Variables|/Game/BluePrints/Spirits/Parent/BP_Spirit.BP_Spirit_C|SetName_Of_Spirit _returnvalue_3 (.OutItem (Utilities|Array|Random (Variables|Default|GetspiritNames)))))
                (Default|UpdateMesh _returnvalue_3 _output_get)))
            (|CallParentFunction)))
        (else
          (Transformation|SetActorTransform (Math|Transform|MakeTransform (.location _returnvalue_2) (.rotation _returnvalue_2) (Math|Vector|MakeVector (- (.x (.scale _returnvalue_2)) _scale) (- (.x (.scale _returnvalue_2)) _scale) (- (.x (.scale _returnvalue_2)) _scale)))))))
    (:Finished
      (Niagara|SpawnSystematLocation "/Game/Particles/V_Dash/V_SS_Wind.V_SS_Wind" (Math|Vector|MakeVector (.x _returnvalue) (.y _returnvalue) (+ (.z _returnvalue) 1e+02)))
      (Audio|PlaySoundatLocation "/Game/Audio/AudioClips/SFX/enemyPopsound.enemyPopsound" (Transformation|GetActorLocation) "0, 0, 0" 0.5 1.0 0.0 "/Game/Audio/EnemyAtten.EnemyAtten" 0 0 0)
      (goto _label))))

(event EventSetCanAttack
  (params (CanAttack :type Boolean))
  (Variables|Default|SetcanAttackSpirits CanAttack))

(event EventTargetPlayer
  (AI|Components|Blackboard|SetValueasBool (AI|GetBlackboard (AI|GetAIController self)) (Utilities|Name|MakeLiteralName "killPlayer") true))

(fn ConstructionScript
  (bind _outactors (Actor|GetAllActorsOfClass "/Game/BluePrints/AI/Combat/BP_Combat_Manager.BP_Combat_Manager_C"))
  (bind _asbp_combat_manager (Utilities|Casting|CastToBP_Combat_Manager (.ReturnValue (Actor|FindNearestActor (Transformation|GetActorLocation) _outactors))))
  (Default|DeathAssigner _asbp_combat_manager self)
  (Utilities|Array|AddUnique (Variables|/Game/BluePrints/AI/Combat/BP_Combat_Manager.BP_Combat_Manager_C|GetEnemy_List _asbp_combat_manager) self))

(fn DetermineAttackLocation
  (params (Defending_Actor :type Actor%20Object%20Reference) (Attack_Direction :type Integer) (Attack_Radius%20 :type Float%20%28double-precision%29))
  (LocalVariables|SetTemp_Location (Transformation|GetActorLocation Defending_Actor))
  (switch int Attack_Direction
    (:Default
      (LocalVariables|SetTemp_Location (* (Transformation|GetActorForwardVector Defending_Actor) Attack_Radius%20) :!label _label))
    (:0
      (goto _label))
    (:1
      (LocalVariables|SetTemp_Location (* (Transformation|GetActorRightVector Defending_Actor) Attack_Radius%20)))
    (:2
      (LocalVariables|SetTemp_Location (* (Transformation|GetActorForwardVector Defending_Actor) Attack_Radius%20 -1.0)))
    (:3
      (LocalVariables|SetTemp_Location (* (Transformation|GetActorRightVector Defending_Actor) Attack_Radius%20 -1.0))))
  (bind _randomlocation (Class|NavigationSystemV1|GetRandomLocationinNavigableRadius (LocalVariables|GetTemp_Location) Attack_Radius%20 0 0))
  (return _randomlocation))