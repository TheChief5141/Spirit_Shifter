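; BP_ChiliTurret is an enemy turret that fires BP_EnemyProjectile with random yaw spread.
; On spawn it registers with a BP_Combat_Manager within 6000 units and starts a self-recalling fire loop gated by CanShoot.
; Pawn sensing eases its rotation toward the player and enables shooting.
; Damage briefly flashes a material parameter, and death plays a scale-down and wind effect before calling the parent's UnitDeath.
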(event OnSeePawn(PawnSensing)
  (params (Pawn :type Pawn%20Object%20Reference))
  (Utilities|Casting|CastToBP_Iso_PlayerCharacter Pawn)
  (Transformation|SetActorRotation (Math|Rotator|Lerp(Rotator) (Math|Rotator|FindLookatRotation (Transformation|GetActorLocation) (Transformation|GetActorLocation Pawn)) (Transformation|GetActorRotation) 0.125))
  (Variables|Default|SetCanShoot true)
  (Utilities|FlowControl|DoOnce false
    (:Completed
      (CallFunction|FireProj))))

(event Custom|CheckHealth
  (if (<= (Variables|/Game/BluePrints/AI/AC_EnemyHealth.AC_EnemyHealth_C|Gethealth (Variables|Default|GetAC_EnemyHealth)) 0.0)
    (Audio|PlaySoundatLocation "/Game/Audio/AudioClips/SFX/Monster-2.Monster-2" (Transformation|GetActorLocation) "0, 0, 0" 1.0 1.0 0.0 "/Game/Audio/EnemyAtten.EnemyAtten" 0 0 0)
    (Actor|DestroyActor)))

(event Custom|FireProj
  (bind _arrow (Variables|Default|GetArrow))
  (bind _returnvalue (Transformation|GetWorldTransform _arrow))
  (if (Variables|Default|GetCanShoot)
    (if (Class|Actor|WasRecentlyRendered 2.0)
      (Audio|PlaySoundatLocation "/Game/Audio/AudioClips/SFX/projectileshoot.projectileshoot" (Transformation|GetWorldLocation (Variables|Default|GetStaticMesh)) "0, 0, 0" 1.0 1.0 0.0 "/Game/Audio/EnemyAtten.EnemyAtten" 0 0 0))
    (Animation|PlayAnimMontage "/Game/Animations/BanChili-Anims/BC_Attack_Anim_Montage.BC_Attack_Anim_Montage" 1.0 "None")
    (Game|SpawnActorfromClass "/Game/BluePrints/AI/BP_EnemyProjectile.BP_EnemyProjectile_C" (Math|Transform|MakeTransform (.location _returnvalue) (Math|Rotator|MakeRotator (.roll (.rotation _returnvalue)) (.pitch (.rotation _returnvalue)) (+ (.yaw (.rotation _returnvalue)) (Math|Random|RandomFloatinRange -15.0 15.0))) "2.000000,2.000000,2.000000") "AlwaysSpawn" "MultiplyWithRoot" 0 0)
    (Utilities|FlowControl|Delay (Variables|Default|GetfireRate))
    (CallFunction|FireProj)
    (else
      (Utilities|FlowControl|Delay 1.0)
      (Variables|Default|SetCanShoot false)
      (CallFunction|FireProj)
      (Utilities|FlowControl|DoOnce false) ; enters at Reset
    )))

(event EventBeginPlay
  (CallFunction|FireProj)
  (bind _outactors (Actor|GetAllActorsOfClass "/Game/BluePrints/AI/Combat/BP_Combat_Manager.BP_Combat_Manager_C"))
  (bind _array_element (Utilities|Array|ForEachLoopwithBreak _outactors :!label _label)
    (:LoopBody
      (if (< (Math|Vector|Distance(Vector) (Transformation|GetActorLocation _array_element) (Transformation|GetActorLocation)) 6e+03)
        (bind _asbp_combat_manager (Utilities|Casting|CastToBP_Combat_Manager _array_element))
        (Default|DeathAssigner _asbp_combat_manager self)
        (Utilities|Array|AddUnique (Variables|/Game/BluePrints/AI/Combat/BP_Combat_Manager.BP_Combat_Manager_C|GetEnemy_List _asbp_combat_manager) self)
        (goto _label Break)))))

(event Collision|EventActorBeginOverlap
  (params (OtherActor :type Actor%20Object%20Reference)))

(event EventTick
  (params (DeltaSeconds :type Float%20%28single-precision%29)))

(event EventUnitDeath
  (Utilities|FlowControl|DoOnce false
    (:Completed
      (bind _scale (Timeline|ScaleDown PlayFromStart)
        (:Update
          (Transformation|SetActorScale3D (Math|Vector|MakeVector _scale _scale _scale)))
        (:Finished
          (Components|DestroyComponent (Variables|Character|GetMesh))
          (Variables|Default|SetCanShoot false)
          (Niagara|SpawnSystematLocation "/Game/Particles/V_Dash/V_SS_Wind.V_SS_Wind" (Transformation|GetActorLocation))
          (Utilities|FlowControl|Delay 1.5)
          (|CallParentFunction))))))

(event EventAnyDamage
  (params (Damage :type Float%20%28single-precision%29) (DamageType :type Damage%20Type%20Object%20Reference) (InstigatedBy :type Controller%20Object%20Reference) (DamageCauser :type Actor%20Object%20Reference))
  (|CallParentFunction Damage DamageType InstigatedBy DamageCauser)
  (Rendering|Material|SetScalarParameterValueonMaterials (Variables|Character|GetMesh) "health" 2e+02)
  (Utilities|FlowControl|Delay 0.2)
  (Rendering|Material|SetScalarParameterValueonMaterials (Variables|Character|GetMesh) "health" 1.0))

(fn ConstructionScript)

(fn RandomizeSpread)