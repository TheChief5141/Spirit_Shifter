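; BP_WaterBossTurret is a water boss turret that spins by a yaw offset each tick, or turns to face the player when SeenPlayer is true.
; Tick handles both rotations, using a look-at yaw toward player 0's character for tracking.
; PawnSensing's see event only prints a debug "Hello"; the player cast that would set SeenPlayer is disconnected, so nothing here switches it to tracking.
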(event OnSeePawn(PawnSensing)
  (params (Pawn :type Pawn%20Object%20Reference))
  (Development|PrintString "Hello"))

(event EventBeginPlay)

(event Collision|EventActorBeginOverlap
  (params (OtherActor :type Actor%20Object%20Reference)))

(event EventTick
  (params (DeltaSeconds :type Float%20%28single-precision%29))
  (if (Variables|Default|GetseenPlayer)
    (Transformation|SetActorRotation (Math|Rotator|MakeRotator 0.0 0.0 (.yaw (Math|Rotator|FindLookatRotation (Transformation|GetActorLocation) (Transformation|GetActorLocation (Game|GetPlayerCharacter 0))))))
    (else
      (Transformation|AddActorLocalRotation (Math|Rotator|MakeRotator 0.0 0.0 (Variables|Default|GetrandomRotateVal)) false false))))

(fn ConstructionScript)