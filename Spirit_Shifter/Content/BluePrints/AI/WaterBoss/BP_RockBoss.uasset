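; BP_RockBoss is a rock hazard in the water boss AI set that deals damage when its box overlaps the isometric player character.
; When HasLifeSpawn is set, BeginPlay gives it a short lifespan, picks random per-axis spin values and has the box ignore the owner while moving.
; The mesh rotation logic that would use those spin values is disconnected, and Tick is empty.
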(event OnComponentBeginOverlap(Box)
  (params (OverlappedComponent :type Primitive%20Component%20Object%20Reference) (OtherActor :type Actor%20Object%20Reference) (OtherComp :type Primitive%20Component%20Object%20Reference) (OtherBodyIndex :type Integer) (bFromSweep :type Boolean) (SweepResult :type Hit%20Result%20Structure%20%28by%20ref%29))
  (Utilities|Casting|CastToBP_Iso_PlayerCharacter OtherActor)
  (Game|Damage|ApplyDamage OtherActor 1e+01 0 0))

(event EventBeginPlay
  (bind _returnvalue (Components|GetOwner))
  (if (Variables|Default|GethasLifeSpawn)
    (Actor|SetLifeSpan 2.0)
    (Variables|Default|SetxRot (Math|Random|RandomFloatinRange -4.0 4.0))
    (Variables|Default|SetyRot (Math|Random|RandomFloatinRange -2.0 2.0))
    (Variables|Default|SetzRot (Math|Random|RandomFloatinRange -4.0 4.0))
    (Collision|IgnoreActorwhenMoving (Variables|Default|GetBox) _returnvalue true)
    (Collision|IgnoreActorwhenMoving (Variables|Default|GetBox) _returnvalue true)))

(event Collision|EventActorBeginOverlap
  (params (OtherActor :type Actor%20Object%20Reference)))

(event EventTick
  (params (DeltaSeconds :type Float%20%28single-precision%29)))

(fn ConstructionScript)