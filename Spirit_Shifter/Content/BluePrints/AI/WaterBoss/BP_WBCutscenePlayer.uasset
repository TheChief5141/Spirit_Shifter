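; BP_WBCutscenePlayer is a trigger volume in the Water Boss folder that plays a level sequence when the player enters its box.
; On overlap it disables player input, binds the player character to the sequence's "Player" tag and starts playback.
; When the sequence finishes, it restores input and destroys itself.
; A loop to destroy ActorsToDestroy exists but is disconnected and never runs.
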(event OnComponentBeginOverlap(Box)
  (params (OverlappedComponent :type Primitive%20Component%20Object%20Reference) (OtherActor :type Actor%20Object%20Reference) (OtherComp :type Primitive%20Component%20Object%20Reference) (OtherBodyIndex :type Integer) (bFromSweep :type Boolean) (SweepResult :type Hit%20Result%20Structure%20%28by%20ref%29))
  (bind _returnvalue (Game|GetPlayerCharacter 0))
  (bind _sequencetoplay (Variables|Default|GetSequenceToPlay))
  (bind _sequenceplayer (Variables|/Script/LevelSequence.LevelSequenceActor|GetSequencePlayer _sequencetoplay))
  (if (== OtherActor _returnvalue)
    (Input|DisableInput (Game|GetPlayerController 0) 0)
    (EventDispatchers|AssignOnFinished _sequenceplayer (delegate Custom|OnFinished_Event))
    (Class|LevelSequenceActor|SetBindingbyTag _sequencetoplay "Player" (Utilities|Array|MakeArray _returnvalue) false)
    (Sequencer|Player|Play _sequenceplayer :!class /Script/MovieScene.MovieSceneSequencePlayer)))

(event Custom|OnFinished_Event
  (Input|EnableInput (Game|GetPlayerController 0) 0)
  (Actor|DestroyActor))

(fn ConstructionScript)