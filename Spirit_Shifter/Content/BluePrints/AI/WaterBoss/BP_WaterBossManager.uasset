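; BP_WaterBossManager is a trigger actor that starts the water boss fight when the isometric player character enters its Box.
; On overlap it runs BT_WaterBoss on the boss's AI controller, waits a tick, then sets the canAttack blackboard key.
; It then calls the boss's fight intro, next-attack selection and health bar start, with no guard against re-triggering.
; BeginPlay caches the Chair's world location, which this graph never reads.
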(event OnComponentBeginOverlap(Box)
  (params (OverlappedComponent :type Primitive%20Component%20Object%20Reference) (OtherActor :type Actor%20Object%20Reference) (OtherComp :type Primitive%20Component%20Object%20Reference) (OtherBodyIndex :type Integer) (bFromSweep :type Boolean) (SweepResult :type Hit%20Result%20Structure%20%28by%20ref%29))
  (Utilities|Casting|CastToBP_Iso_PlayerCharacter OtherActor)
  (bind _returnvalue (Actor|GetActorOfClass "/Game/BluePrints/AI/WaterBoss/BP_WaterBoss.BP_WaterBoss_C"))
  (AI|RunBehaviorTree (AI|GetAIController _returnvalue) "/Game/BluePrints/AI/WaterBoss/BT_WaterBoss.BT_WaterBoss")
  (Utilities|FlowControl|DelayUntilNextTick)
  (AI|Components|Blackboard|SetValueasBool (AI|GetBlackboard (AI|GetAIController _returnvalue)) (Utilities|Name|MakeLiteralName "canAttack") true)
  (Default|BeginningOfFight _returnvalue)
  (Default|DetermineNextAttack _returnvalue)
  (Default|StartHealthBar _returnvalue))

(event EventBeginPlay
  (Variables|Default|SetchairWorldLoc (Transformation|GetWorldLocation (Variables|Default|Getchair))))

(event Collision|EventActorBeginOverlap
  (params (OtherActor :type Actor%20Object%20Reference)))

(event EventTick
  (params (DeltaSeconds :type Float%20%28single-precision%29)))

(fn ConstructionScript)