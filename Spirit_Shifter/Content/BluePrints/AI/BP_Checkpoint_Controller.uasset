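; AI controller that flings its possessed Character toward the player whenever AI perception reports an update for them.
; It solves a high-arc projectile toss to the player's location, keeps only the direction and scales it by LaunchStrength to overwrite the movement component's velocity.
; The update's sensed or lost state is not checked, and a debug string prints on each launch.
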(event OnTargetPerceptionUpdated(AIPerception)
  (params (Actor :type Actor%20Object%20Reference) (Stimulus :type AI%20Stimulus%20Structure))
  (bind _returnvalue (Game|GetPlayerCharacter 0))
  (bind _returnvalue_2 (Pawn|GetControlledPawn))
  (if (== Actor _returnvalue)
    (bind _tossvelocity (Class|GameplayStatics|BlueprintSuggestProjectileVelocity (Transformation|GetActorLocation _returnvalue_2) (Transformation|GetActorLocation _returnvalue) 1e+03 0.0 "DoNotTrace" 2.0 true false))
    (bind _ascharacter (Utilities|Casting|CastToCharacter _returnvalue_2))
    (Variables|/Script/Engine.MovementComponent|SetVelocity (Variables|/Script/Engine.Character|GetCharacterMovement _ascharacter) (* (Math|Vector|Normalize _tossvelocity) (Variables|Default|GetLaunch_Strength)))
    (Development|PrintString "see player")))

(event EventBeginPlay
  (|CallParentFunction) ; This node is disabled and will not be called.\nDrag off pins to build functionality.
)

(event EventTick
  (params (DeltaSeconds :type Float%20%28single-precision%29)))

(fn ConstructionScript
  (|CallParentFunction))