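; Rogue enemy that steals the player's current spirit when the player stays near it.
; Entering the Spiritstealer volume caches that spirit and disables its collision, and Tick pins it to SpiritLoc from then on.
; If the player is inside after a short delay, it removes the player's spirit.
; If the cached spirit remains valid, it gives the player a Winged Spirit and sets the hasSpirit blackboard key.
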(event OnComponentBeginOverlap(spiritstealer)
  (params (OverlappedComponent :type Primitive%20Component%20Object%20Reference) (OtherActor :type Actor%20Object%20Reference) (OtherComp :type Primitive%20Component%20Object%20Reference) (OtherBodyIndex :type Integer) (bFromSweep :type Boolean) (SweepResult :type Hit%20Result%20Structure%20%28by%20ref%29))
  (bind _asbp_iso_player_character (Utilities|Casting|CastToBP_Iso_PlayerCharacter OtherActor))
  (Variables|Default|SetplayerInBounds true)
  (bind _output_get (Variables|Default|SetmySpirit (Variables|/Game/BluePrints/Player/BP_Iso_PlayerCharacter.BP_Iso_PlayerCharacter_C|GetCurrent_Spirit _asbp_iso_player_character)))
  (Collision|SetCollisionEnabled (Variables|/Script/Engine.Character|GetMesh _output_get) "NoCollision")
  (Collision|SetCollisionResponsetoAllChannels (Variables|/Script/Engine.Character|GetMesh _output_get) "ECR_Ignore")
  (Utilities|FlowControl|Delay 3.0)
  (if (Variables|Default|GetplayerInBounds)
    (Default|RemoveSpirit _asbp_iso_player_character)
    (Utilities|IsValid _output_get
      (:Is%20Valid
        (Default|AddSpirit _asbp_iso_player_character "/Game/BluePrints/Spirits/Winged_Snake/AC_Winged_Spirit.AC_Winged_Spirit_C")
        (AI|Components|Blackboard|SetValueasBool (AI|GetBlackboard (AI|GetAIController self)) (Utilities|Name|MakeLiteralName "hasSpirit") true)))))

(event OnComponentEndOverlap(spiritstealer)
  (params (OverlappedComponent :type Primitive%20Component%20Object%20Reference) (OtherActor :type Actor%20Object%20Reference) (OtherComp :type Primitive%20Component%20Object%20Reference) (OtherBodyIndex :type Integer))
  (Utilities|Casting|CastToBP_Iso_PlayerCharacter OtherActor)
  (Variables|Default|SetplayerInBounds false))

(event EventBeginPlay
  (|CallParentFunction) ; This node is disabled and will not be called.\nDrag off pins to build functionality.
)

(event Collision|EventActorBeginOverlap
  (params (OtherActor :type Actor%20Object%20Reference))
  (|CallParentFunction OtherActor) ; This node is disabled and will not be called.\nDrag off pins to build functionality.
)

(event EventTick
  (params (DeltaSeconds :type Float%20%28single-precision%29))
  (bind _myspirit (Variables|Default|GetmySpirit))
  (|CallParentFunction DeltaSeconds)
  (Utilities|IsValid _myspirit
    (:Is%20Valid
      (Transformation|SetActorLocation _myspirit (Transformation|GetWorldLocation (Variables|Default|Getspirit%20loc)) false false))))

(fn ConstructionScript
  (|CallParentFunction))