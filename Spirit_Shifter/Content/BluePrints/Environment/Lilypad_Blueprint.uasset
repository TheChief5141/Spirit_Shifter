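; Lilypad environment actor that starts with its main mesh hidden and can double as a jump pad for the player.
; ToggleState shows or hides that mesh; switching on also forwards the state to a linked actor through BPI_States after a short delay.
; When IsJumpingPlatform is set, Box overlap launches the player with vertical velocity scaled by JumpPower.
; Otherwise, the construction script hides the secondary StaticMesh and disables its collision.
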(event OnComponentBeginOverlap(StaticMeshComponent)
  (params (OverlappedComponent :type Primitive%20Component%20Object%20Reference) (OtherActor :type Actor%20Object%20Reference) (OtherComp :type Primitive%20Component%20Object%20Reference) (OtherBodyIndex :type Integer) (bFromSweep :type Boolean) (SweepResult :type Hit%20Result%20Structure%20%28by%20ref%29)))

(event OnComponentEndOverlap(StaticMeshComponent)
  (params (OverlappedComponent :type Primitive%20Component%20Object%20Reference) (OtherActor :type Actor%20Object%20Reference) (OtherComp :type Primitive%20Component%20Object%20Reference) (OtherBodyIndex :type Integer)))

(event OnComponentBeginOverlap(Box)
  (params (OverlappedComponent :type Primitive%20Component%20Object%20Reference) (OtherActor :type Actor%20Object%20Reference) (OtherComp :type Primitive%20Component%20Object%20Reference) (OtherBodyIndex :type Integer) (bFromSweep :type Boolean) (SweepResult :type Hit%20Result%20Structure%20%28by%20ref%29))
  (if (and (Utilities|ClassIsChildOf (Utilities|GetClass OtherActor) "/Game/BluePrints/Player/BP_Iso_PlayerCharacter.BP_Iso_PlayerCharacter_C") (Variables|Default|GetisJumpingPlatform))
    (bind _asbp_iso_player_character (Utilities|Casting|CastToBP_Iso_PlayerCharacter OtherActor))
    (Pawn|Components|CharacterMovement|SetMovementMode (Variables|/Script/Engine.Character|GetCharacterMovement _asbp_iso_player_character) "MOVE_Falling" 0)
    (bind _output_get (Variables|/Script/Engine.MovementComponent|SetVelocity (Variables|/Script/Engine.Character|GetCharacterMovement _asbp_iso_player_character) (Math|Vector|MakeVector (.X (Class|KismetMathLibrary|BreakVector3f (Variables|/Script/Engine.MovementComponent|GetVelocity (Variables|/Script/Engine.Character|GetCharacterMovement _asbp_iso_player_character)))) (.Y (Class|KismetMathLibrary|BreakVector3f (Variables|/Script/Engine.MovementComponent|GetVelocity (Variables|/Script/Engine.Character|GetCharacterMovement _asbp_iso_player_character)))) (* (.Z (Class|KismetMathLibrary|BreakVector3f (Variables|/Script/Engine.MovementComponent|GetVelocity (Variables|/Script/Engine.Character|GetCharacterMovement _asbp_iso_player_character)))) (Variables|Default|GetJump_Power)))))
    (Character|LaunchCharacter _asbp_iso_player_character _output_get true true)))

(event EventBeginPlay
  (CallFunction|ToggleState false))

(event Collision|EventActorBeginOverlap
  (params (OtherActor :type Actor%20Object%20Reference)))

(event EventTick
  (params (DeltaSeconds :type Float%20%28single-precision%29)))

(event EventToggleState
  (params (On/Off :type Boolean))
  (bind _affected_actor (Variables|Default|GetAffected_Actor))
  (if On/Off
    (Rendering|SetVisibility (Variables|Debug|GetStaticMeshComponent) true true)
    (if (and (Utilities|IsValid _affected_actor) (Utilities|DoesObjectImplementInterface _affected_actor "/Game/BluePrints/Interfaces/BPI_States.BPI_States_C"))
      (Utilities|FlowControl|Delay 0.6)
      (Class|BPIStates|ToggleState(Message) _affected_actor true))
    (else
      (Rendering|SetVisibility (Variables|Debug|GetStaticMeshComponent) false false))))

(fn ConstructionScript
  (bind _staticmesh (Variables|Default|GetStaticMesh))
  (if (not (Variables|Default|GetisJumpingPlatform))
    (Rendering|SetVisibility _staticmesh false false)
    (Collision|SetCollisionEnabled _staticmesh "NoCollision")))