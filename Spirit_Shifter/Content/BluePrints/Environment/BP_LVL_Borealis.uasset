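; BP_LVL_Borealis is an environment actor that moves its Wall component between two marker points, FirstPoint and SecondPoint.
; WallMover plays the MoveWall timeline, which eases the wall toward the current target with VInterpTo, at a speed from its Interpspeed track times Multiplier.
; When the timeline finishes, it flips First and NewTarget selects the other point for the next run.
; Nothing in this Blueprint calls WallMover.
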(event Custom|WallMover
  (bind _interpspeed (Timeline|MoveWall PlayFromStart)
    (:Update
      (Transformation|SetWorldLocation (Variables|Default|Getwall) (Math|Interpolation|VInterpTo (Transformation|GetWorldLocation (Variables|Default|Getwall)) (Variables|Default|GettargetLoc) (Utilities|Time|GetWorldDeltaSeconds) (* _interpspeed (Variables|Default|Getmultiplier))) false false))
    (:Finished
      (Variables|Default|Setfirst (not (Variables|Default|Getfirst)))
      (CallFunction|NewTarget))))

(event Custom|NewTarget
  (if (Variables|Default|Getfirst)
    (Variables|Default|SettargetLoc (Transformation|GetWorldLocation (Variables|Default|Getfirst%20point)))
    (else
      (Variables|Default|SettargetLoc (Transformation|GetWorldLocation (Variables|Default|Getsecond%20point))))))

(event EventBeginPlay
  (CallFunction|NewTarget))

(event Collision|EventActorBeginOverlap
  (params (OtherActor :type Actor%20Object%20Reference)))

(event EventTick
  (params (DeltaSeconds :type Float%20%28single-precision%29)))

(fn ConstructionScript)