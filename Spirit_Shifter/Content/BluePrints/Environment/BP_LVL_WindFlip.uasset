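; Level wind volume that pushes the player along its arrow's direction and can flip its angle.
; While the player overlaps it, a looping timer repeatedly adds arrow-forward velocity scaled by WindStrength, with AffectZ gating the vertical component.
; Rotate_The_Wind alternates a timeline forward and in reverse to pitch WindTunnel by RotateStrength, leaving its ActorToRotate input unused.
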(event Custom|Force_Event
  (bind _returnvalue (Game|GetPlayerCharacter 0))
  (bind _wind_strength (Variables|Default|GetWind_Strength))
  (bind _arrow (Variables|Default|GetArrow))
  (bind _returnvalue_2 (Math|Vector|GetForwardVector _arrow))
  (bind _charactermovement (Variables|/Script/Engine.Character|GetCharacterMovement _returnvalue))
  (bind _returnvalue_3 (* _returnvalue_2 _wind_strength))
  (bind (_x _y _z) (Class|KismetMathLibrary|BreakVector3f _returnvalue_3))
  (Variables|/Script/Engine.MovementComponent|SetVelocity _charactermovement (+ (Variables|/Script/Engine.MovementComponent|GetVelocity _charactermovement) (Math|Vector|MakeVector _x _y (Math|Float|SelectFloat _z 0.0 (Variables|Default|GetAffect_Z))))))

(event Custom|Rotate_The_Wind
  (params (Actor_to_Rotate :type Actor%20Object%20Reference))
  (Utilities|FlowControl|FlipFlop
    (:A
      (Development|PrintString "moving wind")
      (bind _newtrack_0 (Timeline|Timeline Play)
        (:Update
          (Transformation|SetRelativeRotation (Variables|Default|GetWind_Tunnel) (Math|Rotator|MakeRotator 0.0 (* _newtrack_0 (Variables|Default|GetRotate_Strength)) 0.0) false false))))
    (:B
      (Development|PrintString "reverse wind")
      (Timeline|Timeline ReverseFromEnd))))

(event EventBeginPlay)

(event Collision|EventActorBeginOverlap
  (params (OtherActor :type Actor%20Object%20Reference))
  (if (== OtherActor (Game|GetPlayerCharacter 0))
    (bind _returnvalue (Utilities|Time|SetTimerbyEvent (EventDispatchers|CreateEvent :!event Custom|Force_Event) 0.1 true))
    (Variables|Default|SetForce_Timer _returnvalue)
    (Development|PrintString "here")))

(event EventTick
  (params (DeltaSeconds :type Float%20%28single-precision%29)))

(event Collision|EventActorEndOverlap
  (params (OtherActor :type Actor%20Object%20Reference))
  (if (and (== OtherActor (Game|GetPlayerCharacter 0)) (Utilities|Time|IsTimerActivebyHandle (Variables|Default|GetForce_Timer)))
    (Utilities|Time|ClearandInvalidateTimerbyHandle (Variables|Default|GetForce_Timer))))

(fn ConstructionScript)