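; Environment actor for fallen columns that moves and rotates between its placed transform and a target when toggled.
; The construction script caches the original location and rotation.
; ToggleState plays a timeline from the start when on and reverses it when off, with its alpha driving location and rotation lerps.
; The target location is an offset from the original, while the target rotation is absolute.
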(event EventBeginPlay)

(event Collision|EventActorBeginOverlap
  (params (OtherActor :type Actor%20Object%20Reference)))

(event EventTick
  (params (DeltaSeconds :type Float%20%28single-precision%29)))

(event EventToggleState
  (params (On/Off :type Boolean))
  (bind _original_location (Variables|Default|GetOriginal_Location))
  (if On/Off
    (bind _alpha (Timeline|Movement_Timeline PlayFromStart)
      (:Update
        (Transformation|SetActorLocationAndRotation (Math|Vector|Lerp(Vector) _original_location (+ _original_location (Variables|Default|GetTarget_Location)) _alpha) (Math|Rotator|Lerp(Rotator) (Variables|Default|GetOriginal_Rotation) (Variables|Default|GetTarget_Rotation) _alpha))))
    (else
      (Timeline|Movement_Timeline Reverse))))

(fn ConstructionScript
  (Variables|Default|SetOriginal_Location (Transformation|GetActorLocation))
  (Variables|Default|SetOriginal_Rotation (Transformation|GetActorRotation)))