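; BP_Prompt is an environment actor that tracks whether the isometric player character is close enough to interact with it.
; Box overlap begin and end events check for BP_Iso_PlayerCharacter or its subclasses, then call CanInteract or StopInteract to set or clear the IsInteractable flag.
; RunInteract is an empty event, so this graph defines no interaction behavior or visible prompt.
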(event OnComponentBeginOverlap(Box)
  (params (OverlappedComponent :type Primitive%20Component%20Object%20Reference) (OtherActor :type Actor%20Object%20Reference) (OtherComp :type Primitive%20Component%20Object%20Reference) (OtherBodyIndex :type Integer) (bFromSweep :type Boolean) (SweepResult :type Hit%20Result%20Structure%20%28by%20ref%29))
  (if (Utilities|ClassIsChildOf (Utilities|GetClass OtherActor) "/Game/BluePrints/Player/BP_Iso_PlayerCharacter.BP_Iso_PlayerCharacter_C")
    (CallFunction|CanInteract)))

(event OnComponentEndOverlap(Box)
  (params (OverlappedComponent :type Primitive%20Component%20Object%20Reference) (OtherActor :type Actor%20Object%20Reference) (OtherComp :type Primitive%20Component%20Object%20Reference) (OtherBodyIndex :type Integer))
  (if (Utilities|ClassIsChildOf (Utilities|GetClass OtherActor) "/Game/BluePrints/Player/BP_Iso_PlayerCharacter.BP_Iso_PlayerCharacter_C")
    (CallFunction|StopInteract)))

(event EventBeginPlay)

(event Collision|EventActorBeginOverlap
  (params (OtherActor :type Actor%20Object%20Reference)))

(event EventTick
  (params (DeltaSeconds :type Float%20%28single-precision%29)))

(event EventCanInteract
  (Variables|Default|SetIsInteractable true))

(event EventStopInteract
  (Variables|Default|SetIsInteractable false))

(event EventRunInteract)

(fn ConstructionScript)