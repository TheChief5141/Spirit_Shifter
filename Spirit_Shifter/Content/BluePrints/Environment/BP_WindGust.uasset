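; BP_WindGust is a wind gust that launches the isometric player character upward.
; Entering its Trigger caches the character and plays the Mover timeline, whose Force track feeds LaunchCharacter's Z velocity on every update.
; Leaving only clears IsHovering, which the graph never reads, and does not stop the timeline.
; MoveWind, called on BeginPlay, is empty; an older looping plane movement with sound and collision toggling is disconnected.
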(event OnComponentBeginOverlap(trigger)
  (params (OverlappedComponent :type Primitive%20Component%20Object%20Reference) (OtherActor :type Actor%20Object%20Reference) (OtherComp :type Primitive%20Component%20Object%20Reference) (OtherBodyIndex :type Integer) (bFromSweep :type Boolean) (SweepResult :type Hit%20Result%20Structure%20%28by%20ref%29))
  (bind _asbp_iso_player_character (Utilities|Casting|CastToBP_Iso_PlayerCharacter OtherActor))
  (Variables|Default|SetMyChar _asbp_iso_player_character)
  (Variables|Default|SetisHovering true)
  (CallFunction|MoveActor))

(event OnComponentEndOverlap(trigger)
  (params (OverlappedComponent :type Primitive%20Component%20Object%20Reference) (OtherActor :type Actor%20Object%20Reference) (OtherComp :type Primitive%20Component%20Object%20Reference) (OtherBodyIndex :type Integer))
  (Variables|Default|SetisHovering false))

(event Custom|MoveWind)

(event Custom|MoveActor
  (bind _force (Timeline|Mover PlayFromStart)
    (:Update
      (Character|LaunchCharacter (Variables|Default|GetMyChar) (Math|Vector|MakeVector 0.0 0.0 _force) false false))))

(event EventBeginPlay
  (CallFunction|MoveWind))

(event Collision|EventActorBeginOverlap
  (params (OtherActor :type Actor%20Object%20Reference)))

(event EventTick
  (params (DeltaSeconds :type Float%20%28single-precision%29)))

(fn ConstructionScript)