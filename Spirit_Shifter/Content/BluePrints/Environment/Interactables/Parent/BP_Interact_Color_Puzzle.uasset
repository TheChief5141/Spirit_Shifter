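; BP_Interact_Color_Puzzle is an interactable puzzle object that cycles its color state from Wind to Light to Time and back on each interaction.
; RunInteract calls RunInteractForColor, which passes the next state to ChangeColor and stores the result in Color.
; ChangeColor sets the static mesh's "Base Colour" material parameter, and the construction script uses it to show the initial Color.
; CanInteract, StopInteract and the tether events are empty.
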(event EventBeginPlay
  (|CallParentFunction) ; This node is disabled and will not be called.\nDrag off pins to build functionality.
)

(event Collision|EventActorBeginOverlap
  (params (OtherActor :type Actor%20Object%20Reference))
  (|CallParentFunction OtherActor) ; This node is disabled and will not be called.\nDrag off pins to build functionality.
)

(event EventTick
  (params (DeltaSeconds :type Float%20%28single-precision%29))
  (|CallParentFunction DeltaSeconds) ; This node is disabled and will not be called.\nDrag off pins to build functionality.
)

(event EventEndTether)

(event EventOnTether)

(event EventStopInteract)

(event EventRunInteract
  (CallFunction|RunInteractforColor (Variables|Default|GetColor)))

(event EventCanInteract)

(fn ConstructionScript
  (|CallParentFunction)
  (CallFunction|ChangeColor (Variables|Default|GetColor)))

(fn ChangeColor
  (params (Color%20to%20Change :type E_Level%20Enum :default "NewEnumerator0"))
  (bind _staticmesh (Variables|Default|GetStaticMesh))
  (switch Utilities|FlowControl|Switch|SwitchonE_Level Color%20to%20Change
    (:NewEnumerator0
      (Rendering|Material|SetVectorParameterValueonMaterials _staticmesh "Base Colour" (Variables|Default|GetWind_Color))
      (return "NewEnumerator0"))
    (:NewEnumerator1
      (Rendering|Material|SetVectorParameterValueonMaterials _staticmesh "Base Colour" (Variables|Default|GetLight_Color))
      (return "NewEnumerator1"))
    (:NewEnumerator2
      (Rendering|Material|SetVectorParameterValueonMaterials _staticmesh "Base Colour" (Variables|Default|GetTime_Color))
      (return "NewEnumerator2"))))

(fn RunInteractforColor
  (params (Selection :type E_Level%20Enum :default "NewEnumerator0"))
  (switch Utilities|FlowControl|Switch|SwitchonE_Level Selection
    (:NewEnumerator0
      (bind _current_color (CallFunction|ChangeColor "NewEnumerator1"))
      (Variables|Default|SetColor _current_color))
    (:NewEnumerator1
      (bind _current_color_2 (CallFunction|ChangeColor "NewEnumerator2"))
      (Variables|Default|SetColor _current_color_2))
    (:NewEnumerator2
      (bind _current_color_3 (CallFunction|ChangeColor "NewEnumerator0"))
      (Variables|Default|SetColor _current_color_3))))