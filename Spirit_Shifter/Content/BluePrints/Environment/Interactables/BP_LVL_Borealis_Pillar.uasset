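; Interactable pillar for the Borealis level that triggers a time toggle when the player interacts with it.
; Player overlap with its box starts a looping timer that polls the Interact input, then calls ToggleTime and clears itself on a press.
; An unconnected sky timeline holds logic to drive the Time material parameter, message affected actors through BPI_States and flip IsPast.
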(event OnComponentBeginOverlap(StaticMesh)
  (params (OverlappedComponent :type Primitive%20Component%20Object%20Reference) (OtherActor :type Actor%20Object%20Reference) (OtherComp :type Primitive%20Component%20Object%20Reference) (OtherBodyIndex :type Integer) (bFromSweep :type Boolean) (SweepResult :type Hit%20Result%20Structure%20%28by%20ref%29)))

(event OnComponentBeginOverlap(Box)
  (params (OverlappedComponent :type Primitive%20Component%20Object%20Reference) (OtherActor :type Actor%20Object%20Reference) (OtherComp :type Primitive%20Component%20Object%20Reference) (OtherBodyIndex :type Integer) (bFromSweep :type Boolean) (SweepResult :type Hit%20Result%20Structure%20%28by%20ref%29))
  (if (== OtherActor (Game|GetPlayerCharacter 0))
    (CallFunction|CanInteract)))

(event Custom|Interact_Timer_Event
  (bind _interact_timer (Variables|Default|GetInteract_Timer))
  (if (and (Utilities|Time|IsTimerActivebyHandle _interact_timer) (Input|EnhancedActionValues|GetIA_Interact))
    (CallFunction|RunInteract)
    (Utilities|Time|ClearandInvalidateTimerbyHandle _interact_timer)))

(event EventBeginPlay)

(event Collision|EventActorBeginOverlap
  (params (OtherActor :type Actor%20Object%20Reference)))

(event EventTick
  (params (DeltaSeconds :type Float%20%28single-precision%29)))

(event EventCanInteract
  (bind _returnvalue (Utilities|Time|SetTimerbyEvent (EventDispatchers|CreateEvent :!event Custom|Interact_Timer_Event) 0.1 true))
  (Variables|Default|SetInteract_Timer _returnvalue))

(event EventRunInteract
  (Default|CallToggleTime))

(fn ConstructionScript)