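; Cape interactable that swaps the player character's scarf mesh for its own skeletal mesh and introduces health with a tutorial widget.
; RunInteract passes a DoOnce, destroys the actor, shows the widget and deactivates the linked point-of-interest Niagara effect.
; Widget removal, interact reset and point-of-interest destruction follow a short Delay, placed after the actor's own DestroyActor call.
; Reset_Interact re-arms the DoOnce.
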(event Custom|Reset_Interact
  (bind _point_of_interest (Variables|Default|GetPoint_of_Interest))
  (Utilities|FlowControl|DoOnce false) ; enters at Reset
)

(event EventBeginPlay
  (|CallParentFunction) ; This node is disabled and will not be called.\nDrag off pins to build functionality.
)

(event Collision|EventActorBeginOverlap
  (params (OtherActor :type Actor%20Object%20Reference))
  (|CallParentFunction OtherActor) ; This node is disabled and will not be called.\nDrag off pins to build functionality.
)

(event EventTick
  (params (DeltaSeconds :type Float%20%28single-precision%29))
  (|CallParentFunction DeltaSeconds) ; This node is disabled and will not be called.\nDrag off pins to build functionality.
)

(event EventRunInteract
  (bind _point_of_interest (Variables|Default|GetPoint_of_Interest))
  (Utilities|FlowControl|DoOnce false
    (:Completed
      (Components|SkeletalMesh|SetSkeletalMeshAsset (Variables|/Game/BluePrints/Player/BP_Iso_PlayerCharacter.BP_Iso_PlayerCharacter_C|GetRigged_Scarf (.AsBP%20Iso%20Player%20Character (Utilities|Casting|CastToBP_Iso_PlayerCharacter (Game|GetPlayerCharacter 0)))) (Variables|/Script/Engine.SkeletalMeshComponent|GetSkeletalMeshAsset (Variables|Default|GetSkeletalMesh)))
      (Actor|DestroyActor)
      (bind _returnvalue (UserInterface|CreateWidget "/Game/HUD/WBP_Tutorial.WBP_Tutorial_C" (Game|GetPlayerController 0)))
      (Variables|/Game/HUD/WBP_Tutorial.WBP_Tutorial_C|SetText_To_Display _returnvalue "This is your health...")
      (UserInterface|Viewport|AddtoViewport _returnvalue 0)
      (Utilities|IsValid _point_of_interest
        (:Is%20Valid
          (Components|Activation|Deactivate (Variables|/Game/BluePrints/Environment/BP_Point_of_Interest.BP_Point_of_Interest_C|GetNiagara _point_of_interest)))
        (:Is%20Not%20Valid
          _))
      (Utilities|FlowControl|Delay 1.5)
      (Widget|RemovefromParent _returnvalue)
      (CallFunction|ResetInteract)
      (Actor|DestroyActor _point_of_interest))))

(fn ConstructionScript
  (|CallParentFunction))