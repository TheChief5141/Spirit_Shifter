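; BP_Checkpoint is an interactable checkpoint that drains the player's spirit fresnel glow and can set a linked moving island in motion.
; On interact it reads fresnel power and intensity from MPC_Player; if both are positive, it activates Niagara, enables the island and, for tutorials, spawns a slam effect.
; A DoOnce-gated timeline then lowers both values by clamped steps, regardless of that check, and calls a checkpoint reset on finish.
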(event Custom|Reset_Checkpoint
  (bind _current_fresnel_intesity (Variables|Default|GetCurrent_Fresnel_Intesity))
  (Utilities|FlowControl|DoOnce false) ; enters at Reset
)

(event EventBeginPlay)

(event Collision|EventActorBeginOverlap
  (params (OtherActor :type Actor%20Object%20Reference)))

(event EventTick
  (params (DeltaSeconds :type Float%20%28single-precision%29)))

(event EventCanInteract)

(event EventRunInteract
  (bind _moving_island (Variables|Default|GetMoving_Island))
  (Utilities|FlowControl|Sequence
    (:then_0
      (bind _returnvalue (Rendering|Material|GetScalarParameterValue "/Game/Materials/MPC_Player.MPC_Player" "Spirit_Frensel_Power" :!class /Script/Engine.KismetMaterialLibrary))
      (bind _output_get (Variables|Default|SetCurrent_Frensel_Power _returnvalue))
      (bind _returnvalue_2 (Rendering|Material|GetScalarParameterValue "/Game/Materials/MPC_Player.MPC_Player" "Spirit_Frensel_Intensity" :!class /Script/Engine.KismetMaterialLibrary))
      (bind _output_get_2 (Variables|Default|SetCurrent_Fresnel_Intesity _returnvalue_2))
      (if (and (> _output_get 0.0) (> _output_get_2 0.0))
        (Components|Activation|Activate (Variables|Default|GetNiagara) false)
        (Utilities|IsValid _moving_island
          (:Is%20Valid
            (Variables|/Game/BluePrints/Environment/BP_Moving_Island.BP_Moving_Island_C|SetCanMove _moving_island true)
            (if (Variables|Default|GetisTutorial)
              (Niagara|SpawnSystematLocation "/Game/Particles/VFX_Slam.VFX_Slam" (Transformation|GetWorldLocation (Variables|/Game/BluePrints/Environment/BP_Moving_Island.BP_Moving_Island_C|GettutorialCompleted (Variables|Default|GetMoving_Island)))))))))
    (:then_1
      (Utilities|FlowControl|DoOnce false
        (:Completed
          (bind _alpha (Timeline|Set_Parameter_Values Play)
            (:Update
              (Rendering|Material|SetScalarParameterValue "/Game/Materials/MPC_Player.MPC_Player" "Spirit_Frensel_Power" (Math|Float|Clamp(Float) (Math|Float|Lerp (Variables|Default|GetCurrent_Frensel_Power) (- (Variables|Default|GetCurrent_Frensel_Power) 4.0) _alpha) 0.0 12.0) :!class /Script/Engine.KismetMaterialLibrary)
              (Rendering|Material|SetScalarParameterValue "/Game/Materials/MPC_Player.MPC_Player" "Spirit_Frensel_Intensity" (Math|Float|Clamp(Float) (Math|Float|Lerp (Variables|Default|GetCurrent_Fresnel_Intesity) (- (Variables|Default|GetCurrent_Fresnel_Intesity) 25.0) _alpha) 0.0 75.0) :!class /Script/Engine.KismetMaterialLibrary))
            (:Finished
              (CallFunction|ResetCheckpoint))))))))

(event EventStopInteract)

(fn ConstructionScript)