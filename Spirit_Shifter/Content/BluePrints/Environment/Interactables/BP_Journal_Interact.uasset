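; BP_Journal_Interact is an interactable actor that shows story text when the player uses it.
; Its Box overlap sets IsInteracting while a BP_Iso_PlayerCharacter is inside and clears it on exit.
; While that flag is set, IA_Interact creates WBP_Story_Interact, fills it with TextToDisplay, focuses it in Game and UI input mode and pauses the game.
; BeginPlay also adds the IMC_Iso_Player_Controls mapping context to the player controller.
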(event OnComponentBeginOverlap(Box)
  (params (OverlappedComponent :type Primitive%20Component%20Object%20Reference) (OtherActor :type Actor%20Object%20Reference) (OtherComp :type Primitive%20Component%20Object%20Reference) (OtherBodyIndex :type Integer) (bFromSweep :type Boolean) (SweepResult :type Hit%20Result%20Structure%20%28by%20ref%29))
  (if (Utilities|ClassIsChildOf (Utilities|GetClass OtherActor) "/Game/BluePrints/Player/BP_Iso_PlayerCharacter.BP_Iso_PlayerCharacter_C")
    (CallFunction|CanInteract)))

(event OnComponentEndOverlap(Box)
  (params (OverlappedComponent :type Primitive%20Component%20Object%20Reference) (OtherActor :type Actor%20Object%20Reference) (OtherComp :type Primitive%20Component%20Object%20Reference) (OtherBodyIndex :type Integer))
  (if (Utilities|ClassIsChildOf (Utilities|GetClass OtherActor) "/Game/BluePrints/Player/BP_Iso_PlayerCharacter.BP_Iso_PlayerCharacter_C")
    (CallFunction|StopInteract)))

(event Input|EnhancedActionEvents|EnhancedInputActionIA_Interact
  (params (ActionValue :type Boolean) (ElapsedSeconds :type Float%20%28double-precision%29) (TriggeredSeconds :type Float%20%28double-precision%29) (InputAction :type Input%20Action%20Object%20Reference :default "/Game/Controls/Input_Actions/IA_Interact.IA_Interact"))
  (:Started
    (if (Variables|Default|GetIsInteracting?)
      (CallFunction|RunInteract))))

(event EventBeginPlay
  (bind _asbp_iso_player_controller (Utilities|Casting|CastToBP_Iso_Player_Controller (Game|GetPlayerController 0)))
  (Utilities|IsValid (PlayerController|LocalPlayerSubsystems|GetEnhancedInputLocalPlayerSubsystem _asbp_iso_player_controller)
    (:Is%20Valid
      (Input|AddMappingContext (PlayerController|LocalPlayerSubsystems|GetEnhancedInputLocalPlayerSubsystem _asbp_iso_player_controller) "/Game/Controls/Input_Actions/IMC_Iso_Player_Controls.IMC_Iso_Player_Controls" 0 "(bIgnoreAllPressedKeysUntilRelease=True,bForceImmediately=False)"))))

(event Collision|EventActorBeginOverlap
  (params (OtherActor :type Actor%20Object%20Reference)))

(event EventTick
  (params (DeltaSeconds :type Float%20%28single-precision%29)))

(event EventRunInteract
  (bind _returnvalue (Game|GetPlayerController 0))
  (if (Variables|Default|GetIsInteracting?)
    (bind _returnvalue_2 (UserInterface|CreateWidget "/Game/HUD/WBP_Story_Interact.WBP_Story_Interact_C" _returnvalue))
    (Variables|/Game/HUD/WBP_Story_Interact.WBP_Story_Interact_C|SetText_to_Fill _returnvalue_2 (Variables|Default|GetText_to_Display))
    (UserInterface|Viewport|AddtoViewport _returnvalue_2 0)
    (Input|SetInputModeGameandUI _returnvalue _returnvalue_2 "DoNotLock" true false)
    (Game|SetGamePaused true)))

(event EventCanInteract
  (Variables|Default|SetIsInteracting? true))

(event EventStopInteract
  (Variables|Default|SetIsInteracting? false))

(fn ConstructionScript)