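; Moving island platform that travels between its start and a target, either automatically or when the player steps on it.
; The construction script offsets the target along a chosen axis, unless an instance-specific location is used and resolved at BeginPlay.
; A timeline lerps the mesh, with play rate scaled by distance, and alternates direction after a pause.
; Player contact on an island that cannot move fires a move-to-boss call instead.
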(event OnComponentBeginOverlap(Box)
  (params (OverlappedComponent :type Primitive%20Component%20Object%20Reference) (OtherActor :type Actor%20Object%20Reference) (OtherComp :type Primitive%20Component%20Object%20Reference) (OtherBodyIndex :type Integer) (bFromSweep :type Boolean) (SweepResult :type Hit%20Result%20Structure%20%28by%20ref%29))
  (if (Utilities|ClassIsChildOf (Utilities|GetClass OtherActor) "/Game/BluePrints/Player/BP_Iso_PlayerCharacter.BP_Iso_PlayerCharacter_C")
    (Development|PrintString "player touched island")
    (if (Variables|Default|GetCanMove)
      (Variables|Default|SetIsland_Touched true)
      (CallFunction|MoveIsland)
      (else
        (Development|PrintString "touched boss island hehe")
        (Default|CallMovetoBoss self)))))

(event OnComponentEndOverlap(Box)
  (params (OverlappedComponent :type Primitive%20Component%20Object%20Reference) (OtherActor :type Actor%20Object%20Reference) (OtherComp :type Primitive%20Component%20Object%20Reference) (OtherBodyIndex :type Integer))
  (if (Utilities|ClassIsChildOf (Utilities|GetClass OtherActor) "/Game/BluePrints/Player/BP_Iso_PlayerCharacter.BP_Iso_PlayerCharacter_C")
    (Variables|Default|SetIsland_Touched false)))

(event Custom|Restart_Timeline
  (Variables|Default|SetIsland_Touched false)
  (bind _alpha (Timeline|Move_Timeline Reverse)
    (:Update
      (Transformation|SetRelativeLocation (Variables|Debug|GetStaticMeshComponent) (Math|Vector|Lerp(Vector) (Variables|Default|GetOriginal_Location) (Variables|Default|GetTarget_Location) _alpha) false false))
    (:Finished
      (Utilities|FlowControl|Delay 3.0)
      (if (Variables|Default|GetAtTop)
        (Variables|Default|SetAtTop false)
        (CallFunction|MoveIsland)
        (else
          (Variables|Default|SetAtTop true)
          (CallFunction|RestartTimeline))))))

(event Custom|Move_Island
  (if (Variables|Default|GetAuto_Movement)
    (bind _alpha (Timeline|Move_Timeline Play)
      (:Update
        (Transformation|SetRelativeLocation (Variables|Debug|GetStaticMeshComponent) (Math|Vector|Lerp(Vector) (Variables|Default|GetOriginal_Location) (Variables|Default|GetTarget_Location) _alpha) false false))
      (:Finished
        (Utilities|FlowControl|Delay 3.0)
        (if (Variables|Default|GetAtTop)
          (Variables|Default|SetAtTop false)
          (CallFunction|MoveIsland)
          (else
            (Variables|Default|SetAtTop true)
            (CallFunction|RestartTimeline)))))
    (elif (and (Variables|Default|GetIsland_Touched) (not (Variables|Default|GetAtTop)))
      (Timeline|Move_Timeline Play))))

(event EventBeginPlay
  (bind _move_timeline (Variables|Default|GetMove_Timeline))
  (if (Variables|Default|GetUse_Instance?)
    (Variables|Default|SetTarget_Location (+ (/ (Variables|Default|GetAuto_Location) (/ 1.0 (Transformation|GetWorldScale (Variables|Debug|GetStaticMeshComponent)))) (Variables|Default|GetOriginal_Location)))
    (CallFunction|MoveIsland)
    (Variables|Default|SetMovement_Distance (Math|Vector|Distance(Vector) (Variables|Default|GetOriginal_Location) (Variables|Default|GetTarget_Location))))
  (Components|Timeline|SetPlayRate _move_timeline (/ 1.0 (/ (Variables|Default|GetMovement_Distance) 4e+03)))
  (Components|Timeline|SetTimelineLength _move_timeline 4.0))

(fn ConstructionScript
  (Variables|Default|SetOriginal_Location (Transformation|GetWorldLocation (Variables|Debug|GetStaticMeshComponent)))
  (if (not (Variables|Default|GetUse_Instance?))
    (switch int (Variables|Default|GetMovement_Direction)
      (:0
        (Variables|Default|SetTarget_Location (Math|Vector|MakeVector (+ (.X (Class|KismetMathLibrary|BreakVector3f (Variables|Default|GetOriginal_Location))) (Variables|Default|GetMovement_Distance)) (.Y (Class|KismetMathLibrary|BreakVector3f (Variables|Default|GetOriginal_Location))) (.Z (Class|KismetMathLibrary|BreakVector3f (Variables|Default|GetOriginal_Location))))))
      (:1
        (Variables|Default|SetTarget_Location (Math|Vector|MakeVector (.X (Class|KismetMathLibrary|BreakVector3f (Variables|Default|GetOriginal_Location))) (+ (.Y (Class|KismetMathLibrary|BreakVector3f (Variables|Default|GetOriginal_Location))) (Variables|Default|GetMovement_Distance)) (.Z (Class|KismetMathLibrary|BreakVector3f (Variables|Default|GetOriginal_Location))))))
      (:2
        (Variables|Default|SetTarget_Location (Math|Vector|MakeVector (.X (Class|KismetMathLibrary|BreakVector3f (Variables|Default|GetOriginal_Location))) (.Y (Class|KismetMathLibrary|BreakVector3f (Variables|Default|GetOriginal_Location))) (+ (.Z (Class|KismetMathLibrary|BreakVector3f (Variables|Default|GetOriginal_Location))) (Variables|Default|GetMovement_Distance))))))))