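; Wind spirit pawn that moves toward the player when it sees them and counts as saved on touch.
; Overlap runs a timeline that animates the player's fresnel power and intensity through MPC_Player, then calls SpiritSaved.
; The bound Contact handler shows a tutorial widget, deactivates the Niagara effect and destroys the spirit after a delay.
; Spirits flagged as tutorial also trigger TutorialIsland on moving islands.
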(event OnSeePawn(PawnSensing)
  (params (Pawn :type Pawn%20Object%20Reference))
  (bind _returnvalue (Game|GetPlayerCharacter 0))
  (if (== Pawn _returnvalue)
    (AI|AIMoveTo self "0, 0, 0" _returnvalue 0.0 false
      (:then
        (Development|PrintString "see player")
        (if (Variables|Default|GettutorialSpirit)
          (Default|TutorialIsland (Variables|Default|GettutIsland)))))))

(event OnComponentBeginOverlap(CapsuleComponent)
  (params (OverlappedComponent :type Primitive%20Component%20Object%20Reference) (OtherActor :type Actor%20Object%20Reference) (OtherComp :type Primitive%20Component%20Object%20Reference) (OtherBodyIndex :type Integer) (bFromSweep :type Boolean) (SweepResult :type Hit%20Result%20Structure%20%28by%20ref%29))
  (bind _wind_to_move_character (Variables|Default|GetWind_to_Move_Character))
  (bind _affected_actor (Variables|/Game/BluePrints/Environment/Interactables/BP_Checkpoint.BP_Checkpoint_C|GetAffected_Actor _wind_to_move_character))
  (if (== OtherActor (Game|GetPlayerCharacter 0))
    (Utilities|FlowControl|Sequence
      (:then_0
        (bind _returnvalue (Rendering|Material|GetScalarParameterValue "/Game/Materials/MPC_Player.MPC_Player" "Spirit_Frensel_Power" :!class /Script/Engine.KismetMaterialLibrary))
        (Variables|Default|SetCurrent_Frensel_Power _returnvalue)
        (bind _returnvalue_2 (Rendering|Material|GetScalarParameterValue "/Game/Materials/MPC_Player.MPC_Player" "Spirit_Frensel_Intensity" :!class /Script/Engine.KismetMaterialLibrary))
        (Variables|Default|SetCurrent_Frensel_Intensity _returnvalue_2))
      (:then_1
        (bind _scale (Timeline|SetScale Play)
          (:Update
            (Rendering|Material|SetScalarParameterValue "/Game/Materials/MPC_Player.MPC_Player" "Spirit_Frensel_Power" (Math|Float|Clamp(Float) (Math|Float|Lerp (+ (Variables|Default|GetCurrent_Frensel_Power) 4.0) (Variables|Default|GetCurrent_Frensel_Power) _scale) 0.0 12.0) :!class /Script/Engine.KismetMaterialLibrary)
            (Rendering|Material|SetScalarParameterValue "/Game/Materials/MPC_Player.MPC_Player" "Spirit_Frensel_Intensity" (Math|Float|Clamp(Float) (Math|Float|Lerp (+ (Variables|Default|GetCurrent_Frensel_Intensity) 25.0) (Variables|Default|GetCurrent_Frensel_Intensity) _scale) 0.0 75.0) :!class /Script/Engine.KismetMaterialLibrary))
          (:Finished
            (Utilities|FlowControl|DoOnce false
              (:Completed
                (Default|CallSpiritSaved self)
                (CallFunction|ResetSpiritSaved))))))
      (:then_2
        (if (Variables|Default|GettutorialSpirit)
          (if (Utilities|ClassIsChildOf (Utilities|GetClass _affected_actor) "/Game/BluePrints/Environment/BP_Moving_Island.BP_Moving_Island_C")
            (Default|TutorialIsland (.AsBP%20Moving%20Island (Utilities|Casting|CastToBP_Moving_Island _affected_actor)))))))))

(event Custom|Reset_Spirit_Saved
  (Utilities|FlowControl|DoOnce false) ; enters at Reset
)

(event Custom|Contact
  (params (Saved_Spirit :type BP%20LVL%20Wind%20Spirit%20Object%20Reference))
  (bind _wind_to_move_character (Variables|Default|GetWind_to_Move_Character))
  (bind _affected_actor (Variables|/Game/BluePrints/Environment/Interactables/BP_Checkpoint.BP_Checkpoint_C|GetAffected_Actor _wind_to_move_character))
  (bind _returnvalue (UserInterface|CreateWidget "/Game/HUD/WBP_Tutorial.WBP_Tutorial_C" (Game|GetPlayerController 0)))
  (Variables|/Game/HUD/WBP_Tutorial.WBP_Tutorial_C|SetText_To_Display _returnvalue (Variables|Default|GetText_for_Tutorial))
  (if (Variables|Default|GettutorialSpirit)
    (Utilities|FlowControl|Sequence
      (:then_0
        (UserInterface|Viewport|AddtoViewport _returnvalue 0 :!label _label)
        (Components|Activation|Deactivate (Variables|Default|GetNiagara))
        (Utilities|FlowControl|Delay 3.5)
        (Widget|RemovefromParent _returnvalue)
        (Actor|DestroyActor))
      (:then_1
        (if (Utilities|ClassIsChildOf (Utilities|GetClass _affected_actor) "/Game/BluePrints/Environment/BP_Moving_Island.BP_Moving_Island_C")
          (Default|TutorialIsland (.AsBP%20Moving%20Island (Utilities|Casting|CastToBP_Moving_Island _affected_actor))))))
    (else
      (goto _label))))

(event EventBeginPlay
  (EventDispatchers|BindEventtoSpiritSaved (delegate Custom|Contact)))

(fn ConstructionScript)