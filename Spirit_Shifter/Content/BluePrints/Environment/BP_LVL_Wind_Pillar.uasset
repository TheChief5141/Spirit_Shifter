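; Level pillar the player interacts with to trigger a wind-rotation cutscene affecting every BP_LVL_WindFlip actor.
; Player overlap with its box starts a looping timer that polls the Interact input until pressed.
; It then blends the view to CameraActor with input disabled, calls RotateTheWind on each WindFlip actor after a delay, and later blends back to the player and restores input.
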(event OnComponentBeginOverlap(StaticMesh)
  (params (OverlappedComponent :type Primitive%20Component%20Object%20Reference) (OtherActor :type Actor%20Object%20Reference) (OtherComp :type Primitive%20Component%20Object%20Reference) (OtherBodyIndex :type Integer) (bFromSweep :type Boolean) (SweepResult :type Hit%20Result%20Structure%20%28by%20ref%29)))

(event OnComponentBeginOverlap(Box)
  (params (OverlappedComponent :type Primitive%20Component%20Object%20Reference) (OtherActor :type Actor%20Object%20Reference) (OtherComp :type Primitive%20Component%20Object%20Reference) (OtherBodyIndex :type Integer) (bFromSweep :type Boolean) (SweepResult :type Hit%20Result%20Structure%20%28by%20ref%29))
  (if (== OtherActor (Game|GetPlayerCharacter 0))
    (CallFunction|CanInteract)))

(event Custom|Interact_Timer_Event
  (bind _interact_timer (Variables|Default|GetInteract_Timer))
  (if (and (Utilities|Time|IsTimerActivebyHandle _interact_timer) (Input|EnhancedActionValues|GetIA_Interact))
    (CallFunction|RunInteract)
    (Utilities|Time|ClearandInvalidateTimerbyHandle _interact_timer)))

(event EventBeginPlay)

(event Collision|EventActorBeginOverlap
  (params (OtherActor :type Actor%20Object%20Reference)))

(event EventTick
  (params (DeltaSeconds :type Float%20%28single-precision%29)))

(event EventCanInteract
  (bind _returnvalue (Utilities|Time|SetTimerbyEvent (EventDispatchers|CreateEvent :!event Custom|Interact_Timer_Event) 0.1 true))
  (Variables|Default|SetInteract_Timer _returnvalue))

(event EventRunInteract
  (bind _returnvalue (Game|GetPlayerController 0))
  (bind _camera_actor (Variables|Default|GetCamera_Actor))
  (Utilities|IsValid (Actor|GetComponentbyClass _camera_actor "/Script/Engine.CameraComponent")
    (:Is%20Valid
      (Game|Player|SetViewTargetwithBlend _returnvalue _camera_actor 2.0 "VTBlend_EaseIn" 1.0 false)
      (Input|DisableInput _returnvalue 0)
      (bind _outactors (Actor|GetAllActorsOfClass "/Game/BluePrints/Environment/BP_LVL_WindFlip.BP_LVL_WindFlip_C"))
      (Utilities|FlowControl|Delay 2.0)
      (Utilities|FlowControl|Sequence
        (:then_0
          (for _array_element _outactors
            (Default|RotatetheWind _array_element _array_element)
            (Utilities|FlowControl|Delay 0.4)))
        (:then_1
          (Utilities|FlowControl|Delay 2.0)
          (Game|Player|SetViewTargetwithBlend _returnvalue (Game|GetPlayerCharacter 0) 2.0 "VTBlend_EaseIn" 1.0 false)
          (Input|EnableInput _returnvalue 0))))))

(fn ConstructionScript)