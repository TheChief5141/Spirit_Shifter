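; Game mode for Spirit Shifter that handles player death by reloading the Lush Forest level.
; BeginPlay binds to the player character's destroyed event, with Respawn_Player reopening the level unless DontRespawnPlayer is set.
; ToMainMenu sets that flag but opens the same forest level.
; A separate RespawnPlayer event spawns and possesses a new pawn, while an older delayed respawn with camera refocus is left unconnected.
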(event Custom|RespawnPlayer
  (params (myPlayer :type Character%20Object%20Reference))
  (bind _returnvalue (Game|SpawnActorfromClass (Utilities|GetClass myPlayer) (Variables|Default|GetspawnTransform) "Undefined" "MultiplyWithRoot" 0 0))
  (bind _asbp_iso_player_controller (Utilities|Casting|CastToBP_Iso_Player_Controller (Game|GetPlayerController 0)))
  (Pawn|Possess _asbp_iso_player_controller _returnvalue))

(event Custom|Respawn_Player
  (params (DestroyedActor :type Actor%20Object%20Reference))
  (if (not (Variables|Default|GetdontRespawnPlayer))
    (Game|OpenLevel(byName) "LVL_Lush_Forest_Real")))

(event Custom|ToMainMenu
  (Variables|Default|SetdontRespawnPlayer true)
  (Game|OpenLevel(byName) "LVL_Lush_Forest_Real"))

(event EventBeginPlay
  (Game|BindEventtoOnDestroyed (.AsBP%20Iso%20Player%20Character (Utilities|Casting|CastToBP_Iso_PlayerCharacter (Game|GetPlayerCharacter 0))) (EventDispatchers|CreateEvent :!event Custom|Respawn_Player)))

(event EventTick
  (params (DeltaSeconds :type Float%20%28single-precision%29)))

(fn ConstructionScript)