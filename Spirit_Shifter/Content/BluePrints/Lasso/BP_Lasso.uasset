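; Lasso actor that shoots a snake head toward a target actor, growing a body of mesh segments behind it.
; Firing sets the Head_Movement timeline's play rate from squared distance to the target, then each update lerps the head toward the target's current location.
; Segments chain by sockets whenever the newest piece is far enough from the actor, and reset destroys them.
; Construction and spline functions are empty stubs.
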(event Custom|Stop_Lasso
  (bind _headmesh (Variables|Default|GetHeadMesh))
  (bind _alpha (Timeline|Head_Movement Stop)
    (:Update
      (Transformation|SetWorldLocation _headmesh (Math|Vector|Lerp(Vector) (Transformation|GetWorldLocation _headmesh) (Transformation|GetActorLocation (stale Custom|Fire_Lasso Target_Actor)) _alpha) false false)
      (if (> (Class|KismetMathLibrary|VectorDistanceSquared (Transformation|GetWorldLocation (Variables|Default|GetClosest_Piece)) (Transformation|GetActorLocation)) 196.0)
        (bind _returnvalue (AddComponent|AddStaticMeshComponent false (Transformation|GetSocketTransform (Variables|Default|GetClosest_Piece) "End" "RTS_World")))
        (Transformation|AttachComponentToComponent _returnvalue (Variables|Default|GetClosest_Piece) "Start" "SnapToTarget" "SnapToTarget" "SnapToTarget" true)
        (Variables|Default|SetClosest_Piece _returnvalue)
        (Utilities|Array|Add (Variables|Default|GetLasso_Components) _returnvalue)))
    (:Finished
      (CallFunction|StopLasso)
      (CallFunction|SetNewTime)
      (CallFunction|ResetLasso))))

(event Custom|Set_New_Time
  (bind _headmesh (Variables|Default|GetHeadMesh))
  (bind _alpha (Timeline|Head_Movement SetNewTime)
    (:Update
      (Transformation|SetWorldLocation _headmesh (Math|Vector|Lerp(Vector) (Transformation|GetWorldLocation _headmesh) (Transformation|GetActorLocation (stale Custom|Fire_Lasso Target_Actor)) _alpha) false false)
      (if (> (Class|KismetMathLibrary|VectorDistanceSquared (Transformation|GetWorldLocation (Variables|Default|GetClosest_Piece)) (Transformation|GetActorLocation)) 196.0)
        (bind _returnvalue (AddComponent|AddStaticMeshComponent false (Transformation|GetSocketTransform (Variables|Default|GetClosest_Piece) "End" "RTS_World")))
        (Transformation|AttachComponentToComponent _returnvalue (Variables|Default|GetClosest_Piece) "Start" "SnapToTarget" "SnapToTarget" "SnapToTarget" true)
        (Variables|Default|SetClosest_Piece _returnvalue)
        (Utilities|Array|Add (Variables|Default|GetLasso_Components) _returnvalue)))
    (:Finished
      (CallFunction|StopLasso)
      (CallFunction|SetNewTime)
      (CallFunction|ResetLasso))))

(event Custom|Fire_Lasso
  (params (Target_Actor :type Actor%20Object%20Reference))
  (bind _headmesh (Variables|Default|GetHeadMesh))
  (Components|Timeline|SetPlayRate (Variables|Default|GetHead_Movement) (/ (Class|KismetMathLibrary|VectorDistanceSquared (Transformation|GetWorldLocation _headmesh) (Transformation|GetActorLocation Target_Actor)) (Variables|Default|GetDistanceRate)))
  (Variables|Default|SetClosest_Piece (Variables|Default|GetSnakeBodyRepeatable))
  (CallFunction|ResetLasso)
  (bind _alpha (Timeline|Head_Movement Play)
    (:Update
      (Transformation|SetWorldLocation _headmesh (Math|Vector|Lerp(Vector) (Transformation|GetWorldLocation _headmesh) (Transformation|GetActorLocation Target_Actor) _alpha) false false)
      (if (> (Class|KismetMathLibrary|VectorDistanceSquared (Transformation|GetWorldLocation (Variables|Default|GetClosest_Piece)) (Transformation|GetActorLocation)) 196.0)
        (bind _returnvalue (AddComponent|AddStaticMeshComponent false (Transformation|GetSocketTransform (Variables|Default|GetClosest_Piece) "End" "RTS_World")))
        (Transformation|AttachComponentToComponent _returnvalue (Variables|Default|GetClosest_Piece) "Start" "SnapToTarget" "SnapToTarget" "SnapToTarget" true)
        (Variables|Default|SetClosest_Piece _returnvalue)
        (Utilities|Array|Add (Variables|Default|GetLasso_Components) _returnvalue)))
    (:Finished
      (CallFunction|StopLasso)
      (CallFunction|SetNewTime)
      (CallFunction|ResetLasso))))

(event Custom|Reset_Lasso
  (bind _lasso_components (Variables|Default|GetLasso_Components))
  (for _array_element _lasso_components
    (Components|DestroyComponent _array_element))
  (Utilities|Array|Clear _lasso_components))

(event EventBeginPlay)

(event Collision|EventActorBeginOverlap
  (params (OtherActor :type Actor%20Object%20Reference)))

(event EventTick
  (params (DeltaSeconds :type Float%20%28single-precision%29)))

(fn ConstructionScript
  (CallFunction|LassoStart))

(fn LassoStart)

(fn CreateLassoSpline
  (params (Point_Along_Spline :type Integer) (Spline_Component :type Spline%20Component%20Object%20Reference)))