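; Trigger volume that switches the isometric player's camera to focus on a spirit while the player character stands inside it.
; Box begin overlap tells the player controller to switch to the entry camera and sets its focus to the spirit's skeletal mesh.
; End overlap switches to the return camera and refocuses it on the player character's root component.
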(event OnComponentBeginOverlap(Box)
  (params (OverlappedComponent :type Primitive%20Component%20Object%20Reference) (OtherActor :type Actor%20Object%20Reference) (OtherComp :type Primitive%20Component%20Object%20Reference) (OtherBodyIndex :type Integer) (bFromSweep :type Boolean) (SweepResult :type Hit%20Result%20Structure%20%28by%20ref%29))
  (bind _camera_to_enter (Variables|Default|GetCamera_To_Enter))
  (if (Utilities|ClassIsChildOf (Utilities|GetClass OtherActor) "/Game/BluePrints/Player/BP_Iso_PlayerCharacter.BP_Iso_PlayerCharacter_C")
    (Default|CallSwitchCameraMode (.AsBP%20Iso%20Player%20Controller (Utilities|Casting|CastToBP_Iso_Player_Controller (Game|GetPlayerController 0))) _camera_to_enter)
    (Default|SetFocusedActor _camera_to_enter (Variables|/Game/BluePrints/Spirits/Parent/BP_Player_Spirit_Parent.BP_Player_Spirit_Parent_C|GetSkeletalMesh (Variables|Default|GetSpirit_To_Focus)))))

(event OnComponentEndOverlap(Box)
  (params (OverlappedComponent :type Primitive%20Component%20Object%20Reference) (OtherActor :type Actor%20Object%20Reference) (OtherComp :type Primitive%20Component%20Object%20Reference) (OtherBodyIndex :type Integer))
  (bind _camera_to_return (Variables|Default|GetCamera_To_Return))
  (if (Utilities|ClassIsChildOf (Utilities|GetClass OtherActor) "/Game/BluePrints/Player/BP_Iso_PlayerCharacter.BP_Iso_PlayerCharacter_C")
    (Default|CallSwitchCameraMode (.AsBP%20Iso%20Player%20Controller (Utilities|Casting|CastToBP_Iso_Player_Controller (Game|GetPlayerController 0))) _camera_to_return)
    (Default|SetFocusedActor _camera_to_return (Variables|/Script/Engine.Actor|GetRootComponent (Game|GetPlayerCharacter 0)))))

(event EventBeginPlay)

(event Collision|EventActorBeginOverlap
  (params (OtherActor :type Actor%20Object%20Reference)))

(event EventTick
  (params (DeltaSeconds :type Float%20%28single-precision%29)))

(fn ConstructionScript)