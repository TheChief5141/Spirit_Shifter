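; BP_Camera_Animations is a camera actor Blueprint that plays camera animation sequences for the first player and returns the view to the character afterwards.
; Play_Camera_Animation starts a sequence through the GameplayCamerasSubsystem, blends the view target to this actor, and stores the handle.
; End_Camera_Animation stops that handle non-immediately and blends the view back to the player character over a given blend time.
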(event Custom|Play_Camera_Animation
  (params (Sequence :type Camera%20Animation%20Sequence%20Object%20Reference) (Blend_Time :type Float%20%28double-precision%29))
  (bind _returnvalue (Game|GetPlayerController 0))
  (bind _returnvalue_2 (CameraAnimation|PlayCameraAnimation (Subsystems|GetGameplayCamerasSubsystem) _returnvalue Sequence :!class /Script/GameplayCameras.GameplayCamerasSubsystem))
  (Game|Player|SetViewTargetwithBlend _returnvalue self Blend_Time "VTBlend_Linear" 0.0 false)
  (Variables|Default|SetCamera_Anim_REF _returnvalue_2))

(event Custom|End_Camera_Animation
  (params (Blend_Time :type Float%20%28double-precision%29))
  (bind _returnvalue (Game|GetPlayerController 0))
  (CameraAnimation|StopCameraAnimation (Subsystems|GetGameplayCamerasSubsystem) _returnvalue (Variables|Default|GetCamera_Anim_REF) :!class /Script/GameplayCameras.GameplayCamerasSubsystem)
  (Game|Player|SetViewTargetwithBlend _returnvalue (Game|GetPlayerCharacter 0) Blend_Time "VTBlend_Linear" 0.0 false))

(event EventBeginPlay)

(event Collision|EventActorBeginOverlap
  (params (OtherActor :type Actor%20Object%20Reference)))

(event EventTick
  (params (DeltaSeconds :type Float%20%28single-precision%29)))

(fn ConstructionScript)