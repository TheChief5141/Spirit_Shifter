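; Spline-rail camera actor that follows a focused actor, defaulting to the isometric player character when none is set on BeginPlay.
; Each tick it rotates the camera to look at that actor.
; Outside main-menu mode, it also moves the camera with sweep at a constant interpolation speed toward the spline point closest to the actor.
; Set_Focused_Actor lets other code switch the target.
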(event Custom|Set_Focused_Actor
  (params (Focused_Actor :type Actor%20Object%20Reference))
  (Variables|Default|SetFocused_Actor Focused_Actor))

(event EventBeginPlay
  (bind _output_get (Variables|Default|SetAs%20BP%20Iso%20Player%20Character (.AsBP%20Iso%20Player%20Character (Utilities|Casting|CastToBP_Iso_PlayerCharacter (Game|GetPlayerCharacter 0)))))
  (Utilities|IsValid _output_get
    (:Is%20Valid
      (Utilities|IsValid (Variables|Default|GetFocused_Actor)
        (:Is%20Not%20Valid
          (Variables|Default|SetFocused_Actor _output_get))))))

(event Collision|EventActorBeginOverlap
  (params (OtherActor :type Actor%20Object%20Reference)))

(event EventTick
  (params (DeltaSeconds :type Float%20%28single-precision%29))
  (bind _camera (Variables|Default|GetCamera))
  (bind _focused_actor (Variables|Default|GetFocused_Actor))
  (bind _returnvalue (Transformation|GetWorldLocation _camera))
  (Transformation|SetWorldRotation _camera (Math|Rotator|FindLookatRotation _returnvalue (Transformation|GetActorLocation _focused_actor)) false false)
  (if (not (Variables|Default|GetisMainMenu))
    (Transformation|SetWorldLocation _camera (Math|Interpolation|VInterptoConstant _returnvalue (Spline|FindLocationClosesttoWorldLocation (Variables|Default|GetSpline) (Transformation|GetWorldLocation (Variables|/Script/Engine.Actor|GetRootComponent _focused_actor)) "World") (Utilities|Time|GetWorldDeltaSeconds) 6e+03) true false)))

(fn ConstructionScript)