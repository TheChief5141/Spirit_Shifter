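; Camera switching volume that changes the player's camera when the player character hits its box.
; On a component hit, it checks that the other actor's class matches or derives from the player character's, then passes TargetCameraReference to BP_Iso_Player_Controller's CallSwitchCameraMode.
; The overlap events are empty.
; Unconnected logic holds a CanSwitch-gated variant and a switch to CameraEndReference with a delayed re-enable, neither of which runs.
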(event OnComponentBeginOverlap(Box)
  (params (OverlappedComponent :type Primitive%20Component%20Object%20Reference) (OtherActor :type Actor%20Object%20Reference) (OtherComp :type Primitive%20Component%20Object%20Reference) (OtherBodyIndex :type Integer) (bFromSweep :type Boolean) (SweepResult :type Hit%20Result%20Structure%20%28by%20ref%29)))

(event OnComponentEndOverlap(Box)
  (params (OverlappedComponent :type Primitive%20Component%20Object%20Reference) (OtherActor :type Actor%20Object%20Reference) (OtherComp :type Primitive%20Component%20Object%20Reference) (OtherBodyIndex :type Integer)))

(event OnComponentHit(Box)
  (params (HitComponent :type Primitive%20Component%20Object%20Reference) (OtherActor :type Actor%20Object%20Reference) (OtherComp :type Primitive%20Component%20Object%20Reference) (NormalImpulse :type Vector :default "0, 0, 0") (Hit :type Hit%20Result%20Structure%20%28by%20ref%29))
  (if (Utilities|ClassIsChildOf (Utilities|GetClass OtherActor) (Utilities|GetClass (Game|GetPlayerCharacter 0)))
    (Default|CallSwitchCameraMode (.AsBP%20Iso%20Player%20Controller (Utilities|Casting|CastToBP_Iso_Player_Controller (Game|GetPlayerController 0))) (Variables|Default|GetTarget_Camera_Reference))))

(event EventBeginPlay)

(event Collision|EventActorBeginOverlap
  (params (OtherActor :type Actor%20Object%20Reference)))

(event EventTick
  (params (DeltaSeconds :type Float%20%28single-precision%29)))

(fn ConstructionScript)