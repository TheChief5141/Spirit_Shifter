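; BP_OwlChar is an owl character that shows a line of dialogue the first time the player comes near.
; Its Box overlap handler casts to BP_Iso_PlayerCharacter and uses the SeenDialogue flag to fire only once.
; It passes its Dialogue variable to a new WBP_FancyDialogue widget, adds it to the viewport, then removes it after a fixed delay.
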(event OnComponentBeginOverlap(Box)
  (params (OverlappedComponent :type Primitive%20Component%20Object%20Reference) (OtherActor :type Actor%20Object%20Reference) (OtherComp :type Primitive%20Component%20Object%20Reference) (OtherBodyIndex :type Integer) (bFromSweep :type Boolean) (SweepResult :type Hit%20Result%20Structure%20%28by%20ref%29))
  (Utilities|Casting|CastToBP_Iso_PlayerCharacter OtherActor)
  (if (not (Variables|Default|GetseenDialogue))
    (bind _returnvalue (UserInterface|CreateWidget "/Game/HUD/WBP_FancyDialogue.WBP_FancyDialogue_C" (Game|GetPlayerController 0)))
    (Variables|/Game/HUD/WBP_FancyDialogue.WBP_FancyDialogue_C|SetdialogueText _returnvalue (Variables|Default|Getdialogue))
    (UserInterface|Viewport|AddtoViewport _returnvalue 0)
    (Variables|Default|SetseenDialogue true)
    (Utilities|FlowControl|Delay 5.0)
    (Widget|RemovefromParent _returnvalue)))

(event EventBeginPlay)

(event Collision|EventActorBeginOverlap
  (params (OtherActor :type Actor%20Object%20Reference)))

(event EventTick
  (params (DeltaSeconds :type Float%20%28single-precision%29)))

(fn ConstructionScript)