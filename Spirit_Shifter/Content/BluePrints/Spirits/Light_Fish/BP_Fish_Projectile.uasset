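; Projectile for the Light Fish spirit that takes the player character's rotation on spawn, sets its movement speed and starts a two-second timer.
; Overlapping anything but the player triggers the explosion and damages BP_UnitStats-derived actors.
; The explosion spawns a random number of BP_Fish_Projectile_Explode fragments in random horizontal directions, then after a delay destroys every actor of that class in the level.
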(event OnComponentBeginOverlap(Sphere)
  (params (OverlappedComponent :type Primitive%20Component%20Object%20Reference) (OtherActor :type Actor%20Object%20Reference) (OtherComp :type Primitive%20Component%20Object%20Reference) (OtherBodyIndex :type Integer) (bFromSweep :type Boolean) (SweepResult :type Hit%20Result%20Structure%20%28by%20ref%29))
  (Variables|Default|SetIsExploded true)
  (if (!= OtherActor (Game|GetPlayerCharacter 0))
    (CallFunction|ExplodeProjectile)
    (if (Utilities|ClassIsChildOf (Utilities|GetClass OtherActor) "/Game/BluePrints/AI/BP_UnitStats.BP_UnitStats_C")
      (Game|Damage|ApplyDamage OtherActor (Variables|Default|GetDamage) 0 0))))

(event Custom|Launch_Projectile)

(event Custom|Explode_Projectile
  (bind _returnvalue (Transformation|GetActorTransform))
  (Development|PrintString "exploded")
  (bind _output_get (Variables|Default|SetNum_Of_Projectiles (Math|Random|RandomInteger 16)))
  (for _index (range 0 _output_get)
    (Game|SpawnActorfromClass "/Game/BluePrints/Spirits/Light_Fish/BP_Fish_Projectile_Explode.BP_Fish_Projectile_Explode_C" (Math|Transform|MakeTransform (.location _returnvalue) (Math|Conversions|RotationFromXVector (Math|Vector|MakeVector (Math|Random|RandomFloatinRange -1.0 1.0) (Math|Random|RandomFloatinRange -1.0 1.0) 0.0)) (.scale _returnvalue)) "Undefined" "MultiplyWithRoot" 0 0))
  (Utilities|FlowControl|Delay 3.0)
  (bind _outactors (Actor|GetAllActorsOfClass "/Game/BluePrints/Spirits/Light_Fish/BP_Fish_Projectile_Explode.BP_Fish_Projectile_Explode_C"))
  (for _array_element _outactors
    (Actor|DestroyActor _array_element)))

(event EventBeginPlay
  (Transformation|SetActorRotation (Transformation|GetActorRotation (Game|GetPlayerCharacter 0)))
  (Variables|/Script/Engine.ProjectileMovementComponent|SetInitialSpeed (Variables|Default|GetProjectileMovement) (Variables|Default|GetProjectile_Speed))
  (Utilities|Time|SetTimerbyEvent (EventDispatchers|CreateEvent :!event Custom|Explode_Projectile) 2.0))

(event Collision|EventActorBeginOverlap
  (params (OtherActor :type Actor%20Object%20Reference)))

(event EventTick
  (params (DeltaSeconds :type Float%20%28single-precision%29)))

(fn ConstructionScript)