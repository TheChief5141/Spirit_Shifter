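; Light Fish spirit component that gives the isometric player a dash, a projectile and a lure-placement action through Enhanced Input.
; Dash spawns a wave along last input, then makes one interpolated move toward any forward capsule-trace hit.
; Projectile fires along the camera's flattened forward vector.
; Level action sphere-traces from the camera, falls back to a downward line trace, and relocates the existing BP_Lure onto island-material surfaces.
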(event Custom|Dash
  (bind _as_bp_iso_player_character (Variables|Default|GetAs%20BP%20Iso%20Player%20Character))
  (bind _as_bp_iso_player_character_2 (Variables|Default|GetAs%20BP%20Iso%20Player%20Character))
  (bind _returnvalue (Transformation|GetActorLocation _as_bp_iso_player_character))
  (bind _ascapsule_collision (Utilities|Casting|CastToCapsuleComponent (Variables|/Script/Engine.Actor|GetRootComponent _as_bp_iso_player_character))
    (:then
      (bind (_outhit _returnvalue_2) (Collision|CapsuleTraceByChannel _returnvalue (+ (* (Math|Vector|GetForwardVector (Transformation|GetActorRotation _as_bp_iso_player_character)) (Variables|Default|GetDash_Distance_0)) _returnvalue) (Components|Capsule|GetScaledCapsuleRadius _ascapsule_collision) (Components|Capsule|GetScaledCapsuleHalfHeight _ascapsule_collision) "TraceTypeQuery1" false (Utilities|Array|MakeArray _as_bp_iso_player_character) "None"))
      (if _returnvalue_2
        (Transformation|SetActorLocation _as_bp_iso_player_character_2 (Math|Interpolation|VInterpTo (Transformation|GetActorLocation _as_bp_iso_player_character_2) (.Location (Collision|BreakHitResult _outhit)) (Utilities|Time|GetWorldDeltaSeconds) (Variables|Default|GetDash_Speed)) true false)))
    (:CastFailed
      (Development|PrintString "Hello"))))

(event Input|EnhancedActionEvents|EnhancedInputActionIA_Projectile
  (params (ActionValue :type Boolean) (ElapsedSeconds :type Float%20%28double-precision%29) (TriggeredSeconds :type Float%20%28double-precision%29) (InputAction :type Input%20Action%20Object%20Reference :default "/Game/Controls/Input_Actions/IA_Projectile.IA_Projectile"))
  (:Started
    (CallFunction|FishProjectile)))

(event Input|EnhancedActionEvents|EnhancedInputActionIA_Spirit_LevelAction
  (params (ActionValue :type Boolean) (ElapsedSeconds :type Float%20%28double-precision%29) (TriggeredSeconds :type Float%20%28double-precision%29) (InputAction :type Input%20Action%20Object%20Reference :default "/Game/Controls/Input_Actions/IA_Spirit_LevelAction.IA_Spirit_LevelAction"))
  (bind _returnvalue (Game|GetPlayerController 0))
  (bind _returnvalue_2 (Components|GetOwner))
  (bind _array (Utilities|Array|MakeArray _returnvalue_2))
  (bind _playercameramanager (Variables|/Script/Engine.PlayerController|GetPlayerCameraManager _returnvalue))
  (bind _returnvalue_3 (Transformation|GetActorLocation _playercameramanager))
  (:Started
    (bind (_outhit _returnvalue_4) (Collision|SphereTraceByChannel _returnvalue_3 (+ _returnvalue_3 (* (Transformation|GetActorForwardVector _playercameramanager) (Variables|Default|GetDistance_Multipler))) 2e+01 "TraceTypeQuery1" true _array "ForDuration"))
    (if _returnvalue_4
      (if (== (.ReturnValue (Class|PrimitiveComponent|GetMaterialfromCollisionFaceIndex (.HitComponent (Collision|BreakHitResult _outhit)) (.ElementIndex (Collision|BreakHitResult _outhit)))) "/Game/Models/Island/IslandMAT_Inst.IslandMAT_Inst")
        (bind _returnvalue_5 (Actor|GetActorOfClass "/Game/BluePrints/Spirits/Light_Fish/BP_Lure.BP_Lure_C"))
        (Default|ToggleState _returnvalue_5 false)
        (Utilities|FlowControl|Delay 0.5)
        (Transformation|SetActorLocationAndRotation _returnvalue_5 (- (.Location (Collision|BreakHitResult _outhit)) "") (Math|Conversions|RotationFromXVector (Math|Vector|ProjectVectorontoPlane (.Normal (Collision|BreakHitResult _outhit)) "0.000000,0.000000,1.000000")) false true)
        (Default|ToggleState _returnvalue_5 true))
      (else
        (bind (_outhit_2 _returnvalue_6) (Collision|LineTraceByChannel (.TraceEnd (Collision|BreakHitResult _outhit)) (- (.TraceEnd (Collision|BreakHitResult _outhit)) (Math|Vector|MakeVector 0.0 0.0 (Variables|Default|GetDistance_Multipler))) "TraceTypeQuery1" true _array "ForDuration"))
        (if _returnvalue_6
          (if (== (.ReturnValue (Class|PrimitiveComponent|GetMaterialfromCollisionFaceIndex (.HitComponent (Collision|BreakHitResult _outhit_2)) (.ElementIndex (Collision|BreakHitResult _outhit_2)))) "/Game/Models/Island/IslandMAT_Inst.IslandMAT_Inst")
            (bind _returnvalue_7 (Actor|GetActorOfClass "/Game/BluePrints/Spirits/Light_Fish/BP_Lure.BP_Lure_C"))
            (Default|ToggleState _returnvalue_7 false)
            (Utilities|FlowControl|Delay 0.5)
            (Transformation|SetActorLocationAndRotation _returnvalue_7 (- (.Location (Collision|BreakHitResult _outhit_2)) "") (Math|Conversions|RotationFromXVector (Math|Vector|ProjectVectorontoPlane (.Normal (Collision|BreakHitResult _outhit_2)) "0.000000,0.000000,1.000000")) false true)
            (Default|ToggleState _returnvalue_7 true)))))))

(event Input|EnhancedActionEvents|EnhancedInputActionIA_Dash
  (params (ActionValue :type Boolean) (ElapsedSeconds :type Float%20%28double-precision%29) (TriggeredSeconds :type Float%20%28double-precision%29) (InputAction :type Input%20Action%20Object%20Reference :default "/Game/Controls/Input_Actions/IA_Dash.IA_Dash"))
  (:Started
    (CallFunction|FishDash)))

(event EventBeginPlay
  (Input|AddMappingContext (PlayerController|LocalPlayerSubsystems|GetEnhancedInputLocalPlayerSubsystem (.AsBP%20Iso%20Player%20Controller (Utilities|Casting|CastToBP_Iso_Player_Controller (Game|GetPlayerController 0)))) "/Game/Controls/Input_Actions/IMC_Iso_Player_Controls.IMC_Iso_Player_Controls" 0 "(bIgnoreAllPressedKeysUntilRelease=True,bForceImmediately=False)")
  (Variables|Default|SetAs%20BP%20Iso%20Player%20Character (.AsBP%20Iso%20Player%20Character (Utilities|Casting|CastToBP_Iso_PlayerCharacter (Game|GetPlayerCharacter 0))))
  (Variables|Default|SetDash_Distance 6e+02))

(event EventTick
  (params (DeltaSeconds :type Float%20%28single-precision%29)))

(event EventSpiritProjectile
  (CallFunction|FishProjectile))

(fn FishProjectile
  (bind _returnvalue (Game|GetPlayerController 0))
  (bind _as_bp_iso_player_character (Variables|Default|GetAs%20BP%20Iso%20Player%20Character))
  (bind _returnvalue_2 (Transformation|GetActorTransform _as_bp_iso_player_character))
  (bind _playercameramanager (Variables|/Script/Engine.PlayerController|GetPlayerCameraManager _returnvalue))
  (bind _returnvalue_3 (Transformation|GetActorForwardVector _playercameramanager))
  (bind (_x _y) (Class|KismetMathLibrary|BreakVector3f _returnvalue_3))
  (Audio|PlaySoundatLocation "/Game/Audio/AudioClips/SFX/phase2/fishprojectile.fishprojectile" (.location _returnvalue_2) "0, 0, 0" 1.0 1.0 0.0 "/Game/Audio/EnemyAtten.EnemyAtten" 0 0 0)
  (bind _returnvalue_4 (Game|SpawnActorfromClass "/Game/BluePrints/Spirits/Light_Fish/BP_Fish_Projectile.BP_Fish_Projectile_C" (Math|Transform|MakeTransform (.location _returnvalue_2) (Math|Conversions|RotationFromXVector (Math|Vector|MakeVector _x _y 0.0)) (.scale _returnvalue_2)) "Undefined" "MultiplyWithRoot" 0 0))
  (Variables|/Game/BluePrints/Spirits/Light_Fish/BP_Fish_Projectile.BP_Fish_Projectile_C|SetSpawner _returnvalue_4 (Variables|/Script/Engine.Actor|GetRootComponent _as_bp_iso_player_character)))

(fn FishDash
  (bind _as_bp_iso_player_character (Variables|Default|GetAs%20BP%20Iso%20Player%20Character))
  (bind _returnvalue (Transformation|GetActorTransform _as_bp_iso_player_character))
  (Audio|PlaySoundatLocation "/Game/Audio/AudioClips/SFX/phase2/beachwaveshort.beachwaveshort" (.location _returnvalue) "0, 0, 0" 1.0 1.0 0.0 "/Game/Audio/EnemyAtten.EnemyAtten" 0 0 0)
  (bind _returnvalue_2 (Game|SpawnActorfromClass "/Game/BluePrints/Spirits/Light_Fish/BP_Fish_Wave.BP_Fish_Wave_C" (Math|Transform|MakeTransform (.location _returnvalue) (Math|Conversions|RotationFromXVector (Pawn|Components|PawnMovement|GetLastInputVector (Variables|/Script/Engine.Character|GetCharacterMovement (Game|GetPlayerCharacter 0)))) (.scale _returnvalue)) "Undefined" "MultiplyWithRoot" 0 0))
  (Variables|/Game/BluePrints/Spirits/Light_Fish/BP_Fish_Wave.BP_Fish_Wave_C|SetSpawner _returnvalue_2 (Variables|/Script/Engine.Actor|GetRootComponent _as_bp_iso_player_character))
  (CallFunction|Dash))