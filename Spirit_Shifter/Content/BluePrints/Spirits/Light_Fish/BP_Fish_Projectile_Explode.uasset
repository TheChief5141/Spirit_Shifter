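; Projectile for the Light Fish spirit's explosion that flies off in a random horizontal direction and damages units it touches.
; On BeginPlay it picks a random yaw and copies ExplosionSpeed into the ProjectileMovement component's InitialSpeed.
; Its Sphere overlap applies Damage to any BP_UnitStats actor, then destroys that actor rather than the projectile.
; Launch_Projectile is an empty event.
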(event OnComponentBeginOverlap(Sphere)
  (params (OverlappedComponent :type Primitive%20Component%20Object%20Reference) (OtherActor :type Actor%20Object%20Reference) (OtherComp :type Primitive%20Component%20Object%20Reference) (OtherBodyIndex :type Integer) (bFromSweep :type Boolean) (SweepResult :type Hit%20Result%20Structure%20%28by%20ref%29))
  (if (Utilities|ClassIsChildOf (Utilities|GetClass OtherActor) "/Game/BluePrints/AI/BP_UnitStats.BP_UnitStats_C")
    (Game|Damage|ApplyDamage OtherActor (Variables|Default|GetDamage) 0 0)
    (Actor|DestroyActor OtherActor)))

(event Custom|Launch_Projectile)

(event EventBeginPlay
  (Transformation|SetActorRotation (Math|Conversions|RotationFromXVector (Math|Vector|MakeVector (Math|Random|RandomFloatinRange -1.0 1.0) (Math|Random|RandomFloatinRange -1.0 1.0) 0.0)))
  (Variables|/Script/Engine.ProjectileMovementComponent|SetInitialSpeed (Variables|Default|GetProjectileMovement) (Variables|Default|GetExplosion_Speed)))

(event Collision|EventActorBeginOverlap
  (params (OtherActor :type Actor%20Object%20Reference)))

(event EventTick
  (params (DeltaSeconds :type Float%20%28single-precision%29)))

(fn ConstructionScript)