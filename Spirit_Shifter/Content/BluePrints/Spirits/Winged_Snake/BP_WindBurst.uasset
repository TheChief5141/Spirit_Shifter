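; BP_WindBurst is a wind burst actor for the Winged Snake spirit that launches units vertically.
; When a BP_UnitStats actor overlaps its Sphere, it calls LaunchCharacter with a Z velocity that overrides the unit's current vertical speed.
; ToggleState shows or hides the Niagara effect through its Lifetime parameter, which starts at zero on BeginPlay.
; The toggle affects only the visual, so the overlap launch is not gated by it.
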(event OnComponentBeginOverlap(Sphere)
  (params (OverlappedComponent :type Primitive%20Component%20Object%20Reference) (OtherActor :type Actor%20Object%20Reference) (OtherComp :type Primitive%20Component%20Object%20Reference) (OtherBodyIndex :type Integer) (bFromSweep :type Boolean) (SweepResult :type Hit%20Result%20Structure%20%28by%20ref%29))
  (if (Utilities|ClassIsChildOf (Utilities|GetClass OtherActor) "/Game/BluePrints/AI/BP_UnitStats.BP_UnitStats_C")
    (bind _asbp_unit_stats (Utilities|Casting|CastToBP_UnitStats OtherActor))
    (Character|LaunchCharacter _asbp_unit_stats (Math|Vector|MakeVector 0.0 0.0 (Variables|Default|GetLaunch%20Velocity%20Z)) false true)))

(event EventBeginPlay
  (Effects|Components|ParticleSystem|SetFloatParameter (Variables|Default|GetNiagara) "Lifetime" 0.0))

(event Collision|EventActorBeginOverlap
  (params (OtherActor :type Actor%20Object%20Reference)))

(event EventTick
  (params (DeltaSeconds :type Float%20%28single-precision%29)))

(event EventToggleState
  (params (On/Off :type Boolean))
  (bind _niagara (Variables|Default|GetNiagara))
  (if On/Off
    (Effects|Components|ParticleSystem|SetFloatParameter _niagara "Lifetime" 5.0)
    (else
      (Effects|Components|ParticleSystem|SetFloatParameter _niagara "Lifetime" 0.0))))

(fn ConstructionScript)