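; Winged snake spirit component that gives the player wind burst, projectile and dash abilities.
; Level action relocates the existing BP_WindBurst using a camera sphere trace with downward line-trace fallback, and projectile input spawns BP_Winged_Snake_Spirit along flattened camera forward.
; Dash launches the character along horizontal velocity, limited to two uses until a delayed grounded reset.
; Tether logic pulls spirits in or the owner to tether points, but its visible calls are disconnected.
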(event Custom|On_Enemy_Hit
  (params (OverlappedComponent :type Primitive%20Component%20Object%20Reference) (OtherActor :type Actor%20Object%20Reference) (OtherComp :type Primitive%20Component%20Object%20Reference) (OtherBodyIndex :type Integer) (bFromSweep :type Boolean) (SweepResult :type Hit%20Result%20Structure%20%28by%20ref%29))
  (if (!= OtherActor (Game|GetPlayerCharacter 0))
    (if (or (Utilities|ClassIsChildOf (Utilities|GetClass OtherActor) "/Game/BluePrints/AI/BP_UnitStats.BP_UnitStats_C") (Utilities|ClassIsChildOf (Utilities|GetClass OtherActor) "/Game/BluePrints/AI/MiniBoss/BP_ForestMiniBoss.BP_ForestMiniBoss_C"))
      (Utilities|FlowControl|DoOnce false :!label _label
        (:Completed
          (Game|Damage|ApplyDamage OtherActor (Variables|Default|GetWinged_Spirit_Damage) 0 0)
          (Utilities|FlowControl|Delay 1.0)
          (goto _label Reset))))))

(event Custom|Winged_Spirit_Projectile
  (bind _returnvalue (Game|GetPlayerController 0))
  (bind _returnvalue_2 (Components|GetOwner))
  (bind _playercameramanager (Variables|/Script/Engine.PlayerController|GetPlayerCameraManager _returnvalue))
  (bind _instigator (Variables|/Script/Engine.Actor|GetInstigator _returnvalue_2))
  (bind _returnvalue_3 (Transformation|GetActorForwardVector _playercameramanager))
  (bind _rootcomponent (Variables|/Script/Engine.Actor|GetRootComponent _instigator))
  (bind (_x _y) (Class|KismetMathLibrary|BreakVector3f _returnvalue_3))
  (bind _returnvalue_4 (Transformation|GetWorldTransform _rootcomponent))
  (bind (_location _rotation _scale) (Math|Transform|BreakTransform _returnvalue_4))
  ;[1 1 1] Projectile
  (Audio|PlaySoundatLocation "/Game/Audio/AudioClips/SFX/phase2/snkpro.snkpro" (Transformation|GetActorLocation _returnvalue_2) "0, 0, 0" 1.0 1.0 0.0 "/Game/Audio/EnemyAtten.EnemyAtten" 0 0 0)
  (if (not (Variables|Default|GetIsWeaponActive))
    (Variables|Default|SetIsWeaponActive true)
    (bind _returnvalue_5 (Game|SpawnActorfromClass "/Game/BluePrints/Spirits/Winged_Snake/BP_Winged_Snake_Spirit.BP_Winged_Snake_Spirit_C" (Math|Transform|MakeTransform _location (Math|Conversions|RotationFromXVector (Math|Vector|MakeVector _x _y 0.0)) (* _scale 2.0)) "Undefined" "MultiplyWithRoot" 0 _instigator))
    (Variables|/Script/Engine.ProjectileMovementComponent|SetInitialSpeed (Variables|/Game/BluePrints/Spirits/Winged_Snake/BP_Winged_Snake_Spirit.BP_Winged_Snake_Spirit_C|GetProjectileMovement _returnvalue_5) (Math|Vector|VectorLength (Transformation|GetVelocity _instigator)))
    (Variables|Default|SetIsWeaponActive false)))

(event Custom|Winged_Snake_Dash
  (CallFunction|WingedSpiritDash))

(event Custom|Winged_Snake_Tether
  (if (not (Variables|Default|GetIsTetherActive))
    (bind (_end_location _hit_successful) (CallFunction|CalculateTetherHit))
    (if _hit_successful
      (Variables|Default|SetEnd_Location_Of_Tether _end_location)
      (Variables|Default|SetIsTetherActive true))))

(event Custom|Reset_Dash
  (params (Hit :type Hit%20Result%20Structure%20%28by%20ref%29))
  (Utilities|FlowControl|Delay 0.01)
  (if (== (Variables|Default|GetDash_Used) 2)
    (if (not (AI|Components|NavMovement|IsFalling (Variables|/Script/Engine.Character|GetCharacterMovement (Variables|Default|GetAs%20BP%20Iso%20Player%20Character))))
      (Utilities|FlowControl|Delay 2.0)
      (Variables|Default|SetDash_Used 0))))

(event Custom|Winged_Spirit_Tether_Movement
  (bind _returnvalue (Components|GetOwner))
  (bind _returnvalue_2 (Components|GetOwner))
  (bind _hit_actor (Variables|Default|GetHit%20Actor))
  (bind _returnvalue_3 (Transformation|GetActorLocation _returnvalue_2))
  (if (Variables|Default|GetIsTetherActive)
    (Utilities|IsValid _hit_actor
      (:Is%20Valid
        (Transformation|SetActorLocation _hit_actor (Math|Interpolation|VInterptoConstant (Transformation|GetActorLocation _hit_actor) _returnvalue_3 (Utilities|Time|GetWorldDeltaSeconds) 2e+03) false false)
        (if (<= (Math|Vector|Distance2D(Vector) (Transformation|GetActorLocation _hit_actor) _returnvalue_3) 1.2)
          (Variables|Default|SetIsTetherActive false)))
      (:Is%20Not%20Valid
        (Transformation|SetActorLocation _returnvalue (Math|Interpolation|VInterptoConstant (Transformation|GetActorLocation _returnvalue) (Variables|Default|GetEnd_Location_Of_Tether) (Utilities|Time|GetWorldDeltaSeconds) 2e+03) false false)
        (if (<= (Math|Vector|Distance2D(Vector) (Transformation|GetActorLocation _returnvalue) (Variables|Default|GetEnd_Location_Of_Tether)) 1.2)
          (Variables|Default|SetIsTetherActive false))))))

(event Custom|Reset_Tether
  (Variables|Default|SetIsTetherActive true))

(event Input|EnhancedActionEvents|EnhancedInputActionIA_Projectile
  (params (ActionValue :type Boolean) (ElapsedSeconds :type Float%20%28double-precision%29) (TriggeredSeconds :type Float%20%28double-precision%29) (InputAction :type Input%20Action%20Object%20Reference :default "/Game/Controls/Input_Actions/IA_Projectile.IA_Projectile"))
  (:Started
    (CallFunction|WingedSpiritProjectile)))

(event Input|EnhancedActionEvents|EnhancedInputActionIA_Spirit_LevelAction
  (params (ActionValue :type Boolean) (ElapsedSeconds :type Float%20%28double-precision%29) (TriggeredSeconds :type Float%20%28double-precision%29) (InputAction :type Input%20Action%20Object%20Reference :default "/Game/Controls/Input_Actions/IA_Spirit_LevelAction.IA_Spirit_LevelAction"))
  (bind _returnvalue (Game|GetPlayerController 0))
  (bind _returnvalue_2 (Components|GetOwner))
  (bind _array (Utilities|Array|MakeArray _returnvalue_2))
  (bind _playercameramanager (Variables|/Script/Engine.PlayerController|GetPlayerCameraManager _returnvalue))
  (bind _returnvalue_3 (Transformation|GetActorLocation _playercameramanager))
  (:Started
    (bind (_outhit _returnvalue_4) (Collision|SphereTraceByChannel _returnvalue_3 (+ _returnvalue_3 (* (Transformation|GetActorForwardVector _playercameramanager) (Variables|Default|GetDistance_Multipler))) 2e+01 "TraceTypeQuery1" true _array "ForDuration"))
    (if _returnvalue_4
      (bind _returnvalue_5 (Actor|GetActorOfClass "/Game/BluePrints/Spirits/Winged_Snake/BP_WindBurst.BP_WindBurst_C"))
      (Default|ToggleState _returnvalue_5 false)
      (Transformation|SetActorLocationAndRotation _returnvalue_5 (- (.Location (Collision|BreakHitResult _outhit)) "") (Math|Conversions|RotationFromXVector (Math|Vector|ProjectVectorontoPlane (.Normal (Collision|BreakHitResult _outhit)) "0.000000,0.000000,1.000000")) false true)
      (Default|ToggleState _returnvalue_5 true)
      (else
        (bind (_outhit_2 _returnvalue_6) (Collision|LineTraceByChannel (.TraceEnd (Collision|BreakHitResult _outhit)) (- (.TraceEnd (Collision|BreakHitResult _outhit)) (Math|Vector|MakeVector 0.0 0.0 (Variables|Default|GetDistance_Multipler))) "TraceTypeQuery1" true _array "ForDuration"))
        (if _returnvalue_6
          (bind _returnvalue_7 (Actor|GetActorOfClass "/Game/BluePrints/Spirits/Winged_Snake/BP_WindBurst.BP_WindBurst_C"))
          (Default|ToggleState _returnvalue_7 false)
          (Utilities|FlowControl|Delay 0.5)
          (Transformation|SetActorLocationAndRotation _returnvalue_7 (- (.Location (Collision|BreakHitResult _outhit_2)) "") (Math|Conversions|RotationFromXVector (Math|Vector|ProjectVectorontoPlane (.Normal (Collision|BreakHitResult _outhit_2)) "0.000000,0.000000,1.000000")) false true)
          (Default|ToggleState _returnvalue_7 true))))))

(event EventBeginPlay)

(event EventTick
  (params (DeltaSeconds :type Float%20%28single-precision%29)))

(fn CalculateTetherHit
  (bind _returnvalue (Components|GetOwner))
  (bind _as_bp_iso_player_character (Variables|Default|GetAs%20BP%20Iso%20Player%20Character))
  (bind _capsulecomponent (Variables|/Script/Engine.Character|GetCapsuleComponent _as_bp_iso_player_character))
  (bind _instigator (Variables|/Script/Engine.Actor|GetInstigator _returnvalue))
  (bind _rootcomponent (Variables|/Script/Engine.Actor|GetRootComponent _instigator))
  (bind _returnvalue_2 (Transformation|GetWorldLocation _rootcomponent))
  (bind (_outhit _returnvalue_3) (Collision|LineTraceByChannel _returnvalue_2 (+ _returnvalue_2 (* (Math|Vector|GetForwardVector (Transformation|GetWorldRotation _rootcomponent)) (Variables|Default|GetDistance_Multipler))) "TraceTypeQuery3" false 0 "ForOneFrame"))
  (if _returnvalue_3
    (if (Utilities|ClassIsChildOf (Utilities|GetClass (.HitActor (Collision|BreakHitResult _outhit))) "/Game/BluePrints/Spirits/Parent/BP_Spirit.BP_Spirit_C")
      (Variables|Default|SetHit%20Actor (.HitActor (Collision|BreakHitResult _outhit))))
    (if (Utilities|ClassIsChildOf (Utilities|GetClass (.HitActor (Collision|BreakHitResult _outhit))) "/Game/BluePrints/Spirits/Winged_Snake/BP_Tether_Point.BP_Tether_Point_C")
      (bind _output_get (Variables|Default|SetImpact%20Point (.ImpactPoint (Collision|BreakHitResult _outhit))))
      (bind (_outhit_2 _returnvalue_4) (Collision|CapsuleTraceByChannel (- _output_get (* (Math|Vector|GetUnitDirection(Vector) (.TraceStart (Collision|BreakHitResult _outhit)) (.TraceEnd (Collision|BreakHitResult _outhit))) 2e+02)) _output_get (Components|Capsule|GetScaledCapsuleRadius _capsulecomponent) (Components|Capsule|GetScaledCapsuleHalfHeight _capsulecomponent) "TraceTypeQuery1" false (Utilities|Array|MakeArray (Components|GetOwner)) "None"))
      (if _returnvalue_4
        (return (.Location (Collision|BreakHitResult _outhit_2)) true)
        (else
          (return (.TraceEnd (Collision|BreakHitResult _outhit_2)) true)))
      (elif (Utilities|ClassIsChildOf (Utilities|GetClass (.HitActor (Collision|BreakHitResult _outhit))) "/Game/BluePrints/Spirits/Parent/BP_Spirit.BP_Spirit_C")
        (return (.ImpactPoint (Collision|BreakHitResult _outhit)) true)
        (else
          (return "0, 0, 0" false))))
    (else
      (return "0, 0, 0" false))))

(fn WingedSpiritSetup
  (bind _returnvalue (Game|GetPlayerController 0))
  (bind _asbp_iso_player_controller (Utilities|Casting|CastToBP_Iso_Player_Controller _returnvalue))
  (bind _returnvalue_2 (PlayerController|LocalPlayerSubsystems|GetEnhancedInputLocalPlayerSubsystem _asbp_iso_player_controller))
  (Utilities|IsValid _returnvalue_2
    (:Is%20Valid
      (Input|AddMappingContext _returnvalue_2 "/Game/Controls/Input_Actions/IMC_Iso_Player_Controls.IMC_Iso_Player_Controls" 0 "(bIgnoreAllPressedKeysUntilRelease=True,bForceImmediately=False)")
      (Variables|Default|SetAs%20BP%20Iso%20Player%20Character (.AsBP%20Iso%20Player%20Character (Utilities|Casting|CastToBP_Iso_PlayerCharacter (Game|GetPlayerCharacter 0)))))))

(fn WingedSpiritDash
  (bind _as_bp_iso_player_character (Variables|Default|GetAs%20BP%20Iso%20Player%20Character))
  (bind _returnvalue (Transformation|GetVelocity _as_bp_iso_player_character))
  (bind _returnvalue_2 (Math|Vector|MakeVector (.x _returnvalue) (.y _returnvalue) 0.0))
  (Audio|PlaySoundatLocation "/Game/Audio/AudioClips/SFX/phase2/snakedash.snakedash" (Transformation|GetActorLocation (Components|GetOwner)) "0, 0, 0" 1.0 1.0 0.0 "/Game/Audio/EnemyAtten.EnemyAtten" 0 0 0)
  (Development|PrintString "running winged")
  (if (!= (Variables|Default|GetDash_Used) 2)
    (if (Variables|Default|GetIf_Tethered)
      (Character|LaunchCharacter _as_bp_iso_player_character (* _returnvalue_2 1.2) false false)
      (Math|Integer|IncrementInt (Variables|Default|GetDash_Used)
        (:%20%20
          (CallFunction|ResetDash (Collision|MakeHitResult false false 0.0 0.0 "0, 0, 0" "0, 0, 0" "0,0,1" "0,0,1" 0 0))))
      (else
        (Character|LaunchCharacter _as_bp_iso_player_character (* _returnvalue_2 1e+01) false false)
        (Math|Integer|IncrementInt (Variables|Default|GetDash_Used)
          (:%20%20
            (CallFunction|ResetDash (Collision|MakeHitResult false false 0.0 0.0 "0, 0, 0" "0, 0, 0" "0,0,1" "0,0,1" 0 0))))))))

(fn CalculateTetherPlacement
  (bind _returnvalue (Components|GetOwner))
  (bind _end_location_of_tether (Variables|Default|GetEnd_Location_Of_Tether))
  (bind _returnvalue_2 (Transformation|GetActorLocation _returnvalue))
  (bind _returnvalue_3 (+ _returnvalue_2 _end_location_of_tether))
  (return (Math|Transform|MakeTransform _returnvalue_3 (Math|Conversions|RotationFromXVector (Math|Vector|GetUnitDirection(Vector) (Transformation|GetActorLocation (Components|GetOwner)) _returnvalue_3)) "1.000000,1.000000,1.000000")))

(fn UpdateDashDistance
  (params (Dash_Distance :type Float%20%28double-precision%29))
  (Variables|Default|SetTemp_Dash_Distance Dash_Distance)
  (Variables|Default|SetLast%20Index (Math|Float|Truncate (/ Dash_Distance (* (.OutRadius (Components|Capsule|GetScaledCapsuleSize (Variables|/Script/Engine.Character|GetCapsuleComponent (.AsBP%20Iso%20Player%20Character (Utilities|Casting|CastToBP_Iso_PlayerCharacter (Game|GetPlayerCharacter 0)))))) 2.4)))))

(fn SubtractTempDashDistance
  (Variables|Default|SetTemp_Dash_Distance (- (Variables|Default|GetTemp_Dash_Distance) (* (.OutRadius (Components|Capsule|GetScaledCapsuleSize (Variables|/Script/Engine.Character|GetCapsuleComponent (.AsBP%20Iso%20Player%20Character (Utilities|Casting|CastToBP_Iso_PlayerCharacter (Game|GetPlayerCharacter 0)))))) 2.4))))