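; BP_Winged_Snake is a collectible spirit that the player picks up by touching it.
; An actor overlap or Box hit from the player, if not yet attached, updates the current spirit, plays a collect sound and sets IsAttachedToPlayer.
; Both duplicated paths show WB_SpiritCollect with the spirit's name for a short delay.
; They then remove the widget and set IsSaved on the spirit's AI blackboard.
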(event OnComponentHit(Box)
  (params (HitComponent :type Primitive%20Component%20Object%20Reference) (OtherActor :type Actor%20Object%20Reference) (OtherComp :type Primitive%20Component%20Object%20Reference) (NormalImpulse :type Vector :default "0, 0, 0") (Hit :type Hit%20Result%20Structure%20%28by%20ref%29))
  (bind _returnvalue (Game|GetPlayerCharacter 0))
  (if (== OtherActor _returnvalue)
    (if (not (Variables|Default|GetIs_Attached_To_Player))
      (CallFunction|UpdateCurrentSpirit _returnvalue)
      (Audio|PlaySoundatLocation "/Game/Audio/AudioClips/SFX/spiritcollect.spiritcollect" (Transformation|GetActorLocation) "0, 0, 0" 1.0 1.0 0.0 0 0 0 0)
      (Variables|Default|SetIs_Attached_To_Player true)
      (bind _returnvalue_2 (UserInterface|CreateWidget "/Game/BluePrints/UI/WB_SpiritCollect.WB_SpiritCollect_C" (Game|GetPlayerController 0)))
      (UserInterface|Viewport|AddtoViewport _returnvalue_2 0)
      (Default|SpiritCollected _returnvalue_2 (Variables|Default|GetName_Of_Spirit))
      (Utilities|FlowControl|Delay 2.0)
      (Widget|RemovefromParent _returnvalue_2)
      (AI|Components|Blackboard|SetValueasBool (AI|GetBlackboard (AI|GetAIController self)) (Utilities|Name|MakeLiteralName "IsSaved") true))))

(event Custom|CustomEvent
  (params (OverlappedActor :type Actor%20Object%20Reference) (OtherActor :type Actor%20Object%20Reference))
  (if (== OtherActor (Game|GetPlayerCharacter 0))
    (if (not (Variables|Default|GetIs_Attached_To_Player))
      (CallFunction|UpdateCurrentSpirit OtherActor)
      (Audio|PlaySoundatLocation "/Game/Audio/AudioClips/SFX/spiritcollect.spiritcollect" (Transformation|GetActorLocation) "0, 0, 0" 1.0 1.0 0.0 0 0 0 0)
      (Variables|Default|SetIs_Attached_To_Player true)
      (bind _returnvalue (UserInterface|CreateWidget "/Game/BluePrints/UI/WB_SpiritCollect.WB_SpiritCollect_C" (Game|GetPlayerController 0)))
      (UserInterface|Viewport|AddtoViewport _returnvalue 0)
      (Default|SpiritCollected _returnvalue (Variables|Default|GetName_Of_Spirit))
      (Utilities|FlowControl|Delay 2.0)
      (Widget|RemovefromParent _returnvalue)
      (AI|Components|Blackboard|SetValueasBool (AI|GetBlackboard (AI|GetAIController self)) (Utilities|Name|MakeLiteralName "IsSaved") true))))

(event EventBeginPlay
  (|CallParentFunction)
  (Collision|BindEventtoOnActorBeginOverlap (EventDispatchers|CreateEvent :!event BindedSpiritContact)))

(event Collision|EventActorBeginOverlap
  (params (OtherActor :type Actor%20Object%20Reference))
  (|CallParentFunction OtherActor) ; This node is disabled and will not be called.\nDrag off pins to build functionality.
)

(event EventTick
  (params (DeltaSeconds :type Float%20%28single-precision%29))
  (|CallParentFunction DeltaSeconds) ; This node is disabled and will not be called.\nDrag off pins to build functionality.
)

(fn ConstructionScript
  (|CallParentFunction))