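; Winged snake player spirit Blueprint that animates its skeletal mesh along a spline path.
; While CanMove is set, Tick runs the movement, advancing the distance along the spline by SplineSpeed scaled by delta time.
; The mesh takes the spline's local-space location and rotation with fixed height and yaw offsets, keeping its own scale.
; When IsLooping is set, the distance resets to zero past the spline's end.
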(event Custom|Spirit_Movement
  (bind _skeletalmesh (Variables|Default|GetSkeletalMesh))
  (Variables|Default|SetDistance_Along_Spline (+ (* (Utilities|Time|GetWorldDeltaSeconds) (Variables|Default|GetSpline_Speed)) (Variables|Default|GetDistance_Along_Spline)))
  (Transformation|SetRelativeTransform _skeletalmesh (Math|Transform|MakeTransform (Math|Vector|MakeVector (.x (.location (Spline|GetTransformatDistanceAlongSpline (Variables|Default|GetSpline) (Variables|Default|GetDistance_Along_Spline) "Local" false))) (.y (.location (Spline|GetTransformatDistanceAlongSpline (Variables|Default|GetSpline) (Variables|Default|GetDistance_Along_Spline) "Local" false))) (+ (.z (.location (Spline|GetTransformatDistanceAlongSpline (Variables|Default|GetSpline) (Variables|Default|GetDistance_Along_Spline) "Local" false))) -89.0)) (Math|Rotator|MakeRotator (.roll (.rotation (Spline|GetTransformatDistanceAlongSpline (Variables|Default|GetSpline) (Variables|Default|GetDistance_Along_Spline) "Local" false))) (.pitch (.rotation (Spline|GetTransformatDistanceAlongSpline (Variables|Default|GetSpline) (Variables|Default|GetDistance_Along_Spline) "Local" false))) (+ (.yaw (.rotation (Spline|GetTransformatDistanceAlongSpline (Variables|Default|GetSpline) (Variables|Default|GetDistance_Along_Spline) "Local" false))) 9e+01)) (Variables|/Script/Engine.SceneComponent|GetRelativeScale3D _skeletalmesh)) false false)
  (if (Variables|Default|GetIsLooping)
    (if (> (Variables|Default|GetDistance_Along_Spline) (Spline|GetSplineLength (Variables|Default|GetSpline)))
      (Variables|Default|SetDistance_Along_Spline 0.0))))

(event EventBeginPlay)

(event Collision|EventActorBeginOverlap
  (params (OtherActor :type Actor%20Object%20Reference)))

(event EventTick
  (params (DeltaSeconds :type Float%20%28single-precision%29))
  (if (Variables|Default|GetCanMove)
    (CallFunction|SpiritMovement)))

(fn ConstructionScript)