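; Tether point for the Winged Snake spirit whose skeletal mesh can shuttle back and forth as a moving island.
; The construction script derives a target from a distance along a chosen world axis and scales timeline play rate by duration.
; If IsMoving is set, BeginPlay starts the timeline, which lerps the mesh between origin and target.
; An AtTop flag alternates forward and reverse playback after a short pause, looping endlessly.
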(event Custom|Restart_Timeline
  (bind _alpha (Timeline|Movement_Timeline Reverse)
    (:Update
      (Transformation|SetWorldLocation (Variables|Default|GetSkeletalMesh) (Math|Vector|Lerp(Vector) (Variables|Default|GetOriginal_Location) (Variables|Default|GetTarget_Location) _alpha) false false))
    (:Finished
      (Utilities|FlowControl|Delay 0.3)
      (if (Variables|Default|GetAtTop)
        (Variables|Default|SetAtTop false)
        (CallFunction|MoveIsland)
        (else
          (Variables|Default|SetAtTop true)
          (CallFunction|RestartTimeline))))))

(event Custom|Move_Island
  (if (and (Variables|Default|GetIsland_Touched) (not (Variables|Default|GetAtTop)))
    (bind _alpha (Timeline|Movement_Timeline PlayFromStart)
      (:Update
        (Transformation|SetWorldLocation (Variables|Default|GetSkeletalMesh) (Math|Vector|Lerp(Vector) (Variables|Default|GetOriginal_Location) (Variables|Default|GetTarget_Location) _alpha) false false))
      (:Finished
        (Utilities|FlowControl|Delay 0.3)
        (if (Variables|Default|GetAtTop)
          (Variables|Default|SetAtTop false)
          (CallFunction|MoveIsland)
          (else
            (Variables|Default|SetAtTop true)
            (CallFunction|RestartTimeline)))))))

(event EventBeginPlay
  (if (Variables|Default|GetIsMoving)
    (Variables|Default|SetIsland_Touched true)
    (CallFunction|MoveIsland)))

(event Collision|EventActorBeginOverlap
  (params (OtherActor :type Actor%20Object%20Reference)))

(event EventTick
  (params (DeltaSeconds :type Float%20%28single-precision%29)))

(fn ConstructionScript
  (Variables|Default|SetOriginal_Location (Transformation|GetWorldLocation (Variables|Default|GetSkeletalMesh)))
  (Components|Timeline|SetPlayRate (Variables|Default|GetMovement_Timeline) (/ 1.0 (Variables|Default|GetDuration)))
  (switch int (Variables|Default|GetMovement_Direction)
    (:0
      (Variables|Default|SetTarget_Location (Math|Vector|MakeVector (+ (.X (Class|KismetMathLibrary|BreakVector3f (Variables|Default|GetOriginal_Location))) (Variables|Default|GetMovement_Distance)) (.Y (Class|KismetMathLibrary|BreakVector3f (Variables|Default|GetOriginal_Location))) (.Z (Class|KismetMathLibrary|BreakVector3f (Variables|Default|GetOriginal_Location))))))
    (:1
      (Variables|Default|SetTarget_Location (Math|Vector|MakeVector (.X (Class|KismetMathLibrary|BreakVector3f (Variables|Default|GetOriginal_Location))) (+ (.Y (Class|KismetMathLibrary|BreakVector3f (Variables|Default|GetOriginal_Location))) (Variables|Default|GetMovement_Distance)) (.Z (Class|KismetMathLibrary|BreakVector3f (Variables|Default|GetOriginal_Location))))))
    (:2
      (Variables|Default|SetTarget_Location (Math|Vector|MakeVector (.X (Class|KismetMathLibrary|BreakVector3f (Variables|Default|GetOriginal_Location))) (.Y (Class|KismetMathLibrary|BreakVector3f (Variables|Default|GetOriginal_Location))) (+ (.Z (Class|KismetMathLibrary|BreakVector3f (Variables|Default|GetOriginal_Location))) (Variables|Default|GetMovement_Distance)))))))