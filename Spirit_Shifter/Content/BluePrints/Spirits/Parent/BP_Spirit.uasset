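; Collectible AI spirit whose type (snake, fish or beetle) sets its mesh, animation and the power component passed to the player on contact.
; It registers with a nearby combat manager and drives its AI through blackboard state and IsSaved keys.
; Attackers make it panic, with recursive delayed checks draining health while the nearest enemy is an attacker in range.
; Losing all health damages the player and destroys the spirit, sending attackers back to chasing.
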(event Custom|Binded_Spirit_Contact
  (params (OverlappedActor :type Actor%20Object%20Reference) (OtherActor :type Actor%20Object%20Reference))
  (if (== OtherActor (Game|GetPlayerCharacter 0))
    (if (not (Variables|Default|GetIs_Attached_To_Player))
      (CallFunction|UpdateCurrentSpirit OtherActor)
      (Audio|PlaySoundatLocation "/Game/Audio/AudioClips/SFX/spiritcollect.spiritcollect" (Transformation|GetActorLocation) "0, 0, 0" 1.0 1.0 0.0 0 0 0 0)
      (Variables|Default|SetIs_Attached_To_Player true)
      (bind _returnvalue (UserInterface|CreateWidget "/Game/BluePrints/UI/WB_SpiritCollect.WB_SpiritCollect_C" (Game|GetPlayerController 0)))
      (UserInterface|Viewport|AddtoViewport _returnvalue 0)
      (Default|SpiritCollected _returnvalue (Variables|Default|GetName_Of_Spirit))
      (Utilities|FlowControl|Delay 2.0)
      (Widget|RemovefromParent _returnvalue)
      (AI|Components|Blackboard|SetValueasBool (AI|GetBlackboard (AI|GetAIController self)) (Utilities|Name|MakeLiteralName "IsSaved") true))))

(event Custom|Release_Spirit
  (Variables|Default|SetIs_Attached_To_Player false))

(event Custom|Set_Begin_Follow_Player
  (Utilities|Time|SetTimerbyEvent (delegate Custom|Set_Pace) 0.2)
  (Variables|Default|SetMy_State "NewEnumerator0")
  (Default|CallOnUpdateAnimation))

(event Custom|Set_Pace
  (bind _returnvalue (Game|GetPlayerCharacter 0))
  (Variables|Default|SetPace (Math|Float|SelectFloat 1.0 1.2 (<= (Math|Float|Sign(Float) (Math|Vector|DotProduct (Math|Vector|GetUnitDirection(Vector) (Transformation|GetActorLocation) (Transformation|GetActorLocation _returnvalue)) (Transformation|GetActorForwardVector _returnvalue))) 0.0))))

(event Custom|ADAssign
  (for _array_element (Variables|Default|GetAttackers)
    (bind _asbp_ai (Utilities|Casting|CastToBP_AI _array_element))
    (EventDispatchers|AssignOnDeath _asbp_ai (delegate Custom|On_Attacker_Death_Event))
    (Class|BPIAttacker|Celebrate(Message) _array_element)))

(event Custom|On_Attacker_Death_Event
  (params (Actor :type Actor%20Object%20Reference))
  (Utilities|Array|RemoveItem (Variables|Default|GetAttackers) Actor)
  (CallFunction|CheckAttackers)
  (CallFunction|UpdateBlackBoard))

(event Custom|CheckAttackers
  (bind _attackers (Variables|Default|GetAttackers))
  (bind _returnvalue (Utilities|Array|Length _attackers))
  (if (>= _returnvalue 2)
    (Variables|Default|SetMy_State "NewEnumerator3")
    (Utilities|FlowControl|DelayUntilNextTick :!label _label)
    (Utilities|FlowControl|DoOnce false
      (:Completed
        (CallFunction|PanickTick)
        (AI|Components|Blackboard|SetValueasBool (AI|GetBlackboard (AI|GetAIController self)) (Utilities|Name|MakeLiteralName "IsSaved") false)))
    (elif (== _returnvalue 1)
      (Variables|Default|SetMy_State "NewEnumerator3")
      (goto _label)
      (else
        (Variables|Default|SetMy_State "NewEnumerator1")))))

(event Custom|UpdateBlackBoard
  (CallFunction|SetStateSpeed)
  (AI|Components|Blackboard|SetValueasEnum (AI|GetBlackboard (AI|GetAIController self)) (Utilities|Name|MakeLiteralName "SpiritState") (Variables|Default|GetMy_State))
  (Default|CallOnUpdateAnimation))

(event Custom|PanickTick
  (bind _outactors (Actor|GetAllActorsOfClass "/Game/BluePrints/AI/BP_AI.BP_AI_C"))
  (if (and (Utilities|Array|ContainsItem (Variables|Default|GetAttackers) (.ReturnValue (Actor|FindNearestActor (Transformation|GetActorLocation) _outactors))) (<= (.Distance (Actor|FindNearestActor (Transformation|GetActorLocation) _outactors)) 4e+02))
    (CallFunction|CheckAttackers)
    (Development|PrintString (Utilities|GetDisplayName self))
    (if (and (Variables|Default|GetcanTakeDamage) true)
      (Niagara|SpawnSystematLocation "/Game/BluePrints/Spirits/Parent/NS_SpiritDamage.NS_SpiritDamage" (Transformation|GetActorLocation) "0, 0, 0" "0.500000,0.500000,0.500000")
      (Audio|PlaySoundatLocation "/Game/Audio/AudioClips/SFX/spiritCry.spiritCry" (Transformation|GetActorLocation) "0, 0, 0" 1.75 1.0 0.0 "/Game/Audio/EnemyAtten.EnemyAtten" 0 0 0)
      (bind _output_get (Variables|Default|Sethealth (- (Variables|Default|Gethealth) 2.0)))
      (CallFunction|UpdateHealth _output_get)
      (if (<= _output_get 0.0)
        (Game|Damage|ApplyDamage (Game|GetPlayerCharacter 0) 1e+01 0 0)
        (Actor|DestroyActor)
        (else
          (Utilities|FlowControl|Sequence
            (:then_1
              (Utilities|FlowControl|Delay 2.0)
              (CallFunction|PanickTick))))))
    (else
      (for _array_element (Variables|Default|GetAttackers)
        (Class|BPIAttacker|Chase(Message) _array_element))
      (Utilities|Array|Clear (Variables|Default|GetAttackers))
      (Variables|Default|SetMy_State "NewEnumerator1")
      (CallFunction|UpdateBlackBoard)
      (Utilities|FlowControl|DoOnce false) ; enters at Reset
    )))

(event Custom|SetStateSpeed
  (switch Utilities|FlowControl|Switch|SwitchonSpiritStates (Variables|Default|GetMy_State)
    (:NewEnumerator3
      (Variables|/Script/Engine.CharacterMovementComponent|SetMaxCustomMovementSpeed (Variables|Character|GetCharacterMovement) 0.0))))

(event EventBeginPlay
  (CallFunction|SetBeginFollowPlayer)
  (Collision|BindEventtoOnActorBeginOverlap (EventDispatchers|CreateEvent :!event Custom|Binded_Spirit_Contact))
  (CallFunction|UpdateAnimationBP (Variables|Default|GetName_Of_Spirit))
  (Variables|Default|SetMy_State "NewEnumerator1")
  (CallFunction|UpdateBlackBoard)
  (bind _outactors (Actor|GetAllActorsOfClass "/Game/BluePrints/AI/Combat/BP_Combat_Manager.BP_Combat_Manager_C"))
  (bind _array_element (Utilities|Array|ForEachLoopwithBreak _outactors :!label _label)
    (:LoopBody
      (if (< (Math|Vector|Distance(Vector) (Transformation|GetActorLocation _array_element) (Transformation|GetActorLocation)) 6e+03)
        (bind _asbp_combat_manager (Utilities|Casting|CastToBP_Combat_Manager _array_element))
        (Default|AddSpirit _asbp_combat_manager self)
        (Utilities|Array|AddUnique (Variables|/Game/BluePrints/AI/Combat/BP_Combat_Manager.BP_Combat_Manager_C|GetSpirit_List _asbp_combat_manager) self)
        (goto _label Break)))))

(event Collision|EventActorBeginOverlap
  (params (OtherActor :type Actor%20Object%20Reference)))

(event EventTick
  (params (DeltaSeconds :type Float%20%28single-precision%29))
  (CallFunction|InterpWalkSpeed))

(event EventAddAttacker
  (params (NewAttacker :type Actor%20Object%20Reference))
  (Utilities|Array|AddUnique (Variables|Default|GetAttackers) NewAttacker)
  (Utilities|FlowControl|Sequence
    (:then_0
      (CallFunction|CheckAttackers))
    (:then_1
      (CallFunction|UpdateBlackBoard))
    (:then_2
      (CallFunction|ADAssign))))

(event EventDestroyed
  (Default|CallOnDeath)
  (for _array_element (Variables|Default|GetAttackers)
    (Class|BPIAttacker|Chase(Message) _array_element)))

(fn ConstructionScript
  (CallFunction|UpdateMesh (Variables|Default|GetName_Of_Spirit)))

(fn UpdateCurrentSpirit
  (params (Player_Character :type Actor%20Object%20Reference))
  (Utilities|IsValid (Actor|GetComponentbyClass Player_Character "/Game/BluePrints/Spirits/Parent/AC_Parent_Spirit.AC_Parent_Spirit_C")
    (:Is%20Valid
      (bind _asbp_iso_player_character (Utilities|Casting|CastToBP_Iso_PlayerCharacter Player_Character))
      (Default|CallUpdateCurrentSpirit _asbp_iso_player_character (Variables|Default|GetPower_Class))
      (Variables|/Game/BluePrints/Player/BP_Iso_PlayerCharacter.BP_Iso_PlayerCharacter_C|SetCurrent_Spirit _asbp_iso_player_character self)
      (Variables|Default|SetIs_Attached_To_Player true))))

(fn UpdateCurrentSpiritLocation
  (params (Player%20Character :type Actor%20Object%20Reference)))

(fn UpdateMesh
  (params (Name_of_Spirit :type String))
  (bind _mesh (Variables|Character|GetMesh))
  (switch string Name_of_Spirit
    (:Winged_Snake
      (Components|SkeletalMesh|SetSkeletalMeshAsset _mesh "/Game/Animations/Snake/Snake.Snake")
      (Variables|Default|SetPower_Class "/Game/BluePrints/Spirits/Winged_Snake/AC_Winged_Spirit.AC_Winged_Spirit_C"))
    (:Light_Fish
      (Components|SkeletalMesh|SetSkeletalMeshAsset _mesh "/Game/Animations/3D-Spirits/fish/Fishy.Fishy")
      (Variables|Default|SetPower_Class "/Game/BluePrints/Spirits/Light_Fish/AC_Light_Fish.AC_Light_Fish_C"))
    (:Rolling_Beetle
      (Components|SkeletalMesh|SetSkeletalMeshAsset _mesh "/Game/Animations/3D-Spirits/Beetle/Beetle.Beetle")
      (Variables|Default|SetPower_Class "/Game/BluePrints/Spirits/Rolling_Beetle/AC_Rolling_Beetle.AC_Rolling_Beetle_C")))
  (CallFunction|UpdateAnimationBP Name_of_Spirit))

(fn InterpWalkSpeed
  (bind _charactermovement (Variables|Character|GetCharacterMovement))
  (Variables|/Script/Engine.CharacterMovementComponent|SetMaxWalkSpeed _charactermovement (Math|Interpolation|FInterpTo (Variables|/Script/Engine.CharacterMovementComponent|GetMaxWalkSpeed _charactermovement) (* 5.9e+02 (Variables|Default|GetPace)) (Utilities|Time|GetWorldDeltaSeconds) 2.0)))

(fn ClearAnimBools
  (Variables|Default|SetMy_State "NewEnumerator0")
  (Default|CallOnUpdateAnimation)
  (return))

(fn UpdateAnimationBP
  (params (NameOfSpirit :type String))
  (bind _mesh (Variables|Character|GetMesh))
  (Components|Animation|SetAnimationMode (Variables|Character|GetMesh) "AnimationBlueprint")
  (switch string NameOfSpirit
    (:Winged_Snake
      (Class|SkeletalMeshComponent|SetAnimClass _mesh "/Game/Animations/Snake/AB_NewSnake.AB_NewSnake_C"))
    (:Light_Fish
      (Class|SkeletalMeshComponent|SetAnimClass _mesh "/Game/Animations/3D-Spirits/fish/AB_NewFish.AB_NewFish_C"))
    (:Rolling_Beetle
      (Class|SkeletalMeshComponent|SetAnimClass _mesh "/Game/Animations/3D-Spirits/Beetle/AB_Beetle.AB_Beetle_C"))))

(fn UpdateHealth
  (params (Health :type Float%20%28double-precision%29))
  (Rendering|Material|SetScalarParameterValueonMaterials (Variables|Character|GetMesh) "Position" (Math|Float|Lerp 0.0 3.0 (/ Health 15.0)))
  (Development|PrintString (Utilities|String|ToString(Float) Health)))

(fn CanbeAttacked
  (for _array_element (Variables|Default|GetAttackers)
    (Utilities|IsValid _array_element
      (:Is%20Not%20Valid
        (Utilities|Array|RemoveItem (Variables|Default|GetAttackers) _array_element))))
  (if (< (Utilities|Array|Length (Variables|Default|GetAttackers)) (- (Variables|Default|GetmaxAttackers) 1))
    (return true)
    (else
      (return false))))

(fn GetMaxAttackers
  (return (Variables|Default|GetmaxAttackers)))