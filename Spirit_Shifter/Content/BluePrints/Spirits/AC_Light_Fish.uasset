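; Light Fish spirit ability component for the isometric player character, implementing only the winged spirit level mechanic.
; The mechanic runs a debug-drawn visibility line trace from the player mesh along its forward vector, scaled by a distance multiplier.
; It stores the impact point, sets the tethered flag and switches the character to flying without checking for a hit.
; Dash and projectile events are empty stubs.
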(event Custom|Use_Current_Spirit_Projectile)

(event Custom|Use_Current_Spirit_Dash)

(event Custom|Use_Winged_Spirit_Level_Mechanic
  (bind _returnvalue (Game|GetPlayerCharacter 0))
  (bind _asbp_iso_player_character (Utilities|Casting|CastToBP_Iso_PlayerCharacter _returnvalue))
  (bind _mesh (Variables|/Script/Engine.Character|GetMesh _asbp_iso_player_character))
  (bind _returnvalue_2 (Transformation|GetWorldTransform _mesh))
  (bind _outhit (Collision|LineTraceByChannel (.location _returnvalue_2) (+ (.location _returnvalue_2) (* (Math|Vector|GetForwardVector (.rotation _returnvalue_2)) (Variables|Default|GetDistance_Multipler))) "TraceTypeQuery1" false 0 "ForDuration"))
  (Variables|Default|SetImpact%20Point (.ImpactPoint (Collision|BreakHitResult _outhit)))
  (Variables|Default|SetIf_Tethered true)
  (Pawn|Components|CharacterMovement|SetMovementMode (Variables|/Script/Engine.Character|GetCharacterMovement _asbp_iso_player_character) "MOVE_Flying" 0))

(event EventBeginPlay)

(event EventTick
  (params (DeltaSeconds :type Float%20%28single-precision%29)))