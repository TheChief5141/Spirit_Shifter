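; Rock projectile for the Rolling Beetle spirit that temporarily immobilizes units it touches.
; When its Sphere overlaps a BP_UnitStats actor other than player character 0, it disables that unit's character movement, then restores Walking mode after a five-second Delay.
; A single Delay serves every overlap, so hits during the wait share one timer rather than each getting their own.
; The graph applies no damage and never destroys the projectile.
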(event OnComponentBeginOverlap(Sphere)
  (params (OverlappedComponent :type Primitive%20Component%20Object%20Reference) (OtherActor :type Actor%20Object%20Reference) (OtherComp :type Primitive%20Component%20Object%20Reference) (OtherBodyIndex :type Integer) (bFromSweep :type Boolean) (SweepResult :type Hit%20Result%20Structure%20%28by%20ref%29))
  (bind _asbp_unit_stats (Utilities|Casting|CastToBP_UnitStats OtherActor))
  (bind _charactermovement (Variables|/Script/Engine.Character|GetCharacterMovement _asbp_unit_stats))
  (if (and (Utilities|ClassIsChildOf (Utilities|GetClass OtherActor) "/Game/BluePrints/AI/BP_UnitStats.BP_UnitStats_C") (!= OtherActor (Game|GetPlayerCharacter 0)))
    (Pawn|Components|CharacterMovement|DisableMovement _charactermovement)
    (Utilities|FlowControl|Delay 5.0)
    (Pawn|Components|CharacterMovement|SetMovementMode _charactermovement "MOVE_Walking" 0)))

(event EventBeginPlay)

(event Collision|EventActorBeginOverlap
  (params (OtherActor :type Actor%20Object%20Reference)))

(event EventTick
  (params (DeltaSeconds :type Float%20%28single-precision%29)))

(fn ConstructionScript)