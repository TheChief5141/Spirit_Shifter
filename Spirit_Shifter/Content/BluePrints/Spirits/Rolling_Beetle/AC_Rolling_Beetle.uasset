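; Actor component for the Rolling Beetle spirit's input-driven abilities: dash stun, projectile and ground wall placement.
; BeginPlay adds the Enhanced Input mapping; the dash event sphere-traces around the owner to briefly disable BP_UnitStats movement.
; The projectile event spawns at capsule base along flattened camera forward.
; The level action camera-traces, falling back to a downward trace, and relocates the existing BP_Ground_Wall onto island-material surfaces, toggling it around the move.
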(event Custom|Beetle_Projectile
  (bind _returnvalue (Game|GetPlayerController 0))
  (bind _returnvalue_2 (Components|GetOwner))
  (bind _returnvalue_3 (Transformation|GetActorTransform _returnvalue_2))
  (bind _playercameramanager (Variables|/Script/Engine.PlayerController|GetPlayerCameraManager _returnvalue))
  (bind _returnvalue_4 (Transformation|GetActorForwardVector _playercameramanager))
  (bind (_x _y) (Class|KismetMathLibrary|BreakVector3f _returnvalue_4))
  (Audio|PlaySoundatLocation "/Game/Audio/AudioClips/SFX/phase2/beetleprojectile.beetleprojectile" (Transformation|GetActorLocation _returnvalue_2) "0, 0, 0" 1.0 1.0 0.0 "/Game/Audio/EnemyAtten.EnemyAtten" 0 0 0)
  (Game|SpawnActorfromClass "/Game/BluePrints/Spirits/Rolling_Beetle/BP_RollingBeetle_Projectile.BP_RollingBeetle_Projectile_C" (Math|Transform|MakeTransform (Math|Vector|MakeVector (.x (.location _returnvalue_3)) (.y (.location _returnvalue_3)) (- (.z (.location _returnvalue_3)) (Components|Capsule|GetScaledCapsuleHalfHeight (Variables|/Script/Engine.Character|GetCapsuleComponent (.AsCharacter (Utilities|Casting|CastToCharacter (Variables|/Script/Engine.Actor|GetInstigator _returnvalue_2))))))) (Math|Conversions|RotationFromXVector (Math|Vector|MakeVector _x _y 0.0)) (.scale _returnvalue_3)) "Undefined" "MultiplyWithRoot" 0 0))

(event Custom|Beetle_Dash
  (bind _returnvalue (Components|GetOwner))
  (bind _returnvalue_2 (Transformation|GetActorLocation _returnvalue))
  (Audio|PlaySoundatLocation "/Game/Audio/AudioClips/SFX/phase2/beetledash.beetledash" _returnvalue_2 "0, 0, 0" 1.0 1.0 0.0 "/Game/Audio/EnemyAtten.EnemyAtten" 0 0 0)
  (Utilities|FlowControl|Delay 0.2)
  (bind (_outhits _returnvalue_3) (Collision|MultiSphereTraceByChannel _returnvalue_2 _returnvalue_2 (Variables|Default|GetStun_Radius) "TraceTypeQuery1" false 0 "ForDuration"))
  (if _returnvalue_3
    (for _array_element _outhits
      (if (Utilities|ClassIsChildOf (Utilities|GetClass (.HitActor (Collision|BreakHitResult _array_element))) "/Game/BluePrints/AI/BP_UnitStats.BP_UnitStats_C")
        (Pawn|Components|CharacterMovement|DisableMovement (Variables|/Script/Engine.Character|GetCharacterMovement (.AsBP%20Unit%20Stats (Utilities|Casting|CastToBP_UnitStats (.HitActor (Collision|BreakHitResult _array_element))))))
        (Utilities|FlowControl|Delay 3.0)
        (Pawn|Components|CharacterMovement|SetMovementMode (Variables|/Script/Engine.Character|GetCharacterMovement (.AsBP%20Unit%20Stats (Utilities|Casting|CastToBP_UnitStats (.HitActor (Collision|BreakHitResult _array_element))))) "MOVE_Walking" 0)))))

(event Input|EnhancedActionEvents|EnhancedInputActionIA_Dash
  (params (ActionValue :type Boolean) (ElapsedSeconds :type Float%20%28double-precision%29) (TriggeredSeconds :type Float%20%28double-precision%29) (InputAction :type Input%20Action%20Object%20Reference :default "/Game/Controls/Input_Actions/IA_Dash.IA_Dash"))
  (:Started
    (CallFunction|BeetleDash)))

(event Input|EnhancedActionEvents|EnhancedInputActionIA_Projectile
  (params (ActionValue :type Boolean) (ElapsedSeconds :type Float%20%28double-precision%29) (TriggeredSeconds :type Float%20%28double-precision%29) (InputAction :type Input%20Action%20Object%20Reference :default "/Game/Controls/Input_Actions/IA_Projectile.IA_Projectile"))
  (:Started
    (CallFunction|BeetleProjectile)))

(event Input|EnhancedActionEvents|EnhancedInputActionIA_Spirit_LevelAction
  (params (ActionValue :type Boolean) (ElapsedSeconds :type Float%20%28double-precision%29) (TriggeredSeconds :type Float%20%28double-precision%29) (InputAction :type Input%20Action%20Object%20Reference :default "/Game/Controls/Input_Actions/IA_Spirit_LevelAction.IA_Spirit_LevelAction"))
  (bind _returnvalue (Game|GetPlayerController 0))
  (bind _returnvalue_2 (Components|GetOwner))
  (bind _array (Utilities|Array|MakeArray _returnvalue_2))
  (bind _playercameramanager (Variables|/Script/Engine.PlayerController|GetPlayerCameraManager _returnvalue))
  (bind _returnvalue_3 (Transformation|GetActorLocation _playercameramanager))
  (:Started
    (bind (_outhit _returnvalue_4) (Collision|SphereTraceByChannel _returnvalue_3 (+ _returnvalue_3 (* (Transformation|GetActorForwardVector _playercameramanager) (Variables|Default|GetDistance_Multipler))) 2e+01 "TraceTypeQuery1" true _array "ForDuration"))
    (if _returnvalue_4
      (if (== (.ReturnValue (Class|PrimitiveComponent|GetMaterialfromCollisionFaceIndex (.HitComponent (Collision|BreakHitResult _outhit)) (.ElementIndex (Collision|BreakHitResult _outhit)))) "/Game/Models/Island/IslandMAT_Inst.IslandMAT_Inst")
        (bind _returnvalue_5 (Actor|GetActorOfClass "/Game/BluePrints/Spirits/Rolling_Beetle/BP_Ground_Wall.BP_Ground_Wall_C"))
        (Default|ToggleState _returnvalue_5 false)
        (Utilities|FlowControl|Delay 0.5)
        (Transformation|SetActorLocationAndRotation _returnvalue_5 (- (.Location (Collision|BreakHitResult _outhit)) "0.000000,0.000000,200.000000") (Math|Conversions|RotationFromXVector (Math|Vector|ProjectVectorontoPlane (.Normal (Collision|BreakHitResult _outhit)) "0.000000,0.000000,1.000000")) false true)
        (Default|ToggleState _returnvalue_5 true))
      (else
        (bind (_outhit_2 _returnvalue_6) (Collision|LineTraceByChannel (.TraceEnd (Collision|BreakHitResult _outhit)) (- (.TraceEnd (Collision|BreakHitResult _outhit)) (Math|Vector|MakeVector 0.0 0.0 (Variables|Default|GetDistance_Multipler))) "TraceTypeQuery1" true _array "ForDuration"))
        (if _returnvalue_6
          (if (== (.ReturnValue (Class|PrimitiveComponent|GetMaterialfromCollisionFaceIndex (.HitComponent (Collision|BreakHitResult _outhit_2)) (.ElementIndex (Collision|BreakHitResult _outhit_2)))) "/Game/Models/Island/IslandMAT_Inst.IslandMAT_Inst")
            (bind _returnvalue_7 (Actor|GetActorOfClass "/Game/BluePrints/Spirits/Rolling_Beetle/BP_Ground_Wall.BP_Ground_Wall_C"))
            (Default|ToggleState _returnvalue_7 false)
            (Utilities|FlowControl|Delay 0.5)
            (Transformation|SetActorLocationAndRotation _returnvalue_7 (- (.Location (Collision|BreakHitResult _outhit_2)) "0.000000,0.000000,200.000000") (Math|Conversions|RotationFromXVector (Math|Vector|ProjectVectorontoPlane (.Normal (Collision|BreakHitResult _outhit_2)) "0.000000,0.000000,1.000000")) false true)
            (Default|ToggleState _returnvalue_7 true)))))))

(event EventBeginPlay
  (CallFunction|SetupRollingBeetle)
  (Variables|Default|SetDash_Distance 8e+02))

(event EventTick
  (params (DeltaSeconds :type Float%20%28single-precision%29)))

(fn SetupRollingBeetle
  (bind _returnvalue (Game|GetPlayerController 0))
  (bind _asbp_iso_player_controller (Utilities|Casting|CastToBP_Iso_Player_Controller _returnvalue))
  (bind _returnvalue_2 (PlayerController|LocalPlayerSubsystems|GetEnhancedInputLocalPlayerSubsystem _asbp_iso_player_controller))
  (Utilities|IsValid _returnvalue_2
    (:Is%20Valid
      (Input|AddMappingContext _returnvalue_2 "/Game/Controls/Input_Actions/IMC_Iso_Player_Controls.IMC_Iso_Player_Controls" 0 "(bIgnoreAllPressedKeysUntilRelease=True,bForceImmediately=False)"))))