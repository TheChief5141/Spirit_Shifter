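; BP_Ground_Wall is a ground wall actor in the Rolling Beetle spirit folder that slides its mesh vertically.
; On BeginPlay it plays the Wall_Enter timeline, which lerps the static mesh's relative Z from zero to DownMultiplier.
; ToggleState plays that entrance from the start when on, or reverses the timeline to undo it when off.
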(event Custom|Wall_Exit
  (bind _staticmesh (Variables|Default|GetStaticMesh))
  (bind _relativelocation (Variables|/Script/Engine.SceneComponent|GetRelativeLocation _staticmesh))
  (bind _location (Timeline|Wall_Enter Reverse)
    (:Update
      (Transformation|SetRelativeLocation _staticmesh (Math|Vector|MakeVector (.x _relativelocation) (.y _relativelocation) (Math|Float|Lerp 0.0 (Variables|Default|GetDownMultiplier) _location)) false false))))

(event Custom|Wall_Entrance
  (bind _staticmesh (Variables|Default|GetStaticMesh))
  (bind _relativelocation (Variables|/Script/Engine.SceneComponent|GetRelativeLocation _staticmesh))
  (bind _location (Timeline|Wall_Enter PlayFromStart)
    (:Update
      (Transformation|SetRelativeLocation _staticmesh (Math|Vector|MakeVector (.x _relativelocation) (.y _relativelocation) (Math|Float|Lerp 0.0 (Variables|Default|GetDownMultiplier) _location)) false false))))

(event EventBeginPlay
  (CallFunction|WallEntrance))

(event Collision|EventActorBeginOverlap
  (params (OtherActor :type Actor%20Object%20Reference)))

(event EventTick
  (params (DeltaSeconds :type Float%20%28single-precision%29)))

(event EventToggleState
  (params (On/Off :type Boolean))
  (if On/Off
    (CallFunction|WallEntrance)
    (else
      (CallFunction|WallExit))))

(fn ConstructionScript)