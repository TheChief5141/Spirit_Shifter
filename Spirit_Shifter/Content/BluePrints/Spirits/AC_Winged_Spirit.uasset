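; Winged Spirit ability component for the isometric player character, providing a tether swing, dash and projectile effect.
; Holding Level Action traces forward for a tether point, spawns a cable and switches to Flying; Tick applies force toward the anchor, biased by sideways input.
; Dash launches along horizontal velocity, weaker while tethered, with two charges restored after a grounded delay.
; Projectile input only spawns a short-lived Niagara effect, with no hit logic.
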(event Custom|Use_Winged_Spirit_Level_Mechanic)

(event Custom|Reset_Dash
  (params (Hit :type Hit%20Result%20Structure%20%28by%20ref%29))
  (Utilities|FlowControl|Delay 0.01)
  (if (== (Variables|Default|GetDash_Used) 2)
    (if (not (AI|Components|NavMovement|IsFalling (Variables|/Script/Engine.Character|GetCharacterMovement (Variables|Default|GetAs%20BP%20Iso%20Player%20Character))))
      (Utilities|FlowControl|Delay 2.0)
      (Variables|Default|SetDash_Used 0))))

(event Input|EnhancedActionEvents|EnhancedInputActionIA_Projectile
  (params (ActionValue :type Boolean) (ElapsedSeconds :type Float%20%28double-precision%29) (TriggeredSeconds :type Float%20%28double-precision%29) (InputAction :type Input%20Action%20Object%20Reference :default "/Game/Controls/Input_Actions/IA_Projectile.IA_Projectile"))
  (bind _as_bp_iso_player_character (Variables|Default|GetAs%20BP%20Iso%20Player%20Character))
  (:Started
    (bind _returnvalue (Game|AddComponentbyClass _as_bp_iso_player_character "/Script/Niagara.NiagaraComponent" false (Transformation|GetRelativeTransform (Variables|/Game/BluePrints/Player/BP_Iso_PlayerCharacter.BP_Iso_PlayerCharacter_C|GetSpirit_Transform _as_bp_iso_player_character))))
    (Class|NiagaraComponent|SetAsset _returnvalue (Variables|Default|GetProjectile_Niagara_System) true)
    (Utilities|FlowControl|Delay 1.2)
    (Components|DestroyComponent _returnvalue)))

(event Input|EnhancedActionEvents|EnhancedInputActionIA_Level_Action
  (params (ActionValue :type Boolean) (ElapsedSeconds :type Float%20%28double-precision%29) (TriggeredSeconds :type Float%20%28double-precision%29) (InputAction :type Input%20Action%20Object%20Reference :default "/Game/Controls/Input_Actions/IA_Level_Action.IA_Level_Action"))
  (bind _as_bp_iso_player_character (Variables|Default|GetAs%20BP%20Iso%20Player%20Character))
  (bind _capsulecomponent (Variables|/Script/Engine.Character|GetCapsuleComponent _as_bp_iso_player_character))
  (bind _returnvalue (Transformation|GetWorldLocation _capsulecomponent))
  (:Started
    (bind (_outhit _returnvalue_2) (Collision|LineTraceByChannel _returnvalue (+ _returnvalue (* (Math|Vector|GetForwardVector (Transformation|GetWorldRotation _capsulecomponent)) (Variables|Default|GetDistance_Multipler))) "TraceTypeQuery1" false 0 "ForDuration"))
    (if _returnvalue_2
      (if (Utilities|ClassIsChildOf (Utilities|GetClass (.HitActor (Collision|BreakHitResult _outhit))) "/Game/BluePrints/Spirits/Winged_Snake/BP_Tether_Point.BP_Tether_Point_C")
        (Variables|Default|SetImpact%20Point (.ImpactPoint (Collision|BreakHitResult _outhit)))
        (bind _returnvalue_3 (Game|AddComponentbyClass _as_bp_iso_player_character "/Script/CableComponent.CableComponent" false (Transformation|GetRelativeTransform (Variables|/Script/Engine.Character|GetMesh (Variables|Default|GetAs%20BP%20Iso%20Player%20Character)))))
        (Pawn|Components|CharacterMovement|SetMovementMode (Variables|/Script/Engine.Character|GetCharacterMovement _as_bp_iso_player_character) "MOVE_Flying" 0)
        (bind _output_get (Variables|Default|SetCable_Component _returnvalue_3))
        (Rendering|SetVisibility _output_get true false)
        (Rendering|Material|SetMaterial _output_get 0 "/Game/Megascans/Surfaces/White_Cotton_Rope_umjmccocw/MI_White_Cotton_Rope_umjmccocw_2K.MI_White_Cotton_Rope_umjmccocw_2K")
        (Variables|Default|SetIf_Tethered true))))
  (:Completed
    (if (Variables|Default|GetIf_Tethered)
      (Variables|Default|SetIf_Tethered false)
      (Rendering|SetVisibility (Variables|Default|GetCable_Component) false false)
      (Components|DestroyComponent (Variables|Default|GetCable_Component))
      (Pawn|Components|CharacterMovement|SetMovementMode (Variables|/Script/Engine.Character|GetCharacterMovement (Variables|Default|GetAs%20BP%20Iso%20Player%20Character)) "MOVE_Walking" 0))))

(event Input|EnhancedActionEvents|EnhancedInputActionIA_Dash
  (params (ActionValue :type Boolean) (ElapsedSeconds :type Float%20%28double-precision%29) (TriggeredSeconds :type Float%20%28double-precision%29) (InputAction :type Input%20Action%20Object%20Reference :default "/Game/Controls/Input_Actions/IA_Dash.IA_Dash"))
  (bind _as_bp_iso_player_character (Variables|Default|GetAs%20BP%20Iso%20Player%20Character))
  (bind _returnvalue (Transformation|GetVelocity _as_bp_iso_player_character))
  (bind _returnvalue_2 (Math|Vector|MakeVector (.x _returnvalue) (.y _returnvalue) 0.0))
  (:Started
    (if (!= (Variables|Default|GetDash_Used) 2)
      (if (Variables|Default|GetIf_Tethered)
        (Character|LaunchCharacter _as_bp_iso_player_character (* _returnvalue_2 1.2) false false)
        (Math|Integer|IncrementInt (Variables|Default|GetDash_Used)
          (:%20%20
            (CallFunction|ResetDash (Collision|MakeHitResult false false 0.0 0.0 "0, 0, 0" "0, 0, 0" "0,0,1" "0,0,1" 0 0))))
        (else
          (Character|LaunchCharacter _as_bp_iso_player_character (* _returnvalue_2 1e+01) false false)
          (Math|Integer|IncrementInt (Variables|Default|GetDash_Used)
            (:%20%20
              (CallFunction|ResetDash (Collision|MakeHitResult false false 0.0 0.0 "0, 0, 0" "0, 0, 0" "0,0,1" "0,0,1" 0 0)))))))))

(event EventBeginPlay
  (bind _asbp_iso_player_controller (Utilities|Casting|CastToBP_Iso_Player_Controller (Pawn|GetController (Variables|/Script/Engine.Actor|GetInstigator (Components|GetOwner)))))
  (Utilities|IsValid (PlayerController|LocalPlayerSubsystems|GetEnhancedInputLocalPlayerSubsystem _asbp_iso_player_controller)
    (:Is%20Valid
      (Input|AddMappingContext (PlayerController|LocalPlayerSubsystems|GetEnhancedInputLocalPlayerSubsystem _asbp_iso_player_controller) "/Game/Controls/Input_Actions/IMC_Iso_Player_Controls.IMC_Iso_Player_Controls" 0 "(bIgnoreAllPressedKeysUntilRelease=True,bForceImmediately=False)")
      (bind _output_get (Variables|Default|SetAs%20BP%20Iso%20Player%20Character (.AsBP%20Iso%20Player%20Character (Utilities|Casting|CastToBP_Iso_PlayerCharacter (Components|GetOwner)))))
      (EventDispatchers|BindEventtoLandedDelegate _output_get (EventDispatchers|CreateEvent :!event Custom|Reset_Dash)))))

(event EventTick
  (params (DeltaSeconds :type Float%20%28single-precision%29))
  (bind _returnvalue (Components|GetOwner))
  (bind _asbp_iso_player_character (Utilities|Casting|CastToBP_Iso_PlayerCharacter _returnvalue))
  (if (Variables|Default|GetIf_Tethered)
    (Variables|/Script/CableComponent.CableComponent|SetEndLocation (Variables|Default|GetCable_Component) (Math|Transform|InverseTransformLocation (Transformation|GetActorTransform _asbp_iso_player_character) (Variables|Default|GetImpact%20Point)))
    (Physics|AddForce (Variables|/Script/Engine.Character|GetCharacterMovement (Variables|Default|GetAs%20BP%20Iso%20Player%20Character)) (* (Math|Vector|Normalize (+ (Math|Vector|GetUnitDirection(Vector) (Transformation|GetActorLocation _asbp_iso_player_character) (Variables|Default|GetImpact%20Point)) (* (* (Transformation|GetActorRightVector _asbp_iso_player_character) (.x (Input|EnhancedActionValues|GetIA_Move))) 0.7))) 2.5e+05))))