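; Collectible spirit pawn that, on player overlap, hands its power to the player and becomes the current spirit, replacing the previous one.
; NameOfSpirit selects the Winged Snake, Light Fish or Rolling Beetle mesh, and the construction script also sets the matching component reference.
; Once attached, it follows through a repeating AI MoveTo loop, holding position when near the player, until Release_Spirit clears the attachment.
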(event OnComponentBeginOverlap(Box)
  (params (OverlappedComponent :type Primitive%20Component%20Object%20Reference) (OtherActor :type Actor%20Object%20Reference) (OtherComp :type Primitive%20Component%20Object%20Reference) (OtherBodyIndex :type Integer) (bFromSweep :type Boolean) (SweepResult :type Hit%20Result%20Structure%20%28by%20ref%29))
  (if (== OtherActor (Game|GetPlayerCharacter 0))
    (if (not (Variables|Default|GetIs_Attached_To_Player))
      (CallFunction|UpdateCurrentSpirit OtherActor)
      (Audio|PlaySoundatLocation "/Game/Audio/AudioClips/SFX/spiritcollect.spiritcollect" (Transformation|GetActorLocation) "0, 0, 0" 1.0 1.0 0.0 0 0 0 0)
      (CallFunction|FollowPlayer OtherActor))))

(event Custom|Follow_Player
  (params (Player_Character :type Actor%20Object%20Reference))
  (bind _self self)
  (if (Variables|Default|GetIs_Attached_To_Player)
    (if (>= (Transformation|GetDistanceTo self Player_Character) 2e+02)
      (AI|AIMoveTo self "0, 0, 0" (Game|GetPlayerCharacter 0) 5.0 false
        (:then
          _))
      (else
        (AI|AIMoveTo _self "0, 0, 0" _self 5.0 false
          (:then
            _))))
    (Utilities|FlowControl|Delay 0.2)
    (CallFunction|FollowPlayer (Game|GetPlayerCharacter 0))))

(event Custom|Release_Spirit
  (Variables|Default|SetIs_Attached_To_Player false))

(event EventBeginPlay
  (CallFunction|UpdateMesh (Variables|Default|GetName_Of_Spirit)))

(event Collision|EventActorBeginOverlap
  (params (OtherActor :type Actor%20Object%20Reference)))

(event EventTick
  (params (DeltaSeconds :type Float%20%28single-precision%29)))

(fn ConstructionScript
  (bind _mesh (Variables|Character|GetMesh))
  (switch string (Variables|Default|GetName_Of_Spirit)
    (:Winged_Snake
      (Components|SkeletalMesh|SetSkeletalMeshAsset _mesh "/Game/Animations/3D-Spirits/WingedSerpent/WingedSerpent_Idle.WingedSerpent_Idle")
      (Variables|Default|SetAC_Reference "/Game/BluePrints/Spirits/Winged_Snake/AC_Winged_Spirit.AC_Winged_Spirit_C"))
    (:Light_Fish
      (Components|SkeletalMesh|SetSkeletalMeshAsset _mesh "/Game/Animations/3D-Spirits/fish/Fish_Idle01.Fish_Idle01")
      (Variables|Default|SetAC_Reference "/Game/BluePrints/Spirits/Light_Fish/AC_Light_Fish.AC_Light_Fish_C"))
    (:Rolling_Beetle
      (Components|SkeletalMesh|SetSkeletalMeshAsset _mesh "/Game/Animations/3D-Spirits/Beetle/Beetle_Idle.Beetle_Idle")
      (Variables|Default|SetAC_Reference "/Game/BluePrints/Spirits/Rolling_Beetle/AC_Rolling_Beetle.AC_Rolling_Beetle_C"))))

(fn UpdateCurrentSpirit
  (params (Player_Character :type Actor%20Object%20Reference))
  (Utilities|IsValid (Actor|GetComponentbyClass Player_Character "/Game/BluePrints/Spirits/AC_Parent_Spirit.AC_Parent_Spirit_C")
    (:Is%20Valid
      (bind _asbp_iso_player_character (Utilities|Casting|CastToBP_Iso_PlayerCharacter Player_Character))
      (Default|RemoveSpirit _asbp_iso_player_character)
      (Default|AddSpirit _asbp_iso_player_character (Variables|Default|GetPower_Class))
      (Variables|/Game/BluePrints/Player/BP_Iso_PlayerCharacter.BP_Iso_PlayerCharacter_C|SetCurrent_Spirit _asbp_iso_player_character self)
      (Variables|Default|SetIs_Attached_To_Player true))))

(fn UpdateCurrentSpiritLocation
  (params (Player%20Character :type Actor%20Object%20Reference)))

(fn UpdateMesh
  (params (Name_of_Spirit :type String))
  (bind _mesh (Variables|Character|GetMesh))
  (switch string Name_of_Spirit
    (:Winged_Snake
      (Components|SkeletalMesh|SetSkeletalMeshAsset _mesh "/Game/Animations/3D-Spirits/WingedSerpent/WingedSerpent_Idle.WingedSerpent_Idle"))
    (:Light_Fish
      (Components|SkeletalMesh|SetSkeletalMeshAsset _mesh "/Game/Animations/3D-Spirits/fish/Fish_Idle01.Fish_Idle01"))
    (:Rolling_Beetle
      (Components|SkeletalMesh|SetSkeletalMeshAsset _mesh "/Game/Animations/3D-Spirits/Beetle/Beetle_Idle.Beetle_Idle"))))