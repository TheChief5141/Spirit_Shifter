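; Game manager that reacts when checkpoint spirits are saved, updating points of interest and spirit totems.
; The construction script pairs parallel arrays into maps from each checkpoint to its POI and totem, binding to spirit-saved events.
; On a save, it destroys the matching POI, increments the GameInstance checkpoint threshold, and calls CanInteract on the totem, or on every totem in its group if grouped.
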(event Custom|Checkpoint_Saved_Spirit
  (params (Saved_Spirit :type BP%20LVL%20Wind%20Spirit%20Object%20Reference))
  (bind _spirittotems_checkpoint_map (Variables|Default|GetSpiritTotems_Checkpoint_Map))
  (bind _value (Utilities|Map|Find _spirittotems_checkpoint_map Saved_Spirit))
  (Actor|DestroyActor (.Value (Utilities|Map|Find (Variables|Default|GetPOI_Checkpoint_Map) Saved_Spirit)))
  (Default|CheckpointThresholdIncrement (Variables|Default|GetAs%20GI%20Spirit%20Shifter))
  (if (Variables|/Game/BluePrints/Environment/Interactables/BP_Checkpoint.BP_Checkpoint_C|GetInGroup? _value)
    (for _array_element (Variables|/Game/BluePrints/Environment/Interactables/BP_Checkpoint.BP_Checkpoint_C|GetGrouped_Checkpoints _value)
      (Default|CanInteract _array_element))
    (else
      (Default|CanInteract _value))))

(event EventBeginPlay
  (Variables|Default|SetAs%20BP%20Iso%20Player%20Character (.AsBP%20Iso%20Player%20Character (Utilities|Casting|CastToBP_Iso_PlayerCharacter (Game|GetPlayerCharacter 0))))
  (Variables|Default|SetAs%20GI%20Spirit%20Shifter (.AsGI%20Spirit%20Shifter (Utilities|Casting|CastToGI_Spirit_Shifter (Game|GetGameInstance)))))

(fn ConstructionScript
  (CallFunction|CreatePOIMap)
  (CallFunction|CreateCheckpointMap))

(fn CreatePOIMap
  (bind _poi_checkpoint_map (Variables|Default|GetPOI_Checkpoint_Map))
  (for (_array_element _array_index) (Variables|Default|GetCheckpoints)
    (if (not (Utilities|Map|Contains _poi_checkpoint_map _array_element))
      (Utilities|Map|Add _poi_checkpoint_map _array_element (Utilities|Array|Get(acopy) (Variables|Default|GetPoints_of_Interest) _array_index))
      (EventDispatchers|BindEventtoSpiritSaved _array_element (EventDispatchers|CreateEvent :!event Custom|Checkpoint_Saved_Spirit)))))

(fn CreateCheckpointMap
  (bind _spirittotems_checkpoint_map (Variables|Default|GetSpiritTotems_Checkpoint_Map))
  (for (_array_element _array_index) (Variables|Default|GetCheckpoints)
    (if (not (Utilities|Map|Contains _spirittotems_checkpoint_map _array_element))
      (Utilities|Map|Add _spirittotems_checkpoint_map _array_element (Utilities|Array|Get(acopy) (Variables|Default|GetSpirit_Totems) _array_index))
      (EventDispatchers|BindEventtoSpiritSaved _array_element (EventDispatchers|CreateEvent :!event Custom|Checkpoint_Saved_Spirit)))))