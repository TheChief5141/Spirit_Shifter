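; Isometric player character for a spirit-shifting game, with dash, tether, interaction and death retry screen.
; Spirits are swapped as actor components with matching headgear, while scarf materials reflect health.
; Dash tests progressively shorter distances with ground and collision traces for a safe landing.
; Tick runs interaction sphere traces and interpolates dash and cable-tether movement, pulling spirits or rocks to the player or the player to tether points.
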(event Custom|Remove_Spirit
  (bind _returnvalue (Actor|GetComponentbyClass "/Game/BluePrints/Spirits/Parent/AC_Parent_Spirit.AC_Parent_Spirit_C"))
  (Utilities|IsValid _returnvalue
    (:Is%20Valid
      (Components|DestroyComponent _returnvalue)
      (CallFunction|ReleaseSpirit (Variables|Default|GetCurrent_Spirit))
      (CallFunction|UpdateHeadgear "/Game/BluePrints/Spirits/Winged_Snake/AC_Winged_Spirit.AC_Winged_Spirit_C"))))

(event Custom|Add_Spirit
  (params (Added_Spirit :type AC%20Parent%20Spirit%20Class%20Reference))
  (bind _returnvalue (Actor|GetComponentbyClass "/Game/BluePrints/Spirits/Parent/AC_Parent_Spirit.AC_Parent_Spirit_C"))
  (Utilities|IsValid _returnvalue
    (:Is%20Valid
      (Components|DestroyComponent _returnvalue))
    (:Is%20Not%20Valid
      _))
  (Game|AddComponentbyClass self Added_Spirit)
  (CallFunction|UpdateHeadgear Added_Spirit)
  (Utilities|Array|Add (Variables|/Game/BluePrints/Gamemode/GI_Spirit_Shifter.GI_Spirit_Shifter_C|GetActive_Spirit_List (.AsGI%20Spirit%20Shifter (Utilities|Casting|CastToGI_Spirit_Shifter (Game|GetGameInstance)))) 0))

(event Custom|Release_Spirit
  (params (Spirit_To_Release :type BP%20Spirit%20Object%20Reference))
  (if (Utilities|ClassIsChildOf (Utilities|GetClass Spirit_To_Release) "/Game/BluePrints/Spirits/Parent/BP_Spirit.BP_Spirit_C")
    (Variables|/Game/BluePrints/Spirits/Parent/BP_Spirit.BP_Spirit_C|SetIs_Attached_To_Player Spirit_To_Release false)))

(event Custom|Update_Current_Spirit_Event
  (params (Spirit_Info_Class :type AC%20Parent%20Spirit%20Class%20Reference))
  (Game|AddComponentbyClass Spirit_Info_Class)
  (CallFunction|UpdateHeadgear Spirit_Info_Class))

(event Custom|Remove_Current_Spirit_Event
  (params (Spirit_Info_Class :type AC%20Parent%20Spirit%20Class%20Reference))
  (bind _returnvalue (Actor|GetComponentbyClass Spirit_Info_Class))
  (Utilities|IsValid _returnvalue
    (:Is%20Valid
      (Components|DestroyComponent _returnvalue)
      (CallFunction|ReleaseSpirit (Variables|Default|GetCurrent_Spirit))
      (CallFunction|UpdateHeadgear))))

(event Custom|Update_Headgear
  (params (New_Headgear :type AC%20Parent%20Spirit%20Class%20Reference))
  (bind _headgear_map (Variables|Default|GetHeadgear_Map))
  (bind (_value _returnvalue) (Utilities|Map|Find _headgear_map New_Headgear))
  (if _returnvalue
    (Components|StaticMesh|SetStaticMesh (Variables|Default|GetHeadGear) _value)
    (Components|Activation|Activate (Variables|Default|GetGearSwitch_VFX) false)))

(event Custom|NewSave
  (params (newPos :type Vector))
  (bind _mysave (Variables|Default|GetmySave))
  (Variables|/Game/BluePrints/Saves/BP_Save.BP_Save_C|SetspawnPosition _mysave newPos)
  (SaveGame|SaveGametoSlot _mysave "save1"))

(event Input|EnhancedActionEvents|EnhancedInputActionIA_Projectile
  (params (ActionValue :type Boolean) (ElapsedSeconds :type Float%20%28double-precision%29) (TriggeredSeconds :type Float%20%28double-precision%29) (InputAction :type Input%20Action%20Object%20Reference :default "/Game/Controls/Input_Actions/IA_Projectile.IA_Projectile"))
  (:Started
    (Animation|Montage|PlayMontage (Variables|Character|GetMesh) "/Game/Animations/Channeler_New_Model/Animations/AM_Projectile.AM_Projectile")))

(event Input|EnhancedActionEvents|EnhancedInputActionIA_Move
  (params (ActionValue :type Vector%202D%20Structure) (ElapsedSeconds :type Float%20%28double-precision%29) (TriggeredSeconds :type Float%20%28double-precision%29) (InputAction :type Input%20Action%20Object%20Reference :default "/Game/Controls/Input_Actions/IA_Move.IA_Move"))
  (:Started
    (Components|Activation|Activate (Variables|Default|GetFootstep_VFX) false)))

(event Input|EnhancedActionEvents|EnhancedInputActionIA_Interact
  (params (ActionValue :type Boolean) (ElapsedSeconds :type Float%20%28double-precision%29) (TriggeredSeconds :type Float%20%28double-precision%29) (InputAction :type Input%20Action%20Object%20Reference :default "/Game/Controls/Input_Actions/IA_Interact.IA_Interact"))
  (bind _spirit_interaction_actor (Variables|Default|GetSpirit_Interaction_Actor))
  (:Triggered
    (Utilities|IsValid _spirit_interaction_actor :!label _label
      (:Is%20Valid
        (Class|BIInteract|RunInteract(Message) _spirit_interaction_actor))))
  (:Started
    (goto _label)))

(event Input|EnhancedActionEvents|EnhancedInputActionIA_Jump
  (params (ActionValue :type Boolean) (ElapsedSeconds :type Float%20%28double-precision%29) (TriggeredSeconds :type Float%20%28double-precision%29) (InputAction :type Input%20Action%20Object%20Reference :default "/Game/Controls/Input_Actions/IA_Jump.IA_Jump")))

(event Input|EnhancedActionEvents|EnhancedInputActionIA_RemoveSpirit
  (params (ActionValue :type Boolean) (ElapsedSeconds :type Float%20%28double-precision%29) (TriggeredSeconds :type Float%20%28double-precision%29) (InputAction :type Input%20Action%20Object%20Reference :default "/Game/Controls/Input_Actions/IA_RemoveSpirit.IA_RemoveSpirit"))
  (:Started
    (CallFunction|RemoveSpirit)
    (CallFunction|AddSpirit "/Game/BluePrints/Spirits/Winged_Snake/AC_Winged_Spirit.AC_Winged_Spirit_C")))

(event Input|EnhancedActionEvents|EnhancedInputActionIA_Tether
  (params (ActionValue :type Boolean) (ElapsedSeconds :type Float%20%28double-precision%29) (TriggeredSeconds :type Float%20%28double-precision%29) (InputAction :type Input%20Action%20Object%20Reference :default "/Game/Controls/Input_Actions/IA_Tether.IA_Tether"))
  (:Triggered
    (bind _hit_successful (CallFunction|TetherStart))
    (if _hit_successful
      (Animation|Montage|PlayMontage (Variables|Character|GetMesh) "/Game/Animations/Channeler_New_Model/Animations/AM_Tether.AM_Tether" 2.0))))

(event EventTick
  (params (DeltaSeconds :type Float%20%28single-precision%29))
  (CallFunction|InteractionTrace)
  (CallFunction|TetherMovement)
  (if (Variables|Default|GetIsDashing)
    (CallFunction|DashStart self)
    (if (<= (Math|Vector|Distance2D(Vector) (Transformation|GetActorLocation (Game|GetPlayerCharacter 0)) (Variables|Default|GetDash_End_Location)) 16.0)
      (Variables|Default|SetIsDashing false))))

(event EventBeginPlay
  (bind _asbp_iso_player_controller (Utilities|Casting|CastToBP_Iso_Player_Controller (Pawn|GetController)))
  (Variables|Default|SetAs%20BP%20Iso%20Player%20Controller _asbp_iso_player_controller)
  (Utilities|IsValid (PlayerController|LocalPlayerSubsystems|GetEnhancedInputLocalPlayerSubsystem _asbp_iso_player_controller)
    (:Is%20Valid
      (Input|AddMappingContext (PlayerController|LocalPlayerSubsystems|GetEnhancedInputLocalPlayerSubsystem _asbp_iso_player_controller) "/Game/Controls/Input_Actions/IMC_Iso_Player_Controls.IMC_Iso_Player_Controls" 0 "(bIgnoreAllPressedKeysUntilRelease=True,bForceImmediately=False)")
      (bind _returnvalue (Actor|GetActorOfClass "/Game/BluePrints/Camera/BP_Camera_Spline.BP_Camera_Spline_C"))
      (Variables|Default|SetCamera_Spline_Reference _returnvalue)
      (Variables|Default|SetCurrent_AC (Variables|Default|GetWinged_Spirit))
      (CallFunction|UpdateDashDistance (Variables|Default|GetDash_Distance))
      (EventDispatchers|BindEventtoUpdateCurrentSpirit (EventDispatchers|CreateEvent :!event Custom|Add_Spirit))
      (EventDispatchers|BindEventtoRemoveCurrentSpirit (EventDispatchers|CreateEvent :!event Custom|Remove_Current_Spirit_Event))
      (Variables|Default|SetisEnemy false)
      (CallFunction|UpdateHealth)
      (Variables|Default|SetCurrent_AC 0))))

(event EventDestroyed
  (Development|PrintString "destroyed in character")
  (bind _asgmb_spirit_shifter (Utilities|Casting|CastToGMB_Spirit_Shifter (Game|GetGameMode)))
  (Utilities|FlowControl|DoOnce false
    (:Completed
      (Default|RespawnPlayer _asgmb_spirit_shifter self))))

(event Collision|EventActorBeginOverlap
  (params (OtherActor :type Actor%20Object%20Reference)))

(event EventOnLanded
  (params (Hit :type Hit%20Result%20Structure%20%28by%20ref%29))
  (Variables|/Script/Engine.CharacterMovementComponent|SetGravityScale (Variables|Character|GetCharacterMovement) 1.0)
  (Audio|PlaySoundatLocation "/Game/Audio/AudioClips/SFX/phase2/grassreal.grassreal" (Transformation|GetActorLocation) "0, 0, 0" 1.0 1.0 0.0 0 0 0 0))

(event Game|Damage|EventAnyDamage
  (params (Damage :type Float%20%28single-precision%29) (DamageType :type Damage%20Type%20Object%20Reference) (InstigatedBy :type Controller%20Object%20Reference) (DamageCauser :type Actor%20Object%20Reference))
  (|CallParentFunction Damage 0 0 0)
  (CallFunction|UpdateHealth)
  (Rendering|Material|SetScalarParameterValueonMaterials (Variables|Default|GetRigged_Scarf) "Mask" (* (- (/ (Variables|Default|GetunitHealth) 1e+02) 1.0) -1.0)))

(event EventUnitDeath
  (bind _returnvalue (Game|GetPlayerController 0))
  (Components|DestroyComponent (Variables|Character|GetMesh))
  (Components|DestroyComponent (Variables|Default|GetHeadGear))
  (bind _returnvalue_2 (UserInterface|CreateWidget "/Game/HUD/WBP_RetryScreen.WBP_RetryScreen_C" _returnvalue))
  (UserInterface|Viewport|AddtoViewport _returnvalue_2 0)
  (Input|SetInputModeUIOnly _returnvalue _returnvalue_2 "DoNotLock" false))

(event EventOnMovementModeChanged
  (params (PrevMovementMode :type EMovementMode%20Enum :default "MOVE_None") (NewMovementMode :type EMovementMode%20Enum :default "MOVE_None") (PrevCustomMode :type Byte :default 0) (NewCustomMode :type Byte :default 0))
  (if (Utilities|Enum|Equal(Enum) NewMovementMode "MOVE_Walking")
    (CallFunction|EndFloat)))

(fn ConstructionScript)

(fn ChangeSpirit
  (params (Current_Component :type AC%20Parent%20Spirit%20Object%20Reference) (Current_Sprite_Index :type Integer) (Current_Sprite_List :type Map%20of%20Strings%20to%20Classs))
  (bind _sprite_index (Variables|Default|GetSprite_Index))
  (bind (_value _returnvalue) (Utilities|Map|Find _sprite_index Current_Sprite_Index))
  (if _returnvalue
    (Components|DestroyComponent Current_Component)
    (switch string _value
      (:Light_Fish
        (bind _returnvalue_2 (Game|AddComponentbyClass (.Value (Utilities|Map|Find Current_Sprite_List _value))))
        (bind _output_get (Variables|Default|SetCurrent_AC _returnvalue_2))
        (return _output_get)))
    (else
      (Development|PrintString "not found"))))

(fn InterlerpRotation
  (params (Current_Rotation :type Rotator) (Target_Rotation :type Rotator))
  (bind _output_get (Variables|Default|SetCurrent_Rotation (Class|KismetMathLibrary|RInterptoConstant Current_Rotation Target_Rotation (Utilities|Time|GetWorldDeltaSeconds) (Variables|Default|GetInterp%20Speed))))
  (return _output_get))

(fn SetTargetForwardX
  (params (Mouse%20Input%20X :type Float%20%28double-precision%29))
  (bind _target_forward (Variables|Default|GetTarget_Forward))
  (return (Math|Vector|MakeVector Mouse%20Input%20X (.y _target_forward) (.z _target_forward))))

(fn SetTargetForwardY
  (params (Mouse_Input_Y :type Float%20%28double-precision%29))
  (bind _target_forward (Variables|Default|GetTarget_Forward))
  (return (Math|Vector|MakeVector (.x _target_forward) Mouse_Input_Y (.z _target_forward))))

(fn DirectiontoRotation
  (params (Target_Forward :type Vector))
  (return (Math|Conversions|RotationFromXVector Target_Forward)))

(fn RotateCharacter
  (bind _returnvalue (Game|GetPlayerController 0))
  (bind _asbp_iso_player_controller (Utilities|Casting|CastToBP_Iso_Player_Controller _returnvalue))
  (Transformation|SetActorRotation (Class|KismetMathLibrary|RInterptoConstant (Transformation|GetActorRotation _asbp_iso_player_controller) (Math|Rotator|FindLookatRotation (Transformation|GetActorLocation _asbp_iso_player_controller) (.WorldLocation (Game|Player|ConvertMouseLocationToWorldSpace _returnvalue))) (Utilities|Time|GetWorldDeltaSeconds) (Variables|Default|GetInterp%20Speed))))

(fn SubtractTempDashDistance
  (Variables|Default|SetTemp_Dash_Distance (- (Variables|Default|GetTemp_Dash_Distance) (* (.OutRadius (Components|Capsule|GetScaledCapsuleSize (Variables|/Script/Engine.Character|GetCapsuleComponent (.AsBP%20Iso%20Player%20Character (Utilities|Casting|CastToBP_Iso_PlayerCharacter (Game|GetPlayerCharacter 0)))))) 2.4))))

(fn UpdateDashDistance
  (params (Dashin :type Float%20%28double-precision%29))
  (Variables|Default|SetTemp_Dash_Distance Dashin)
  (Variables|Default|SetLast%20Index (Math|Float|Truncate (/ Dashin (* (.OutRadius (Components|Capsule|GetScaledCapsuleSize (Variables|/Script/Engine.Character|GetCapsuleComponent (.AsBP%20Iso%20Player%20Character (Utilities|Casting|CastToBP_Iso_PlayerCharacter (Game|GetPlayerCharacter 0)))))) 2.4)))))

(fn InteractionTrace
  (bind _returnvalue (Transformation|GetActorLocation))
  (bind (_outhit _returnvalue_2) (Collision|SphereTraceByChannel _returnvalue (+ (- _returnvalue "0.000000,0.000000,100.000000") (* (Transformation|GetActorForwardVector) (Variables|Default|GetSpirit_Interaction_Distance))) 2e+02 "TraceTypeQuery3" false 0 "None"))
  (if _returnvalue_2
    (if (Utilities|DoesObjectImplementInterface (.HitActor (Collision|BreakHitResult _outhit)) "/Game/BluePrints/Interfaces/BI_Interact.BI_Interact_C")
      (Class|BIInteract|CanInteract(Message) (.HitActor (Collision|BreakHitResult _outhit)))
      (Variables|Default|SetSpirit_Interaction_Actor (.HitActor (Collision|BreakHitResult _outhit))))
    (else
      (Variables|Default|SetSpirit_Interaction_Actor 0))))

(fn StartHealth
  (bind _materialparameterinfo (Utilities|Struct|MakeMaterialParameterInfo "BaseColor" "GlobalParameter" 0))
  (bind _headgear (Variables|Default|GetHeadGear))
  (bind _max_health_color (Variables|Default|GetMax_Health_Color))
  (bind _returnvalue (Rendering|Material|CreateDynamicMaterialInstance _headgear 0 (Rendering|Material|GetMaterial _headgear 0) "None" :!class /Script/Engine.PrimitiveComponent))
  (Variables|Default|SetMaterial%20Parameter%20Info _materialparameterinfo)
  (bind _output_get (Variables|Default|SetDynamic_Material_Reference _returnvalue))
  (Class|MaterialInstanceDynamic|SetVectorParameterValuebyInfo _output_get _materialparameterinfo _max_health_color)
  (Variables|Default|SetCurrent_Health_Color _max_health_color))

(fn UpdateHealth
  (Rendering|Material|SetScalarParameterValueonMaterials (Variables|Character|GetMesh) "Scarf_Mask" (Math|Float|Lerp 1.8 0.5 (Variables|Default|GetunitHealth))))

(fn CalculateJumpVelocity
  (bind _returnvalue (Transformation|GetVelocity))
  (bind _returnvalue_2 (Math|Vector|VectorLength _returnvalue))
  (return (Math|Float|SelectFloat (* _returnvalue_2 0.8) 3.5e+02 (< _returnvalue_2 5e+01))))

(fn IsFalling)

(fn TetherStart
  (bind _mesh (Variables|Character|GetMesh))
  (bind _hit_actor (Variables|Default|GetHit%20Actor))
  (if (not (Variables|Default|GetIsTetherActive))
    (bind (_end_location _hit_successful) (CallFunction|CalculateTetherHit))
    (if _hit_successful
      (bind _returnvalue (AddComponent|AddCableComponent true (Transformation|GetSocketTransform _mesh "CC_Base_R_Hand" "RTS_World")))
      (Transformation|AttachComponentToComponent _returnvalue _mesh "CC_Base_R_Hand" "SnapToTarget" "SnapToTarget" "SnapToTarget" true)
      (Variables|Default|SetTemp_TetherRef _returnvalue)
      (Utilities|IsValid _hit_actor
        (:Is%20Valid
          (Class|CableComponent|SetAttachEndto _returnvalue _hit_actor "None" "None"))
        (:Is%20Not%20Valid
          (Components|DestroyComponent _returnvalue)))
      (Variables|Default|SetEnd_Location_Of_Tether _end_location)
      (bind _output_get (Variables|Default|SetIsTetherActive true))
      (return _output_get))))

(fn CalculateTetherHit
  (bind _returnvalue (Game|GetPlayerController 0))
  (bind _returnvalue_2 (Transformation|GetActorLocation))
  (bind _capsulecomponent (Variables|Default|GetCapsuleComponent))
  (bind _playercameramanager (Variables|/Script/Engine.PlayerController|GetPlayerCameraManager _returnvalue))
  (bind _returnvalue_3 (Transformation|GetActorForwardVector _playercameramanager))
  (bind (_x _y) (Class|KismetMathLibrary|BreakVector3f _returnvalue_3))
  (bind (_outhit _returnvalue_4) (Collision|SphereTraceByChannel _returnvalue_2 (+ _returnvalue_2 (* (Math|Vector|MakeVector _x _y 0.0) (Variables|Default|GetDistance_Multipler))) 6e+01 "TraceTypeQuery3" false 0 "None"))
  (if _returnvalue_4
    (if (or (Utilities|ClassIsChildOf (Utilities|GetClass (.HitActor (Collision|BreakHitResult _outhit))) "/Game/BluePrints/Spirits/Parent/BP_Spirit.BP_Spirit_C") (Utilities|ClassIsChildOf (Utilities|GetClass (.HitActor (Collision|BreakHitResult _outhit))) "/Game/BluePrints/Environment/BP_Rock.BP_Rock_C"))
      (Variables|Default|SetHit%20Actor (.HitActor (Collision|BreakHitResult _outhit))))
    (if (Utilities|ClassIsChildOf (Utilities|GetClass (.HitActor (Collision|BreakHitResult _outhit))) "/Game/BluePrints/Spirits/Winged_Snake/BP_Tether_Point.BP_Tether_Point_C")
      (bind _output_get (Variables|Default|SetImpact%20Point (.ImpactPoint (Collision|BreakHitResult _outhit))))
      (bind (_outhit_2 _returnvalue_5) (Collision|CapsuleTraceByChannel (- _output_get (* (Math|Vector|GetUnitDirection(Vector) (.TraceStart (Collision|BreakHitResult _outhit)) (.TraceEnd (Collision|BreakHitResult _outhit))) 2e+02)) _output_get (Components|Capsule|GetScaledCapsuleRadius _capsulecomponent) (Components|Capsule|GetScaledCapsuleHalfHeight _capsulecomponent) "TraceTypeQuery1" false (Utilities|Array|MakeArray self) "None"))
      (if _returnvalue_5
        (return (.Location (Collision|BreakHitResult _outhit_2)) true)
        (else
          (return (.TraceEnd (Collision|BreakHitResult _outhit_2)) true)))
      (elif (or (Utilities|ClassIsChildOf (Utilities|GetClass (.HitActor (Collision|BreakHitResult _outhit))) "/Game/BluePrints/Spirits/Parent/BP_Spirit.BP_Spirit_C") (Utilities|ClassIsChildOf (Utilities|GetClass (.HitActor (Collision|BreakHitResult _outhit))) "/Game/BluePrints/Environment/BP_Rock.BP_Rock_C"))
        (return (.ImpactPoint (Collision|BreakHitResult _outhit)) true)
        (else
          (return "0, 0, 0" false))))
    (else
      (return "0, 0, 0" false))))

(fn TetherMovement
  (bind _self self)
  (bind _temp_tetherref (Variables|Default|GetTemp_TetherRef))
  (bind _temp_tetherref_2 (Variables|Default|GetTemp_TetherRef))
  (bind _returnvalue (Transformation|GetActorLocation _self))
  (if (Variables|Default|GetIsTetherActive)
    (Utilities|IsValid (Variables|Default|GetHit%20Actor)
      (:Is%20Valid
        (Transformation|SetActorLocation (Variables|Default|GetHit%20Actor) (Math|Interpolation|VInterpTo (Transformation|GetActorLocation (Variables|Default|GetHit%20Actor)) _returnvalue (Utilities|Time|GetWorldDeltaSeconds) 12.0) false false)
        (if (<= (Math|Vector|Distance2D(Vector) (Transformation|GetActorLocation (Variables|Default|GetHit%20Actor)) _returnvalue) 72.0)
          (Variables|Default|SetIsTetherActive false)
          (Variables|Default|SetHit%20Actor 0)
          (Utilities|IsValid _temp_tetherref
            (:Is%20Valid
              (Components|DestroyComponent _temp_tetherref)))))
      (:Is%20Not%20Valid
        (Transformation|SetActorLocation _self (Math|Interpolation|VInterpTo (Transformation|GetActorLocation _self) (Variables|Default|GetEnd_Location_Of_Tether) (Utilities|Time|GetWorldDeltaSeconds) 12.0) false false)
        (if (<= (Math|Vector|Distance2D(Vector) (Transformation|GetActorLocation _self) (Variables|Default|GetEnd_Location_Of_Tether)) 72.0)
          (Variables|Default|SetIsTetherActive false)
          (Utilities|IsValid _temp_tetherref_2
            (:Is%20Valid
              (Components|DestroyComponent _temp_tetherref_2))))))))

(fn StartFloat
  (bind _charactermovement (Variables|Character|GetCharacterMovement))
  (bind _halt_amount (LocalVariables|GetHalt_Amount))
  (Variables|/Script/Engine.MovementComponent|SetVelocity _charactermovement (Math|Vector|MakeVector (/ (.x (Variables|/Script/Engine.MovementComponent|GetVelocity _charactermovement)) _halt_amount) (/ (.y (Variables|/Script/Engine.MovementComponent|GetVelocity _charactermovement)) _halt_amount) (LocalVariables|GetFall_Speed)))
  (Variables|/Script/Engine.CharacterMovementComponent|SetGravityScale _charactermovement 0.0)
  (Variables|Default|SetisGliding? true))

(fn EndFloat
  (Variables|/Script/Engine.CharacterMovementComponent|SetGravityScale (Variables|Character|GetCharacterMovement) 1.0)
  (Variables|Default|SetisGliding? false)
  (Variables|/Game/BluePrints/Player/BP_Iso_Player_Controller.BP_Iso_Player_Controller_C|SetisGliding? (Variables|Default|GetAs%20BP%20Iso%20Player%20Controller) false))

(event Custom|Dash_Tracing
  (params (Possesed_Character :type Character%20Object%20Reference))
  (bind _returnvalue (Game|GetPlayerCharacter 0))
  (bind _returnvalue_2 (Game|GetPlayerCharacter 0))
  (bind _capsulecomponent (Variables|/Script/Engine.Character|GetCapsuleComponent Possesed_Character))
  (bind _returnvalue_3 (Transformation|GetWorldLocation _capsulecomponent))
  (bind _returnvalue_4 (Transformation|GetWorldLocation _capsulecomponent))
  (bind _returnvalue_5 (Components|Capsule|GetScaledCapsuleHalfHeight _capsulecomponent))
  (bind _array (Utilities|Array|MakeArray _returnvalue_2))
  (bind _capsulecomponent_2 (Variables|/Script/Engine.Character|GetCapsuleComponent _returnvalue))
  (bind _returnvalue_6 (Transformation|GetWorldLocation _capsulecomponent_2))
  ;[1 1 1] Dash Trace
  (Utilities|FlowControl|ForLoopwithBreak 0 (Variables|Default|GetLast%20Index)
    (:LoopBody
      (bind (_outhit _returnvalue_7) (Collision|LineTraceByChannel _returnvalue_3 (- _returnvalue_3 "0.000000,0.000000,300.000000") "TraceTypeQuery1" false 0 "None"))
      (if _returnvalue_7
        (bind (_outhit_2 _returnvalue_8) (Collision|SphereTraceByChannel (+ _returnvalue_4 "0.000000,0.000000,100.000000") (+ (+ _returnvalue_4 (* (Math|Vector|Normalize (Math|Vector|ProjectVectorontoPlane (Pawn|Components|PawnMovement|GetLastInputVector (Variables|/Script/Engine.Character|GetCharacterMovement Possesed_Character)) (.Normal (Collision|BreakHitResult _outhit)))) (Variables|Default|GetTemp_Dash_Distance))) "0.000000,0.000000,100.000000") 5e+01 "TraceTypeQuery1" false _array "None"))
        (if _returnvalue_8
          (CallFunction|SubtractTempDashDistance)
          (else
            (bind (_outhit_3 _returnvalue_9) (Collision|LineTraceByChannel (+ (.TraceEnd (Collision|BreakHitResult _outhit_2)) "0.000000,0.000000,100.000000") (+ (.TraceEnd (Collision|BreakHitResult _outhit_2)) "0.000000,0.000000,-1000.000000") "TraceTypeQuery1" false _array "None"))
            (if _returnvalue_9
              (bind (_outhit_4 _returnvalue_10) (Collision|CapsuleTraceByChannel (+ (.Location (Collision|BreakHitResult _outhit_3)) (* (.Normal (Collision|BreakHitResult _outhit_3)) (+ _returnvalue_5 25.0))) (+ (.Location (Collision|BreakHitResult _outhit_3)) (* (.Normal (Collision|BreakHitResult _outhit_3)) (+ _returnvalue_5 25.0))) (Components|Capsule|GetScaledCapsuleRadius _capsulecomponent) _returnvalue_5 "TraceTypeQuery1" false _array "None"))
              (if _returnvalue_10
                (CallFunction|SubtractTempDashDistance)
                (else
                  (Variables|Default|SetDash_End_Location (.TraceEnd (Collision|BreakHitResult _outhit_4)))
                  (CallFunction|BreakDashLoop)))
              (else
                (CallFunction|SubtractTempDashDistance)))))))
    (:Completed
      (Variables|Default|SetTemp_Dash_Distance (Variables|Default|GetDash_Distance))
      (if (not (Variables|Default|GetIsDashing))
        (Variables|Default|SetDash_End_Location _returnvalue_6)
        (Variables|Default|SetIsDashing true)
        (Audio|PlaySoundatLocation "/Game/Audio/AudioClips/SFX/phase2/snakedash.snakedash" _returnvalue_6 "0, 0, 0" 1.0 1.0 0.0 "/Game/Audio/EnemyAtten.EnemyAtten" 0 0 0)))))

(event Custom|Dash_End
  ;[1 1 1] Dashing Start
  (Input|EnableInput (stale Custom|Dash_Start Possesed_Pawn) (Game|GetPlayerController 0))
  (Variables|Default|SetIsDashing false))

(event Custom|Break_Dash_Loop
  (bind _returnvalue (Game|GetPlayerCharacter 0))
  (bind _returnvalue_2 (Game|GetPlayerCharacter 0))
  (bind _array (Utilities|Array|MakeArray _returnvalue_2))
  (bind _capsulecomponent (Variables|/Script/Engine.Character|GetCapsuleComponent _returnvalue))
  (bind _returnvalue_3 (Transformation|GetWorldLocation _capsulecomponent))
  ;[1 1 1] Dash Trace
  (if (not (Variables|Default|GetIsDashing))
    (Variables|Default|SetIsDashing true)
    (Utilities|FlowControl|ForLoopwithBreak 0 (Variables|Default|GetLast%20Index)) ; enters at Break
  ))

(event Custom|Dash_Start
  (params (Possesed_Pawn :type Character%20Object%20Reference))
  ;[1 1 1] Dashing Start
  (Input|DisableInput Possesed_Pawn (Game|GetPlayerController 0))
  (Transformation|SetActorLocation Possesed_Pawn (Math|Interpolation|VInterpTo (Transformation|GetActorLocation Possesed_Pawn) (Variables|Default|GetDash_End_Location) (Utilities|Time|GetWorldDeltaSeconds) (Variables|Default|GetInterp%20Speed)) true false)
  (bind _returnvalue (Utilities|Time|SetTimerbyEvent (delegate Custom|Dash_End) (Variables|Default|GetDash_Time)))
  (Variables|Default|SetTimer _returnvalue))

(event Input|EnhancedActionEvents|EnhancedInputActionIA_Dash
  (params (ActionValue :type Boolean) (ElapsedSeconds :type Float%20%28double-precision%29) (TriggeredSeconds :type Float%20%28double-precision%29) (InputAction :type Input%20Action%20Object%20Reference :default "/Game/Controls/Input_Actions/IA_Dash.IA_Dash"))
  (:Started
    (CallFunction|DashTracing (Game|GetPlayerCharacter 0))
    (Components|Activation|Activate (Variables|Default|GetDash_VFX) true)
    (Animation|Montage|PlayMontage (Variables|Character|GetMesh) "/Game/Animations/Channeler_New_Model/Animations/AM_Dash.AM_Dash")))