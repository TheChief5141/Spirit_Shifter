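; BP_Light_Receiver is an environment actor that reacts to a one-shot ToggleState event, latching on the first call even if OnOff is false.
; If OnOff is true, a timeline drives the mesh material's "Position" parameter.
; On completion it spawns a slam VFX and moves any valid Checkpoint to itself.
; An unconnected chain holds a camera-blend cutscene that would send ToggleStateMessage to ActorList.
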(event EventToggleState
  (params (On/Off :type Boolean))
  (bind _returnvalue (Transformation|GetActorTransform))
  (bind _checkpoint (Variables|Default|GetCheckpoint))
  (if (not (Variables|Default|GetToggled_State))
    (Variables|Default|SetToggled_State true)
    (if On/Off
      (Utilities|FlowControl|Sequence
        (:then_0
          (bind _alpha (Timeline|Timeline Play)
            (:Update
              (Rendering|Material|SetScalarParameterValueonMaterials (Variables|Default|GetStaticMesh) "Position" (Math|Float|Lerp 0.0 1e+01 _alpha)))
            (:Finished
              (Niagara|SpawnSystematLocation "/Game/Particles/VFX_Slam.VFX_Slam" (.location _returnvalue) (.rotation _returnvalue) (.scale _returnvalue))
              (Utilities|IsValid _checkpoint
                (:Is%20Valid
                  (Transformation|SetActorLocation _checkpoint (Transformation|GetActorLocation) false false))))))))))

(fn ConstructionScript)