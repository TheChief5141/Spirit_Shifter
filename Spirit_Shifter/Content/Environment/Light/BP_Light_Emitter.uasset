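; Light emitter that casts a reflecting beam from its arrow, switching on any BP_Light_Receiver it ends on.
; Tick, through a short delay, destroys the previous beams, switches off the last gem, then line traces in a loop, spawning a BP_Light_Cylinder per segment.
; Hits on M_TetherBox material mirror the direction, flattened to horizontal, and continue; anything else ends the loop.
; The bounce counter does not limit reflections, as its check is unwired.
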(event EventTick
  (params (DeltaSeconds :type Float%20%28single-precision%29))
  (bind _arrow (Variables|Default|GetArrow))
  (Utilities|FlowControl|Delay 0.01)
  (CallFunction|CastLight (Transformation|GetWorldLocation _arrow) (Math|Vector|GetForwardVector (Transformation|GetWorldRotation _arrow)) (Variables|Default|GetCast_Distance)))

(fn ConstructionScript)

(fn CastLight
  (params (Cast_Origin :type Vector) (Cast_Direction :type Vector) (Cast_Distance :type Float%20%28double-precision%29))
  (bind _beams (Variables|Default|GetBeams))
  (bind _output_get (LocalVariables|SetTemp_Cast_Origin Cast_Origin))
  (bind _output_get_2 (LocalVariables|SetTemp_Cast_Direction Cast_Direction))
  (bind _output_get_3 (LocalVariables|SetTemp_Cast_Distance Cast_Distance))
  (Variables|Default|SetTotal_Bounces 1)
  (for _array_element _beams
    (Actor|DestroyActor _array_element))
  (Utilities|Array|Clear _beams)
  (Class|BPIStates|ToggleState(Message) (Variables|Default|GetActivated_Gem) false)
  (while (LocalVariables|GetTemp_Continue)
    (Utilities|FlowControl|Sequence
      (:then_0
        (bind (_outhit _returnvalue) (Collision|LineTraceByChannel _output_get (+ _output_get (* _output_get_2 _output_get_3)) "TraceTypeQuery4" true 0 "None"))
        (LocalVariables|SetTemp_Beam_Start (LocalVariables|GetTemp_Cast_Origin))
        (if _returnvalue
          (LocalVariables|SetTemp_Beam_End (.ImpactPoint (Collision|BreakHitResult _outhit)))
          (if (== (.ReturnValue (Class|PrimitiveComponent|GetMaterialfromCollisionFaceIndex (.HitComponent (Collision|BreakHitResult _outhit)))) "/Game/Models/Environment_Pieces/TetherPoint/M_TetherBox.M_TetherBox")
            (LocalVariables|SetTemp_Cast_Origin (.ImpactPoint (Collision|BreakHitResult _outhit)))
            (LocalVariables|SetTemp_Cast_Direction (Math|Vector|ProjectVectorontoPlane (Math|Vector|MirrorVectorbyNormal (LocalVariables|GetTemp_Cast_Direction) (.ImpactNormal (Collision|BreakHitResult _outhit))) "0.000000,0.000000,1.000000"))
            (LocalVariables|SetTemp_Continue true)
            (else
              (if (Utilities|ClassIsChildOf (Utilities|GetClass (.HitActor (Collision|BreakHitResult _outhit))) "/Game/Environment/Light/BP_Light_Receiver.BP_Light_Receiver_C")
                (Class|BPIStates|ToggleState(Message) (.HitActor (Collision|BreakHitResult _outhit)) true)
                (Variables|Default|SetActivated_Gem (.HitActor (Collision|BreakHitResult _outhit))))
              (LocalVariables|SetTemp_Continue false :!label _label)))
          (else
            (LocalVariables|SetTemp_Beam_End (+ _output_get (* _output_get_2 _output_get_3)))
            (goto _label))))
      (:then_1
        (bind _returnvalue_2 (Game|SpawnActorfromClass "/Game/Environment/Light/BP_Light_Cylinder.BP_Light_Cylinder_C" (Math|Transform|MakeTransform "0, 0, 0" "0, 0, 0" "1.000000,1.000000,1.000000") "Undefined" "MultiplyWithRoot" 0 0))
        (Default|SetEnd _returnvalue_2 (LocalVariables|GetTemp_Beam_Start) (LocalVariables|GetTemp_Beam_End))
        (Utilities|Array|Add (Variables|Default|GetBeams) _returnvalue_2)
        (Math|Integer|DecrementInt (Variables|Default|GetTotal_Bounces))))))