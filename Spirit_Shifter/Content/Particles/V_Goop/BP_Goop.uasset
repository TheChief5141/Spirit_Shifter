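; Spline-shaped goop hazard that slows and damages the isometric player character and spirits.
; The construction script tiles query-only spline meshes along the spline, with section length tied to actor Z scale and width following spline scale, and binds overlap events on each.
; Begin overlap lowers walk speed and deals one hit of damage, while end overlap sets a fixed faster speed.
; The damage timer events are empty stubs.
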(event Custom|Actor_Overlap
  (params (OverlappedComponent :type Primitive%20Component%20Object%20Reference) (OtherActor :type Actor%20Object%20Reference) (OtherComp :type Primitive%20Component%20Object%20Reference) (OtherBodyIndex :type Integer) (bFromSweep :type Boolean) (SweepResult :type Hit%20Result%20Structure%20%28by%20ref%29))
  (bind _returnvalue (Utilities|GetClass OtherActor))
  (if (or (Utilities|ClassIsChildOf _returnvalue "/Game/BluePrints/Player/BP_Iso_PlayerCharacter.BP_Iso_PlayerCharacter_C") (Utilities|ClassIsChildOf _returnvalue "/Game/BluePrints/Spirits/Parent/BP_Spirit.BP_Spirit_C"))
    (bind _ascharacter (Utilities|Casting|CastToCharacter OtherActor))
    (Variables|/Script/Engine.CharacterMovementComponent|SetMaxWalkSpeed (Variables|/Script/Engine.Character|GetCharacterMovement _ascharacter) 4e+02)
    (Game|Damage|ApplyDamage OtherActor 12.0 0 0)))

(event Custom|End_Overlap
  (params (OverlappedComponent :type Primitive%20Component%20Object%20Reference) (OtherActor :type Actor%20Object%20Reference) (OtherComp :type Primitive%20Component%20Object%20Reference) (OtherBodyIndex :type Integer))
  (bind _returnvalue (Utilities|GetClass OtherActor))
  (if (or (Utilities|ClassIsChildOf _returnvalue "/Game/BluePrints/Player/BP_Iso_PlayerCharacter.BP_Iso_PlayerCharacter_C") (Utilities|ClassIsChildOf _returnvalue "/Game/BluePrints/Spirits/Parent/BP_Spirit.BP_Spirit_C"))
    (bind _ascharacter (Utilities|Casting|CastToCharacter OtherActor))
    (Variables|/Script/Engine.CharacterMovementComponent|SetMaxWalkSpeed (Variables|/Script/Engine.Character|GetCharacterMovement _ascharacter) 1.2e+03)))

(event Custom|Damage_Timer_Event
  (params (Damaged_Actor :type Actor%20Object%20Reference)))

(event Custom|Damage_Timer_Even_Binded_Timer)

(event EventBeginPlay)

(event Collision|EventActorBeginOverlap
  (params (OtherActor :type Actor%20Object%20Reference)))

(event EventTick
  (params (DeltaSeconds :type Float%20%28single-precision%29)))

(fn ConstructionScript
  (bind _spline (Variables|Default|GetSpline))
  (Variables|Default|SetSection_Length (* 1e+02 (.z (Transformation|GetActorScale3D))))
  (CallFunction|RunWindRail (Math|Float|Truncate (/ (Spline|GetSplineLength _spline) (Variables|Default|GetSection_Length))) _spline))

(fn RunWindRail
  (params (Point_Along_Spline :type Integer) (Spline_Component :type Spline%20Component%20Object%20Reference))
  (for _index (range 0 Point_Along_Spline)
    (bind _returnvalue (AddComponent|AddSplineMeshComponent false))
    (SplineMesh|SetForwardAxis _returnvalue "Y" true)
    (Collision|SetCollisionEnabled _returnvalue "QueryOnly")
    (SplineMesh|SetStartandEnd _returnvalue (Spline|GetLocationatDistanceAlongSpline Spline_Component (* (Variables|Default|GetSection_Length) _index) "Local") (Math|Vector|ClampVectorSize (Spline|GetTangentatDistanceAlongSpline Spline_Component (* (Variables|Default|GetSection_Length) _index) "Local") 0.0 (Variables|Default|GetSection_Length)) (Spline|GetLocationatDistanceAlongSpline Spline_Component (* (Variables|Default|GetSection_Length) (+ _index 1)) "Local") (Math|Vector|ClampVectorSize (Spline|GetTangentatDistanceAlongSpline Spline_Component (* (Variables|Default|GetSection_Length) (+ _index 1)) "Local") 0.0 (Variables|Default|GetSection_Length)) true :!class /Script/Engine.SplineMeshComponent)
    (SplineMesh|SetStartScale _returnvalue (Math|Vector2D|MakeVector2D (.y (Class|SplineComponent|GetScaleatDistanceAlongSpline Spline_Component (* (Variables|Default|GetSection_Length) _index))) (.z (Class|SplineComponent|GetScaleatDistanceAlongSpline Spline_Component (* (Variables|Default|GetSection_Length) _index)))) true :!class /Script/Engine.SplineMeshComponent)
    (SplineMesh|SetEndScale _returnvalue (Math|Vector2D|MakeVector2D (.y (Class|SplineComponent|GetScaleatDistanceAlongSpline Spline_Component (* (Variables|Default|GetSection_Length) (+ _index 1)))) (.z (Class|SplineComponent|GetScaleatDistanceAlongSpline Spline_Component (* (Variables|Default|GetSection_Length) (+ _index 1))))) true :!class /Script/Engine.SplineMeshComponent)
    (Collision|BindEventtoOnComponentBeginOverlap _returnvalue (EventDispatchers|CreateEvent :!event Custom|Actor_Overlap))
    (Collision|BindEventtoOnComponentEndOverlap _returnvalue (EventDispatchers|CreateEvent :!event Custom|End_Overlap))))