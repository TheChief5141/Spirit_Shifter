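; Spline-driven water actor that builds a river or waterfall, selected by TypeOfWaterSpline.
; The construction script divides the spline into sections sized by actor Z scale, adding spline meshes with clamped tangents and spline-point scaling.
; River and waterfall differ in forward axis and collision, while lake only closes the loop because its mesh builder is empty.
; BeginPlay plays the Alpha timeline when UseMeshOnSpline is set, with no update logic attached.
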(event EventBeginPlay
  (if (Variables|Default|GetUseMeshOnSpline?)
    (Timeline|Alpha Play)))

(event Collision|EventActorBeginOverlap
  (params (OtherActor :type Actor%20Object%20Reference)))

(event EventTick
  (params (DeltaSeconds :type Float%20%28single-precision%29)))

(fn ConstructionScript
  (bind _spline (Variables|Default|GetSpline))
  (Variables|Default|SetSection_Length (* 2e+02 (.z (Transformation|GetActorScale3D))))
  (switch Utilities|FlowControl|Switch|SwitchonE_Water_Type (Variables|Default|GetType_Of_Water_Spline)
    (:NewEnumerator0
      (Spline|SetClosedLoop _spline false true)
      (CallFunction|RunRiverWaterSpline (Math|Float|Truncate (/ (Spline|GetSplineLength _spline) (Variables|Default|GetSection_Length))) _spline))
    (:NewEnumerator1
      (Spline|SetClosedLoop _spline false true)
      (CallFunction|RunWaterfallWaterSpline (Math|Float|Truncate (/ (Spline|GetSplineLength _spline) (Variables|Default|GetSection_Length))) _spline))
    (:NewEnumerator2
      (Spline|SetClosedLoop _spline true true)
      (CallFunction|RunLakeWaterSpline 0 0 _spline))))

(fn RunRiverWaterSpline
  (params (Point_Along_Spline :type Integer) (Spline_Component :type Spline%20Component%20Object%20Reference))
  (for _index (range 0 Point_Along_Spline)
    (bind _returnvalue (AddComponent|AddSplineMeshComponent false))
    (SplineMesh|SetForwardAxis _returnvalue "Y" true)
    (Collision|SetCollisionEnabled _returnvalue "ProbeOnly")
    (SplineMesh|SetStartandEnd _returnvalue (Spline|GetLocationatDistanceAlongSpline Spline_Component (* (Variables|Default|GetSection_Length) _index) "Local") (Math|Vector|ClampVectorSize (Spline|GetTangentatDistanceAlongSpline Spline_Component (* (Variables|Default|GetSection_Length) _index) "Local") 0.0 (Variables|Default|GetSection_Length)) (Spline|GetLocationatDistanceAlongSpline Spline_Component (* (Variables|Default|GetSection_Length) (+ _index 1)) "Local") (Math|Vector|ClampVectorSize (Spline|GetTangentatDistanceAlongSpline Spline_Component (* (Variables|Default|GetSection_Length) (+ _index 1)) "Local") 0.0 (Variables|Default|GetSection_Length)) true :!class /Script/Engine.SplineMeshComponent)
    (SplineMesh|SetStartScale _returnvalue (Math|Vector2D|MakeVector2D (.y (Class|SplineComponent|GetScaleatDistanceAlongSpline Spline_Component (* (Variables|Default|GetSection_Length) _index))) (.z (Class|SplineComponent|GetScaleatDistanceAlongSpline Spline_Component (* (Variables|Default|GetSection_Length) _index)))) true :!class /Script/Engine.SplineMeshComponent)
    (SplineMesh|SetEndScale _returnvalue (Math|Vector2D|MakeVector2D (.y (Class|SplineComponent|GetScaleatDistanceAlongSpline Spline_Component (* (Variables|Default|GetSection_Length) (+ _index 1)))) (.z (Class|SplineComponent|GetScaleatDistanceAlongSpline Spline_Component (* (Variables|Default|GetSection_Length) (+ _index 1))))) true :!class /Script/Engine.SplineMeshComponent)))

(fn RunWaterfallWaterSpline
  (params (Point_Along_Spline :type Integer) (Spline_Component :type Spline%20Component%20Object%20Reference))
  (for _index (range 0 Point_Along_Spline)
    (bind _returnvalue (AddComponent|AddSplineMeshComponent false))
    (SplineMesh|SetForwardAxis _returnvalue "X" true)
    (Collision|SetCollisionEnabled _returnvalue "QueryAndPhysics")
    (SplineMesh|SetStartandEnd _returnvalue (Spline|GetLocationatDistanceAlongSpline Spline_Component (* (Variables|Default|GetSection_Length) _index) "Local") (Math|Vector|ClampVectorSize (Spline|GetTangentatDistanceAlongSpline Spline_Component (* (Variables|Default|GetSection_Length) _index) "Local") 0.0 (Variables|Default|GetSection_Length)) (Spline|GetLocationatDistanceAlongSpline Spline_Component (* (Variables|Default|GetSection_Length) (+ _index 1)) "Local") (Math|Vector|ClampVectorSize (Spline|GetTangentatDistanceAlongSpline Spline_Component (* (Variables|Default|GetSection_Length) (+ _index 1)) "Local") 0.0 (Variables|Default|GetSection_Length)) true :!class /Script/Engine.SplineMeshComponent)
    (SplineMesh|SetStartScale _returnvalue (Math|Vector2D|MakeVector2D (.y (Class|SplineComponent|GetScaleatDistanceAlongSpline Spline_Component (* (Variables|Default|GetSection_Length) _index))) (.z (Class|SplineComponent|GetScaleatDistanceAlongSpline Spline_Component (* (Variables|Default|GetSection_Length) _index)))) true :!class /Script/Engine.SplineMeshComponent)
    (SplineMesh|SetEndScale _returnvalue (Math|Vector2D|MakeVector2D (.y (Class|SplineComponent|GetScaleatDistanceAlongSpline Spline_Component (* (Variables|Default|GetSection_Length) (+ _index 1)))) (.z (Class|SplineComponent|GetScaleatDistanceAlongSpline Spline_Component (* (Variables|Default|GetSection_Length) (+ _index 1))))) true :!class /Script/Engine.SplineMeshComponent)))

(fn RunLakeWaterSpline
  (params (Point_Along_Spline :type Integer) (Next_Point_Along_Spline :type Integer) (Spline_Component :type Spline%20Component%20Object%20Reference)))